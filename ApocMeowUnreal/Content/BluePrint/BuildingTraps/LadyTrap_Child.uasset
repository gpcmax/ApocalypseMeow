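; Lady trap child Blueprint, a buildable decoy that shows hearts when AI characters come near.
; Incoming damage adds to Health as build progress, applying the finished material part by part from base to head through nested thresholds.
; Reaching the head threshold makes it movable and ends building.
; Sphere overlaps with BP_AI_Character attach a heart emitter and destroy the stored one on exit.
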(event `self.ReceiveBeginPlay`
  ;[1 1 1] Set if u want to place in world
)

(event `self.ReceiveAnyDamage`
  (params (Damage :type "Float (single-precision)") (DamageType :type "DamageType Object Reference") (InstigatedBy :type "Controller Object Reference") (DamageCauser :type "Actor Object Reference"))
  ;[1 1 1] Take damage to be built
  (set `self.Health` (+ Damage (`self.Health`)))
  ;[1 1 1] Being built
  (set `self.BeingBuilt` true)
  ;[1 1 1] Base health
  (if (>= (`self.Health`) (`self.BaseHealth`))
    (`PrimitiveComponent.SetMaterial` (`self.TrapBase`) 0 "/Game/ART/trap/M_LadyTrap.M_LadyTrap")
    ;[1 1 1] Skirt
    (if (>= (`self.Health`) (`self.SkirtHealth`))
      (`PrimitiveComponent.SetMaterial` (`self.Skirt`) 0 "/Game/ART/trap/M_LadyTrap.M_LadyTrap")
      ;[1 1 1] Shirt
      (if (>= (`self.Health`) (`self.ShirtHealth`))
        (`PrimitiveComponent.SetMaterial` (`self.Shirt`) 0 "/Game/ART/trap/M_LadyTrap.M_LadyTrap")
        ;[1 1 1] Bra
        (if (>= (`self.Health`) (`self.BraHealth`))
          (`PrimitiveComponent.SetMaterial` (`self.Bra`) 0 "/Game/ART/trap/M_LadyTrap.M_LadyTrap")
          ;[1 1 1] Chest
          (if (>= (`self.Health`) (`self.ChestHealth`))
            (`PrimitiveComponent.SetMaterial` (`self.Chest`) 0 "/Game/ART/trap/M_LadyTrap.M_LadyTrap")
            ;[1 1 1] Hands
            (if (>= (`self.Health`) (`self.HandHealth`))
              (`PrimitiveComponent.SetMaterial` (`self.Hands`) 0 "/Game/ART/trap/M_LadyTrap.M_LadyTrap")
              ;[1 1 1] Head
              (if (>= (`self.Health`) (`self.HeadHealth`))
                (`PrimitiveComponent.SetMaterial` (`self.Head`) 0 "/Game/ART/trap/M_LadyTrap.M_LadyTrap")
                ;[1 1 1] Can be moved
                (set `self.CanBeMoved` true)
                ;[1 1 1] Not being built any more
                (set `self.BeingBuilt` false)))))))))

(event `self.Sphere.OnComponentBeginOverlap`
  (params (OverlappedComponent :type "PrimitiveComponent Object Reference") (OtherActor :type "Actor Object Reference") (OtherComp :type "PrimitiveComponent Object Reference") (OtherBodyIndex :type Integer) (bFromSweep :type Boolean) (SweepResult :type "HitResult Structure (by ref)"))
  ;[1 1 1] Enemy is being attracted
  (cast `/Game/BluePrint/AI/BP_AI_Character` OtherActor)
  (bind _returnvalue (`GameplayStatics.SpawnEmitterAttached` "/Game/ART/_POST/Particle/P_Heart.P_Heart" (`self.Scene`) "None" (0.0 0.0 0.0) (struct) (2.5 2.5 2.5) "SnapToTarget"))
  (set `self.Hearts` _returnvalue))

(event `self.Sphere.OnComponentEndOverlap`
  (params (OverlappedComponent :type "PrimitiveComponent Object Reference") (OtherActor :type "Actor Object Reference") (OtherComp :type "PrimitiveComponent Object Reference") (OtherBodyIndex :type Integer))
  (bind _hearts (`self.Hearts`))
  ;[1 1 1] Not attracted anymore
  (cast `/Game/BluePrint/AI/BP_AI_Character` OtherActor)
  (`/Engine/EditorBlueprintResources/StandardMacros.IsValid` _hearts
    (:`Is Valid`
      (`ActorComponent.K2_DestroyComponent` _hearts))))

(fn `UserConstructionScript`
  (`parent.UserConstructionScript`))