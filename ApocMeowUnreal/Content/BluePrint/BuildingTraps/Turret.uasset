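; Buildable turret Blueprint that reveals its top mesh as received damage accumulates, with no targeting or firing logic in this graph.
; BeginPlay hides TurretTop, and AnyDamage adds damage to Health rather than subtracting it, so Health acts like build progress.
; TurretTop becomes visible through two separate checks: Tick compares Health to MaxHealth every frame, while AnyDamage uses a hardcoded threshold.
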(event `self.ReceiveBeginPlay`
  (`SceneComponent.SetVisibility` (`self.TurretTop`) false false))

(event `self.ReceiveTick`
  (params (DeltaSeconds :type "Float (single-precision)"))
  (if (>= (`self.Health`) (`self.MaxHealth`))
    (`SceneComponent.SetVisibility` (`self.TurretTop`) true false)))

(event `self.ReceiveAnyDamage`
  (params (Damage :type "Float (single-precision)") (DamageType :type "DamageType Object Reference") (InstigatedBy :type "Controller Object Reference") (DamageCauser :type "Actor Object Reference"))
  (set `self.Health` (+ Damage (`self.Health`)))
  (if (>= (`self.Health`) 10.0)
    (`SceneComponent.SetVisibility` (`self.TurretTop`) true false)))

(fn `UserConstructionScript`)