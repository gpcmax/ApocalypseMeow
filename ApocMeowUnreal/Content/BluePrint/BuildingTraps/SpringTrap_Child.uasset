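; Buildable spring trap that launches AI characters and the villain player who overlap its box.
; Incoming damage counts as build progress, adding to Health and applying materials to parts at nested thresholds.
; The final threshold makes it movable and, once only, swaps the static parts for a skeletal launch pad played in reverse.
; Launches play animation and sounds and set Used, which makes Tick play the idle animation whenever the pad stops animating.
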(event `self.ReceiveBeginPlay`
  ;[1 1 1] Begin play
  (`SceneComponent.SetVisibility` (`self.SK_LaunchPad`) false false))

(event `self.ReceiveAnyDamage`
  (params (Damage :type "Float (single-precision)") (DamageType :type "DamageType Object Reference") (InstigatedBy :type "Controller Object Reference") (DamageCauser :type "Actor Object Reference"))
  (bind _sk_launchpad (`self.SK_LaunchPad`))
  ;[1 1 1] Take positive damage
  (set `self.Health` (+ Damage (`self.Health`)))
  ;[1 1 1] Being built
  (set `self.BeingBuilt` true)
  ;[1 1 1] Base health
  (if (>= (`self.Health`) (`self.BaseHealth`))
    (`PrimitiveComponent.SetMaterial` (`self.TrapBase`) 0 "/Game/ART/trap/lambert1.lambert1")
    ;[1 1 1] Skirt
    (if (>= (`self.Health`) (`self.SkirtHealth`))
      (`PrimitiveComponent.SetMaterial` (`self.Signs`) 0 "/Game/ART/trap/lambert1.lambert1")
      ;[1 1 1] Shirt
      (if (>= (`self.Health`) (`self.ShirtHealth`))
        (`PrimitiveComponent.SetMaterial` (`self.BasePole`) 0 "/Game/ART/trap/lambert1.lambert1")
        ;[1 1 1] Bra
        (if (>= (`self.Health`) (`self.BraHealth`))
          (`PrimitiveComponent.SetMaterial` (`self.BottomPole`) 0 "/Game/ART/trap/lambert1.lambert1")
          ;[1 1 1] Chest
          (if (>= (`self.Health`) (`self.ChestHealth`))
            (`PrimitiveComponent.SetMaterial` (`self.UpperPole`) 0 "/Game/ART/trap/lambert1.lambert1")
            ;[1 1 1] Hands
            (if (>= (`self.Health`) (`self.HandHealth`))
              (`PrimitiveComponent.SetMaterial` (`self.UpperPole`) 0 "/Game/ART/trap/lambert1.lambert1")
              ;[1 1 1] Head
              (if (>= (`self.Health`) (`self.HeadHealth`))
                (`PrimitiveComponent.SetMaterial` (`self.top`) 0 "/Game/ART/trap/lambert1.lambert1")
                ;[1 1 1] Trap can move
                (set `self.CanBeMoved` true)
                ;[1 1 1] No longer being built
                (set `self.BeingBuilt` false)
                ;[1 1 1] Trap is ready to be placed and has anims
                (`/Engine/EditorBlueprintResources/StandardMacros.DoOnce` false
                  (:`Completed`
                    (`SceneComponent.SetVisibility` (`self.TrapBase`) false true)
                    (`SceneComponent.SetVisibility` _sk_launchpad true false)
                    (`SkeletalMeshComponent.SetPlayRate` _sk_launchpad -1.0)
                    (`SkeletalMeshComponent.PlayAnimation` _sk_launchpad "/Game/ART/trap/SK_LaunchPad_Anim.SK_LaunchPad_Anim" false)
                    (`KismetSystemLibrary.Delay` 0.5)
                    (set `self.Used?` false)))))))))))

(event `self.Box.OnComponentBeginOverlap`
  (params (OverlappedComponent :type "PrimitiveComponent Object Reference") (OtherActor :type "Actor Object Reference") (OtherComp :type "PrimitiveComponent Object Reference") (OtherBodyIndex :type Integer) (bFromSweep :type Boolean) (SweepResult :type "HitResult Structure (by ref)"))
  (bind _returnvalue (`SceneComponent.K2_GetComponentLocation` (`self.TrapBase`)))
  ;[1 1 1] trap overlap
  (`|ExecutionSequence`
    (:`then_0`
      (bind _asbp_ai_character (cast `/Game/BluePrint/AI/BP_AI_Character` OtherActor))
      (`/Game/BluePrint/AI/BP_AI_Character.Launch` _asbp_ai_character))
    (:`then_1`
      (bind _asbp_villian_player (cast `/Game/BluePrint/Players/BP_VillianPlayer` OtherActor))
      (`/Game/BluePrint/Players/BP_VillianPlayer.Launch` _asbp_villian_player)))
  (set `self.Used?` true)
  (`SkeletalMeshComponent.PlayAnimation` (`self.SK_LaunchPad`) "/Game/ART/trap/SK_LaunchPad_Anim.SK_LaunchPad_Anim" false)
  ;[1 1 1] Launch Sounds
  (`GameplayStatics.PlaySoundAtLocation` "/Game/Audio/Traps/BoingCue.BoingCue" _returnvalue)
  (`GameplayStatics.PlaySoundAtLocation` "/Game/Audio/Traps/steamPiston.steamPiston" _returnvalue))

(event `self.ReceiveTick`
  (params (DeltaSeconds :type "Float (single-precision)"))
  (bind _sk_launchpad (`self.SK_LaunchPad`))
  ;[1 1 1] Tick
  (if (`self.Used?`)
    (if (not (`SkeletalMeshComponent.IsPlaying` _sk_launchpad))
      (`SkeletalMeshComponent.PlayAnimation` _sk_launchpad "/Game/ART/trap/Idle_Launch.Idle_Launch" false))))

(fn `UserConstructionScript`
  (`parent.UserConstructionScript`))