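; RadioPuzzle is a VR radio tower puzzle where seven specific pieces unlock a button that calls a jet.
; Each slot's overlap attaches its matching piece to a prop component, clears the player's HasPuzzlePiece flag and rechecks whether all seven are in.
; When unlocked, the player's overlap on the button plays a sound and the end-game level sequence, then destroys the placed pieces and resets the puzzle for reuse.
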(event `self.PuzzleCol01.OnComponentBeginOverlap`
  (params (OverlappedComponent :type "PrimitiveComponent Object Reference") (OtherActor :type "Actor Object Reference") (OtherComp :type "PrimitiveComponent Object Reference") (OtherBodyIndex :type Integer) (bFromSweep :type Boolean) (SweepResult :type "HitResult Structure (by ref)"))
  ;[1 1 1] Piece 1
  (bind _aspuzzle_piece_01 (cast `/Game/BluePrint/RadioTower/PuzzlePiece_01` OtherActor))
  (bind _output_get (set `self.Piece01` _aspuzzle_piece_01))
  (`self.SetLifeSpan` _output_get 0.0)
  (`self.K2_AttachToComponent` _output_get (`self.GameBoy`) "None" "KeepRelative" "KeepRelative" "KeepWorld" true)
  (set `self.P01In` true)
  (`self.PuzzleComplete`)
  (bind _asbp_vrchar_1 (cast `/Game/BluePrint/Players/BP_VRChar1` (`GameplayStatics.GetPlayerPawn` 0)))
  (set `/Game/BluePrint/Players/BP_VRChar1.HasPuzzlePiece` false _asbp_vrchar_1))

(event `self.PuzzleCol02.OnComponentBeginOverlap`
  (params (OverlappedComponent :type "PrimitiveComponent Object Reference") (OtherActor :type "Actor Object Reference") (OtherComp :type "PrimitiveComponent Object Reference") (OtherBodyIndex :type Integer) (bFromSweep :type Boolean) (SweepResult :type "HitResult Structure (by ref)"))
  ;[1 1 1] Puzzle 2
  (bind _aspuzzle_piece_02 (cast `/Game/BluePrint/RadioTower/PuzzlePiece_02` OtherActor))
  (bind _output_get (set `self.Piece02` _aspuzzle_piece_02))
  (`self.SetLifeSpan` _output_get 0.0)
  (`self.K2_AttachToComponent` _output_get (`self.Potatoe`) "None" "SnapToTarget" "SnapToTarget" "KeepWorld" true)
  (set `self.P02In` true)
  (`self.PuzzleComplete`)
  (bind _asbp_vrchar_1 (cast `/Game/BluePrint/Players/BP_VRChar1` (`GameplayStatics.GetPlayerPawn` 0)))
  (set `/Game/BluePrint/Players/BP_VRChar1.HasPuzzlePiece` false _asbp_vrchar_1))

(event `self.PuzzleCol03.OnComponentBeginOverlap`
  (params (OverlappedComponent :type "PrimitiveComponent Object Reference") (OtherActor :type "Actor Object Reference") (OtherComp :type "PrimitiveComponent Object Reference") (OtherBodyIndex :type Integer) (bFromSweep :type Boolean) (SweepResult :type "HitResult Structure (by ref)"))
  ;[1 1 1] Puzzle 3
  (bind _aspuzzle_piece_03 (cast `/Game/BluePrint/RadioTower/PuzzlePiece_03` OtherActor))
  (bind _output_get (set `self.Piece03` _aspuzzle_piece_03))
  (`self.SetLifeSpan` _output_get 0.0)
  (`self.K2_AttachToComponent` _output_get (`self.PEZ`) "None" "SnapToTarget" "SnapToTarget" "KeepWorld" true)
  (set `self.P03In` true)
  (`self.PuzzleComplete`)
  (bind _asbp_vrchar_1 (cast `/Game/BluePrint/Players/BP_VRChar1` (`GameplayStatics.GetPlayerPawn` 0)))
  (set `/Game/BluePrint/Players/BP_VRChar1.HasPuzzlePiece` false _asbp_vrchar_1))

(event `self.PuzzleCol04.OnComponentBeginOverlap`
  (params (OverlappedComponent :type "PrimitiveComponent Object Reference") (OtherActor :type "Actor Object Reference") (OtherComp :type "PrimitiveComponent Object Reference") (OtherBodyIndex :type Integer) (bFromSweep :type Boolean) (SweepResult :type "HitResult Structure (by ref)"))
  ;[1 1 1] Puzzle 4
  (bind _aspuzzle_piece_04 (cast `/Game/BluePrint/RadioTower/PuzzlePiece_04` OtherActor))
  (bind _output_get (set `self.Piece04` _aspuzzle_piece_04))
  (`self.SetLifeSpan` _output_get 0.0)
  (`self.K2_AttachToComponent` _output_get (`self.Spoon`) "None" "SnapToTarget" "SnapToTarget" "KeepWorld" true)
  (set `self.P04In` true)
  (`self.PuzzleComplete`)
  (bind _asbp_vrchar_1 (cast `/Game/BluePrint/Players/BP_VRChar1` (`GameplayStatics.GetPlayerPawn` 0)))
  (set `/Game/BluePrint/Players/BP_VRChar1.HasPuzzlePiece` false _asbp_vrchar_1))

(event `self.PuzzleCol05.OnComponentBeginOverlap`
  (params (OverlappedComponent :type "PrimitiveComponent Object Reference") (OtherActor :type "Actor Object Reference") (OtherComp :type "PrimitiveComponent Object Reference") (OtherBodyIndex :type Integer) (bFromSweep :type Boolean) (SweepResult :type "HitResult Structure (by ref)"))
  ;[1 1 1] Puzzle 5
  (bind _aspuzzle_piece_05 (cast `/Game/BluePrint/RadioTower/PuzzlePiece_05` OtherActor))
  (bind _output_get (set `self.Piece05` _aspuzzle_piece_05))
  (`self.SetLifeSpan` _output_get 0.0)
  (`self.K2_AttachToComponent` _output_get (`self.Bottle`) "None" "SnapToTarget" "SnapToTarget" "KeepWorld" true)
  (set `self.P05In` true)
  (`self.PuzzleComplete`)
  (bind _asbp_vrchar_1 (cast `/Game/BluePrint/Players/BP_VRChar1` (`GameplayStatics.GetPlayerPawn` 0)))
  (set `/Game/BluePrint/Players/BP_VRChar1.HasPuzzlePiece` false _asbp_vrchar_1))

(event `self.PuzzleCol06.OnComponentBeginOverlap`
  (params (OverlappedComponent :type "PrimitiveComponent Object Reference") (OtherActor :type "Actor Object Reference") (OtherComp :type "PrimitiveComponent Object Reference") (OtherBodyIndex :type Integer) (bFromSweep :type Boolean) (SweepResult :type "HitResult Structure (by ref)"))
  ;[1 1 1] Puzzle 6
  (bind _aspuzzle_piece_06 (cast `/Game/BluePrint/RadioTower/PuzzlePiece_06` OtherActor))
  (bind _output_get (set `self.Piece06` _aspuzzle_piece_06))
  (`self.SetLifeSpan` _output_get 0.0)
  (`self.K2_AttachToComponent` _output_get (`self.Battery01`) "None" "SnapToTarget" "SnapToTarget" "KeepWorld" true)
  (set `self.P06In` true)
  (`self.PuzzleComplete`)
  (bind _asbp_vrchar_1 (cast `/Game/BluePrint/Players/BP_VRChar1` (`GameplayStatics.GetPlayerPawn` 0)))
  (set `/Game/BluePrint/Players/BP_VRChar1.HasPuzzlePiece` false _asbp_vrchar_1))

(event `PuzzleComplete`
  ;[1 1 1] Puzzle Complete
  (if (and (`self.P01In`) (`self.P02In`) (`self.P03In`) (`self.P04In`) (`self.P05In`) (`self.P06In`) (`self.P07In`))
    (set `self.CanHitButton` true)
    (else
      (set `self.CanHitButton` false))))

(event `self.PuzzleCol07.OnComponentBeginOverlap`
  (params (OverlappedComponent :type "PrimitiveComponent Object Reference") (OtherActor :type "Actor Object Reference") (OtherComp :type "PrimitiveComponent Object Reference") (OtherBodyIndex :type Integer) (bFromSweep :type Boolean) (SweepResult :type "HitResult Structure (by ref)"))
  ;[1 1 1] Puzzle 7
  (bind _aspuzzle_piece_07 (cast `/Game/BluePrint/RadioTower/PuzzlePiece_07` OtherActor))
  (bind _output_get (set `self.Piece07` _aspuzzle_piece_07))
  (`self.SetLifeSpan` _output_get 0.0)
  (`self.K2_AttachToComponent` _output_get (`self.Battery02`) "None" "SnapToTarget" "SnapToTarget" "KeepWorld" true)
  (set `self.P07In` true)
  (`self.PuzzleComplete`)
  (bind _asbp_vrchar_1 (cast `/Game/BluePrint/Players/BP_VRChar1` (`GameplayStatics.GetPlayerPawn` 0)))
  (set `/Game/BluePrint/Players/BP_VRChar1.HasPuzzlePiece` false _asbp_vrchar_1))

(event `ResetPuzzle`
  (bind _piece07 (`self.Piece07`))
  (bind _piece06 (`self.Piece06`))
  (bind _piece05 (`self.Piece05`))
  (bind _piece04 (`self.Piece04`))
  (bind _piece03 (`self.Piece03`))
  (bind _piece02 (`self.Piece02`))
  (bind _piece01 (`self.Piece01`))
  ;[1 1 1] Reset Puzzle
  (`|ExecutionSequence`
    (:`then_0`
      (set `self.P01In` false)
      (`/Engine/EditorBlueprintResources/StandardMacros.IsValid` _piece01
        (:`Is Valid`
          (`self.K2_DestroyActor` _piece01))))
    (:`then_1`
      (set `self.P02In` false)
      (`/Engine/EditorBlueprintResources/StandardMacros.IsValid` _piece02
        (:`Is Valid`
          (`self.K2_DestroyActor` _piece02))))
    (:`then_2`
      (set `self.P03In` false)
      (`/Engine/EditorBlueprintResources/StandardMacros.IsValid` _piece03
        (:`Is Valid`
          (`self.K2_DestroyActor` _piece03))))
    (:`then_3`
      (set `self.P04In` false)
      (`/Engine/EditorBlueprintResources/StandardMacros.IsValid` _piece04
        (:`Is Valid`
          (`self.K2_DestroyActor` _piece04))))
    (:`then_4`
      (set `self.P05In` false)
      (`/Engine/EditorBlueprintResources/StandardMacros.IsValid` _piece05
        (:`Is Valid`
          (`self.K2_DestroyActor` _piece05))))
    (:`then_5`
      (set `self.P06In` false)
      (`/Engine/EditorBlueprintResources/StandardMacros.IsValid` _piece06
        (:`Is Valid`
          (`self.K2_DestroyActor` _piece06))))
    (:`then_6`
      (set `self.P07In` false)
      (`/Engine/EditorBlueprintResources/StandardMacros.IsValid` _piece07
        (:`Is Valid`
          (`self.K2_DestroyActor` _piece07))))
    (:`then_7`
      (set `self.CanHitButton` false)
      (`self.PuzzleCanBeUsedAgain`))))

(event `self.Button.OnComponentBeginOverlap`
  (params (OverlappedComponent :type "PrimitiveComponent Object Reference") (OtherActor :type "Actor Object Reference") (OtherComp :type "PrimitiveComponent Object Reference") (OtherBodyIndex :type Integer) (bFromSweep :type Boolean) (SweepResult :type "HitResult Structure (by ref)"))
  ;[1 1 1] Button to call jet
  (cast `/Game/BluePrint/Players/BP_VRChar1` OtherActor)
  (if (`self.CanHitButton`)
    (`GameplayStatics.PlaySoundAtLocation` "/Game/Audio/Radio/go-go-go.go-go-go" (`SceneComponent.K2_GetComponentLocation` (`self.Button`)) :!label _label)
    (bind (_outactor _returnvalue) (`LevelSequencePlayer.CreateLevelSequencePlayer` (`self.EndGame_Seq`)))
    (`MovieSceneSequencePlayer.Play` _returnvalue)
    (`self.ResetPuzzle`)))

(event `PuzzleCanBeUsedAgain`
  ;[1 1 1] Button to call jet
  (`/Engine/EditorBlueprintResources/StandardMacros.DoOnce` false :!via `Reset`
    (:`Completed`
      (goto _label))))

(fn `UserConstructionScript`)