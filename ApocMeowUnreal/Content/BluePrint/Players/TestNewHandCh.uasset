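; VR player character that spawns motion-controller hands and two ammo spawners for gunplay with manual reloading.
; BeginPlay spawns left and right BP_PlayerRightHands at the VR origin and BP_AmmoSpawn actors at two spawn points, attaching each.
; Trigger presses drive that hand's TriggerPull, store any returned weapon and attempt ReloadGrab against both ammo spawners; release closes the hand.
; Reload inputs empty that hand's gun.
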(event `self.ReceiveBeginPlay`
  (`|ExecutionSequence`
    (:`then_0`
      (bind _gethand (`self.HandSpawn` "Right" true))
      (set `self.RightHand` _gethand))
    (:`then_1`
      (bind _gethand_2 (`self.HandSpawn` "Left"))
      (set `self.LeftHand` _gethand_2))
    (:`then_2`
      (bind _returnammo (`self.AmmoBoxSpawn` (`self.AmmoSpawnLeft`)))
      (set `self.LeftAmmo` _returnammo))
    (:`then_3`
      (bind _returnammo_2 (`self.AmmoBoxSpawn` (`self.AmmoSpawnRight`)))
      (set `self.RightAmmo` _returnammo_2))))

(event `Key|MotionController_Right_Trigger`
  (params (Key :type "Key Structure"))
  (bind _righthand (`self.RightHand`))
  (:`Pressed`
    (bind (_ammo _currentweapon) (`/Game/BluePrint/Players/BP_PlayerRightHands.TriggerPull` _righthand _righthand))
    (`/Engine/EditorBlueprintResources/StandardMacros.IsValid` _currentweapon
      (:`Is Valid`
        (set `self.Weapon` _currentweapon))
      (:`Is Not Valid`
        _))
    (`/Game/BluePrint/Players/BP_PlayerRightHands.ReloadGrab` _righthand _righthand null (`self.LeftAmmo`))
    (`/Game/BluePrint/Players/BP_PlayerRightHands.ReloadGrab` _righthand _righthand null (`self.RightAmmo`)))
  (:`Released`
    (`/Game/BluePrint/Players/BP_PlayerRightHands.CloseHand` _righthand)))

(event `Key|MotionController_Left_Trigger`
  (params (Key :type "Key Structure"))
  (bind _lefthand (`self.LeftHand`))
  (:`Pressed`
    (bind (_ammo _currentweapon) (`/Game/BluePrint/Players/BP_PlayerRightHands.TriggerPull` _lefthand _lefthand))
    (`/Engine/EditorBlueprintResources/StandardMacros.IsValid` _currentweapon
      (:`Is Valid`
        (set `self.Weapon` _currentweapon))
      (:`Is Not Valid`
        _))
    (`/Game/BluePrint/Players/BP_PlayerRightHands.ReloadGrab` _lefthand _lefthand null (`self.LeftAmmo`))
    (`/Game/BluePrint/Players/BP_PlayerRightHands.ReloadGrab` _lefthand _lefthand null (`self.RightAmmo`)))
  (:`Released`
    (`/Game/BluePrint/Players/BP_PlayerRightHands.CloseHand` _lefthand)))

(event `self.AmmoBox.OnComponentBeginOverlap`
  (params (OverlappedComponent :type "PrimitiveComponent Object Reference") (OtherActor :type "Actor Object Reference") (OtherComp :type "PrimitiveComponent Object Reference") (OtherBodyIndex :type Integer) (bFromSweep :type Boolean) (SweepResult :type "HitResult Structure (by ref)")))

(event `self.AmmoBox.OnComponentEndOverlap`
  (params (OverlappedComponent :type "PrimitiveComponent Object Reference") (OtherActor :type "Actor Object Reference") (OtherComp :type "PrimitiveComponent Object Reference") (OtherBodyIndex :type Integer)))

(event `InputAction|LeftReload`
  (params (Key :type "Key Structure"))
  (:`Pressed`
    (`/Game/BluePrint/Players/BP_PlayerRightHands.EmptyGun` (`self.LeftHand`))))

(event `InputAction|RightReload`
  (params (Key :type "Key Structure"))
  (:`Pressed`
    (`/Game/BluePrint/Players/BP_PlayerRightHands.EmptyGun` (`self.RightHand`))))

(fn `AmmoBoxSpawn`
  (params (SpawnLoc :type "SceneComponent Object Reference"))
  (returns (ReturnAmmo :type "/Game/BluePrint/Players/BP_AmmoSpawn Object Reference"))
  (locals (CurrentAmmo :type "/Game/BluePrint/Players/BP_AmmoSpawn Object Reference"))
  (bind _returnvalue (`|SpawnActorFromClass` "/Game/BluePrint/Players/BP_AmmoSpawn.BP_AmmoSpawn_C" (`SceneComponent.K2_GetComponentToWorld` SpawnLoc) "Undefined" "OverrideRootScale" self null))
  (`self.K2_AttachToComponent` _returnvalue null "None" "SnapToTarget" "SnapToTarget" "KeepWorld" false)
  (return _returnvalue))

(fn `HandSpawn`
  (params (Hand :type "EControllerHand Enum" :default "Left") (RightHand :type Boolean))
  (returns (GetHand :type "/Game/BluePrint/Players/BP_PlayerRightHands Object Reference"))
  (locals (NewLocalVar_0 :type "/Game/BluePrint/ENUMs/EHandGrips Enum" :default "NewEnumerator0"))
  (bind _returnvalue (`|SpawnActorFromClass` "/Game/BluePrint/Players/BP_PlayerRightHands.BP_PlayerRightHands_C" (`SceneComponent.K2_GetComponentToWorld` (`self.VROringe`)) "AlwaysSpawn" "OverrideRootScale" self Hand RightHand null))
  (`self.K2_AttachToComponent` _returnvalue null "None" "SnapToTarget" "SnapToTarget" "KeepWorld" false)
  (return _returnvalue))

(fn `UserConstructionScript`)