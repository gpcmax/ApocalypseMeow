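; VR player character that handles motion-controller weapon use and scrap-gated turret placement.
; Grip, trigger, shoulder and reload inputs send messages to overlapping pistols and rifles, gated by holster flags.
; Left trigger at the ammo pouch spawns hand-held rifle ammo, dropped on release; pistol ammo branches are empty.
; With weapons holstered, right trigger toggles a TurretPlacer preview traced onto Floor-tagged surfaces, though its gate's timeline driver is disconnected.
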(event `self.ReceiveBeginPlay`
  ;[1 1 1] Begin PLay
  (bind _asai_character (cast `AI_Character` (`self.GetOwner`)))
  (set `self.AI_Var` _asai_character))

(event `self.ReceiveTick`
  (params (DeltaSeconds :type "Float (single-precision)"))
  (bind _vrcamera (`self.VRCamera`))
  (bind (_returnvalue_roll _returnvalue_pitch _returnvalue_yaw) (`KismetMathLibrary.BreakRotator` (`SceneComponent.K2_GetComponentRotation` _vrcamera)))
  ;[1 1 1] tick
  (`|ExecutionSequence`
    (:`then_0`
      (`SceneComponent.K2_SetWorldLocationAndRotation` (`self.VRBodyScene`) (`SceneComponent.K2_GetComponentLocation` _vrcamera) (`KismetMathLibrary.MakeRotator` 0.0 0.0 _returnvalue_yaw) false false))
    (:`then_1`
      (set `self.DeltaSecondsVar` DeltaSeconds))
    (:`then_2`
      (`TextRenderComponent.K2_SetText` (`self.ScrapCounter`) (`KismetTextLibrary.Conv_StringToText` (`KismetStringLibrary.Concat_StrStr` "Scrap: " (`KismetStringLibrary.Conv_IntToString` (`self.ScrapInt`))))))))

(event `Key|MotionController_Right_Grip1`
  (params (Key :type "Key Structure"))
  (bind _overlappingactors (`self.GetOverlappingActors` "/Game/BluePrint/Weapons/Rifles/BP_RifleWeaponsMaster.BP_RifleWeaponsMaster_C"))
  ;[1 0.07812 0.07812] Weapon interactons
  ;;[1 1 1] lets player grab the gun
  (:`Pressed`
    (`|ExecutionSequence`
      (:`then_0`
        (message `/Game/BluePrint/Weapons/BP_WeaponInteractions.GrabGun` _overlappingactors null))
      (:`then_1`
        (message `/Game/BluePrint/Weapons/BP_WeaponInteractions.HolsterTheGun` _overlappingactors)))))

(event `Key|MotionController_Right_Grip1`
  (params (Key :type "Key Structure"))
  (bind _overlappingactors (`self.GetOverlappingActors` null))
  ;[1 0.07812 0.07812] Weapon interactons
  ;;[1 1 1] pistol
  (:`Pressed`
    (`|ExecutionSequence`
      (:`then_0`
        (message `/Game/BluePrint/Weapons/BP_WeaponInteractions.GrabGun` _overlappingactors null))
      (:`then_1`
        (message `/Game/BluePrint/Weapons/BP_WeaponInteractions.HolsterTheGun` _overlappingactors)))))

(event `Key|MotionController_Left_Grip1`
  (params (Key :type "Key Structure"))
  ;[1 0.07812 0.07812] Weapon interactons
  ;;[1 1 1] Lets player hold the gun in both hands
  (:`Pressed`
    (message `/Game/BluePrint/Weapons/BP_WeaponInteractions.2ndHandGrip` (`self.GetOverlappingActors` "/Game/BluePrint/Weapons/Rifles/BP_RifleWeaponsMaster.BP_RifleWeaponsMaster_C"))))

(event `InputAction|PistolReload`
  (params (Key :type "Key Structure"))
  (bind _overlappingactors (`self.GetOverlappingActors` null))
  ;[1 0.07812 0.07812] Weapon interactons
  ;;[1 1 1] pistol
  (:`Pressed`
    (if (not (`self.IsHolster?`))
      (`|ExecutionSequence`
        (:`then_0`
          (if (`self.HasSwatPistol`)
            (message `/Game/BluePrint/Weapons/BP_WeaponInteractions.ReloadWeapon` _overlappingactors)))
        (:`then_1`
          (if (`self.HasPixel gun`)
            (message `/Game/BluePrint/Weapons/BP_WeaponInteractions.ReloadWeapon` _overlappingactors)))))))

(event `Key|MotionController_Right_Trigger`
  (params (Key :type "Key Structure"))
  ;[1 0.07812 0.07812] Weapon interactons
  ;;[1 1 1] pistol
  (:`Pressed`
    (if (not (`self.IsHolster?`))
      (message `/Game/BluePrint/Weapons/BP_WeaponInteractions.FireWeapon` (`self.GetOverlappingActors` null)))))

(event `Key|MotionController_Right_Trigger`
  (params (Key :type "Key Structure"))
  ;[1 0.07812 0.07812] Weapon interactons
  ;;[1 1 1] Fires the rifle
  (:`Pressed`
    (if (not (`self.RifleHolstered`))
      (message `/Game/BluePrint/Weapons/BP_WeaponInteractions.FireWeapon` (`self.GetOverlappingActors` "/Game/BluePrint/Weapons/Rifles/BP_RifleWeaponsMaster.BP_RifleWeaponsMaster_C")))))

(event `Key|MotionController_Right_Shoulder`
  (params (Key :type "Key Structure"))
  ;[1 1 1] Drop pistol
  (:`Pressed`
    (if (not (`self.IsHolster?`))
      (message `/Game/BluePrint/Weapons/BP_WeaponInteractions.Drop` (`self.GetOverlappingActors` null))
      (set `self.HasPixel gun` false)
      (set `self.HasSwatPistol` false))))

(event `InputAction|PistolReload`
  (params (Key :type "Key Structure"))
  (bind _rifleammo (`self.RifleAmmo`))
  ;[1 0.07812 0.07812] Weapon interactons
  (:`Pressed`
    (if (not (`self.RifleHolstered`))
      (message `/Game/BluePrint/Weapons/BP_WeaponInteractions.ReloadWeapon` (`self.GetOverlappingActors` "/Game/BluePrint/Weapons/Rifles/BP_RifleWeaponsMaster.BP_RifleWeaponsMaster_C"))
      (`self.K2_DetachFromActor` _rifleammo "KeepWorld" "KeepWorld" "KeepWorld")
      (`PrimitiveComponent.SetCollisionEnabled` (`/Game/BluePrint/Weapons/Ammo/BP_PistolAmmoMaster.AmmoBoxColl` _rifleammo) "NoCollision")
      (`PrimitiveComponent.SetSimulatePhysics` (`/Game/BluePrint/Weapons/Ammo/BP_PistolAmmoMaster.PistolMagMesh` _rifleammo) true)
      (`self.SetLifeSpan` _rifleammo 3.0))))

(event `Key|MotionController_Right_Trigger`
  (params (Key :type "Key Structure"))
  (bind _currentturret (`self.CurrentTurret`))
  (bind _currentturret_2 (`self.CurrentTurret`))
  (bind _righthandmeshsk (`self.RightHandMeshSK`))
  (bind _returnvalue (`SceneComponent.K2_GetComponentLocation` _righthandmeshsk))
  ;[1 1 1] TurretSyste,
  (:`Pressed`
    (if (`self.IsHolster?`)
      (if (`self.RifleHolstered`)
        (if (>= (`self.ScrapInt`) 20)
          (`/Engine/EditorBlueprintResources/StandardMacros.FlipFlop`
            (:`A`
              (`/Engine/EditorBlueprintResources/StandardMacros.Gate` true :!via `Open` :!label _label
                (:`Exit`
                  (`|ExecutionSequence`
                    (:`then_0`
                      (`/Engine/EditorBlueprintResources/StandardMacros.DoOnce` false :!label _label_2
                        (:`Completed`
                          (set `self.TurretRot` (struct))
                          (set `self.TurretRotOffset` 0.0))))
                    (:`then_1`
                      (set `self.TurretRotOffset` (+ (`self.TurretRotOffset`) (* (`self.GetInputAxisKeyValue`) (`self.TurretTurnSpeed`))))
                      (bind _outhit (`KismetSystemLibrary.LineTraceSingle` :`Start` _returnvalue :`End` (+ (* (`SceneComponent.GetForwardVector` _righthandmeshsk) 5000.0) _returnvalue) :`TraceChannel` "TraceTypeQuery1" :`DrawDebugType` "ForDuration"))
                      (bind (_returnvalue_roll _returnvalue_pitch _returnvalue_yaw) (`KismetMathLibrary.BreakRotator` (`KismetMathLibrary.FindLookAtRotation` _returnvalue (`.Location` (`GameplayStatics.BreakHitResult` _outhit)))))
                      (set `self.TurretRot` (`KismetMathLibrary.MakeRotator` 0.0 0.0 (+ _returnvalue_yaw (`self.TurretRotOffset`))))
                      (if (`self.ActorHasTag` (`.HitActor` (`GameplayStatics.BreakHitResult` _outhit)) "Floor")
                        (`|ExecutionSequence`
                          (:`then_0`
                            (`/Engine/EditorBlueprintResources/StandardMacros.DoOnce` false :!label _label_3
                              (:`Completed`
                                (bind _returnvalue_2 (`|SpawnActorFromClass` "/Game/FirstPersonBP/Blueprints/TurretPlacer.TurretPlacer_C" (`KismetMathLibrary.MakeTransform` (`.Location` (`GameplayStatics.BreakHitResult` _outhit))) "Undefined" "OverrideRootScale" null self "(INVALID)" null))
                                (set `self.CurrentTurret` _returnvalue_2))))
                          (:`then_1`
                            (`self.K2_SetActorLocation` _currentturret (`.Location` (`GameplayStatics.BreakHitResult` _outhit)) false false)
                            (`self.K2_SetActorRotation` _currentturret (`self.TurretRot`) false)
                            (set `/Game/FirstPersonBP/Blueprints/TurretPlacer.Placed` false _currentturret)))
                        (else
                          (`/Engine/EditorBlueprintResources/StandardMacros.IsValid` _currentturret_2
                            (:`Is Valid`
                              (`self.K2_DestroyActor` _currentturret_2)
                              (goto _label_3 :!via `Reset`))))))))))
            (:`B`
              (`|ExecutionSequence`
                (:`then_0`
                  (goto _label :!via `Close`))
                (:`then_1`
                  (goto _label_2 :!via `Reset`))
                (:`then_2`
                  (goto _label_3 :!via `Reset`))
                (:`then_3`
                  (set `/Game/FirstPersonBP/Blueprints/TurretPlacer.Placed` true (`self.CurrentTurret`)))))))))))

(event `Key|MotionController_Left_Trigger`
  (params (Key :type "Key Structure"))
  (bind _rifleammo (`self.RifleAmmo`))
  (bind _lefthandmeshsk (`self.LeftHandMeshSK`))
  ;[1 1 1] Reload and dropping ammo
  (:`Pressed`
    (`|ExecutionSequence`
      (:`then_0`
        ;;[1 1 1] Spawn ammo and connect to your hand
        (if (`self.IsHolster?`)
          _
          (elif (not (`PrimitiveComponent.IsOverlappingComponent` (`self.AmmoPouchCol`) (`self.LeftHandCol`)))
            (`|ExecutionSequence`
              (:`then_1`
                (if (`self.HasPixel gun`)
                  _))))))
      (:`then_1`
        (if (`self.RifleHolstered`)
          _
          (elif (`PrimitiveComponent.IsOverlappingComponent` (`self.AmmoPouchCol`) (`self.LeftHandCol`))
            (bind _returnvalue (`|SpawnActorFromClass` "/Game/BluePrint/Weapons/Ammo/BP_RifleAmmo_Child.BP_RifleAmmo_Child_C" (`SceneComponent.K2_GetComponentToWorld` _lefthandmeshsk) "Undefined" "OverrideRootScale" null null))
            (bind _output_get (set `self.RifleAmmo` _returnvalue))
            (`self.K2_AttachToComponent` _output_get _lefthandmeshsk "None" "SnapToTarget" "SnapToTarget" "KeepWorld" true)
            (set `self.HoldingAmmo` true))))))
  (:`Released`
    (if (`self.HoldingAmmo`)
      (`|ExecutionSequence`
        (:`then_0`
          (if (not (`self.IsHolster?`))
            (`|ExecutionSequence`
              (:`then_0`
                (if (`self.HasPixel gun`)
                  _))
              (:`then_1`
                (if (`self.HasSwatPistol`)
                  _)))))
        (:`then_1`
          (if (not (`self.RifleHolstered`))
            (`self.K2_DetachFromActor` _rifleammo "KeepWorld" "KeepWorld" "KeepWorld")
            (`PrimitiveComponent.SetCollisionEnabled` (`/Game/BluePrint/Weapons/Ammo/BP_PistolAmmoMaster.AmmoBoxColl` _rifleammo) "NoCollision")
            (`PrimitiveComponent.SetSimulatePhysics` (`/Game/BluePrint/Weapons/Ammo/BP_PistolAmmoMaster.PistolMagMesh` _rifleammo) true)
            (`self.SetLifeSpan` _rifleammo 3.0)
            (set `self.HoldingAmmo` false)))))))

(fn `Ammo`
  (return))

(fn `GrabGun`
  (params (HandInput :type "/Game/BluePrint/Players/BP_PlayerRightHands Object Reference"))
  (returns (Ammo :type "Actor Class Reference") (CurrentWeapon :type "/Game/BluePrint/Weapons/Rifles/BP_RifleWeaponsMaster Object Reference"))
  (return null null))

(fn `UserConstructionScript`
  (`SceneComponent.SetHiddenInGame` (`self.ScrapCounter`) true false))