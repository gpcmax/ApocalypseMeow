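; VR player character for a game with rifles, a hammer, puzzle pieces and traps.
; It spawns both hands; controller triggers drive context-sensitive grabbing, teleporting, firing and reloading through overlap checks, line traces and weapon messages, while Tick handles hammer-hit tracing and body tracking.
; It also forwards gamepad input to player 1's BP_VillianPlayer for asymmetric local play.
; Turret placement and watch-menu logic are disconnected, as are the timelines feeding trap-movement and enemy-melee gates.
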(event `NewHandsSpawn`
  (bind _returnvalue (`KismetMathLibrary.MakeTransform` (0.0 0.0 0.0)))
  (bind _vrorigin (`self.VROrigin`))
  (`|ExecutionSequence`
    (:`then_0`
      (bind _returnvalue_2 (`|SpawnActorFromClass` "/Game/BluePrint/Players/BP_PlayerRightHands.BP_PlayerRightHands_C" _returnvalue "AlwaysSpawn" "OverrideRootScale" self "Right" true null))
      (bind _output_get (set `self.RightHand` _returnvalue_2))
      (`self.K2_AttachToComponent` (`self.RightHand`) _vrorigin "None" "SnapToTarget" "SnapToTarget" "KeepWorld" true)
      (`self.K2_AttachToComponent` _output_get _vrorigin "None" "SnapToTarget" "SnapToTarget" "KeepWorld" true))
    (:`then_1`
      (bind _returnvalue_3 (`|SpawnActorFromClass` "/Game/BluePrint/Players/BP_PlayerRightHands.BP_PlayerRightHands_C" _returnvalue "AlwaysSpawn" "OverrideRootScale" self "Left" false null))
      (bind _output_get_2 (set `self.LeftHand` _returnvalue_3))
      (`self.K2_AttachToComponent` (`self.LeftHand`) _vrorigin "None" "SnapToTarget" "SnapToTarget" "KeepWorld" true)
      (`self.K2_AttachToComponent` _output_get_2 _vrorigin "None" "SnapToTarget" "SnapToTarget" "KeepWorld" true))))

(event `Key|MotionController_Left_Grip1`
  (params (Key :type "Key Structure"))
  ;[1 1 1] TestNewHands
)

(event `self.ReceiveBeginPlay`
  ;[1 1 1] Begin PLay
  (`PrimitiveComponent.SetOwnerNoSee` (`self.HeadSet`) true)
  (`PrimitiveComponent.SetOwnerNoSee` (`self.playerHead`) true)
  (`SceneComponent.SetVisibility` (`self.MenuScreen`) false false)
  (bind _asai_character (cast `AI_Character` (`self.GetOwner`)))
  (set `self.AI_Var` _asai_character)
  (cast `/Game/BluePrint/Players/BP_VillianPlayer` (`GameplayStatics.GetPlayerCharacter` 1))
  (`HeadMountedDisplayFunctionLibrary.SetClippingPlanes` -100.0 20000.0)
  (`self.NewHandsSpawn`))

(event `HammerGrab`
  ;[1 1 1] Hammer Grab
  (if (`self.HoldingRifle`)
    (if (`self.RifleHolstered`)
      (if (`PrimitiveComponent.IsOverlappingComponent` (`self.RightHandCol`) (`self.HammerCollisionHolster`)) :!label _label
        (if (`self.HoldingHammer`)
          (`SceneComponent.K2_AttachToComponent` (`self.HammerAsset`) (`self.HammerHolster`) "None" "SnapToTarget" "SnapToTarget" "KeepWorld" true)
          (set `self.HoldingHammer` false)
          (else
            (`SceneComponent.K2_AttachToComponent` (`self.HammerAsset`) (`self.HammerInHand`) "None" "SnapToTarget" "SnapToTarget" "KeepWorld" true)
            (set `self.HoldingHammer` true)))))
    (else
      (goto _label))))

(event `RumbleController`
  (params (Scale :type "Float (double-precision)") (Hand :type "EControllerHand Enum" :default "Left"))
  ;[1 1 1] Handles rumble
  (`PlayerController.PlayHapticEffect` (`GameplayStatics.GetPlayerController` 0) "/Game/BluePrint/Players/MotionControllerHaptic.MotionControllerHaptic" Hand Scale false))

(event `HammerHit`
  (params (Hit :type "HitResult Structure"))
  (bind (_bblockinghit _binitialoverlap _time _distance _location _impactpoint _normal _impactnormal _physmat _hitactor) (`GameplayStatics.BreakHitResult` Hit))
  ;[1 0.08141 0.05157] Hammer hit
  (if (!= _hitactor self)
    (set `self.CanHit` false)
    (`GameplayStatics.ApplyDamage` _hitactor 1.0 null self)
    (`GameplayStatics.PlaySoundAtLocation` "/Game/Audio/HammerAudio/Hammer_Cue.Hammer_Cue" _location)
    (`KismetSystemLibrary.Delay` 0.2)
    (set `self.CanHit` true)))

(event `UpdateTrapLocation`
  (bind _rifleinhand (`self.RifleInHand`))
  (bind _returnvalue (`SceneComponent.K2_GetComponentLocation` _rifleinhand))
  ;[1 1 1] Updates trap location
  (if (`self.HasTrap`)
    (set `self.CanPLace` true)
    (`/Engine/EditorBlueprintResources/StandardMacros.Gate` true :!via `Open` :!label _label_2
      (:`Exit`
        (bind _outhit (`KismetSystemLibrary.LineTraceSingle` _returnvalue (+ (* (`SceneComponent.GetForwardVector` _rifleinhand) 10000.0) _returnvalue) "TraceTypeQuery1"))
        (bind (_bblockinghit _binitialoverlap _time _distance _location _impactpoint _normal _impactnormal _physmat _hitactor) (`GameplayStatics.BreakHitResult` _outhit))
        (if (`self.ActorHasTag` _hitactor "Floor")
          (`self.K2_SetActorLocation` (`self.Trap`) _location false false))))))

(event `Place Trap`
  ;[1 1 1] Lets go and places trap
  (if (and (`self.HasTrap`) (`self.CanPLace`))
    (set `self.HasTrap` false)
    (set `self.Has been Place` true)
    (set `/Game/BluePrint/BuildingTraps/MasterTrap.HasBeenPlace` true (`self.Trap`))
    (set `self.CanPLace` false)
    (set `self.Trap` null)
    (goto _label_2 :!via `Close`)))

(event `Key|MotionController_Right_Trigger` :paused true
  (params (Key :type "Key Structure"))
  (bind _widgetinteraction (`self.WidgetInteraction`))
  ;[1 1 1] Widget interaction
  (:`Pressed`
    (`WidgetInteractionComponent.PressPointerKey` _widgetinteraction "LeftMouseButton"))
  (:`Released`
    (`WidgetInteractionComponent.ReleasePointerKey` _widgetinteraction "LeftMouseButton")))

(event `self.ReceiveTick`
  (params (DeltaSeconds :type "Float (single-precision)"))
  (bind _vrcamera (`self.VRCamera`))
  (bind (_returnvalue_roll _returnvalue_pitch _returnvalue_yaw) (`KismetMathLibrary.BreakRotator` (`SceneComponent.K2_GetComponentRotation` _vrcamera)))
  (bind _returnvalue (`SceneComponent.GetSocketLocation` (`self.HammerHead`) "None"))
  ;[1 1 1] tick
  (`|ExecutionSequence`
    (:`then_0`
      ;;[1 0.3333 0.3432] Belt Tracking
      (`SceneComponent.K2_SetWorldLocationAndRotation` (`self.VRBodyScene`) (`SceneComponent.K2_GetComponentLocation` _vrcamera) (`KismetMathLibrary.MakeRotator` 0.0 0.0 _returnvalue_yaw) false false))
    (:`then_1`
      (set `self.DeltaSecondsVar` DeltaSeconds))
    (:`then_2`
      ;;[0.09561 0.1374 1] Scrap Counter
      (`TextRenderComponent.K2_SetText` (`self.ScrapCounter`) (`KismetTextLibrary.Conv_StringToText` (`KismetStringLibrary.Conv_IntToString` (`self.ScrapInt`)))))
    (:`then_3`
      ;[0.2926 0.8393 1] Hammer tracing
      (if (`self.HoldingHammer`)
        (if (`self.CanHit`)
          (bind (_outhit _returnvalue_2) (`KismetSystemLibrary.LineTraceSingle` _returnvalue (`self.HammerColLock`) "TraceTypeQuery1"))
          (if _returnvalue_2
            (`self.HammerHit` _outhit)))))
    (:`then_4`
      (set `self.HammerColLock` _returnvalue))))

(event `Key|MotionController_Left_Grip1`
  (params (Key :type "Key Structure"))
  ;[1 1 1] Lets player hold the gun in both hands
)

(event `CheckTrap`
  (bind _rifleinhand (`self.RifleInHand`))
  (bind _returnvalue (`SceneComponent.K2_GetComponentLocation` _rifleinhand))
  ;[1 1 1] Checks for the trap
  (if (not (`self.HoldingHammer`))
    (bind _outhit (`KismetSystemLibrary.LineTraceSingle` _returnvalue (+ (* (`SceneComponent.GetForwardVector` _rifleinhand) 10000.0) _returnvalue) "TraceTypeQuery1"))
    (bind _asmaster_trap (cast `/Game/BluePrint/BuildingTraps/MasterTrap` (`.HitActor` (`GameplayStatics.BreakHitResult` _outhit))))
    (set `self.Trap` _asmaster_trap)
    (set `self.HasTrap` true)))

(event `Key|MotionController_Right_Shoulder`
  (params (Key :type "Key Structure"))
  (bind _overlappingactors (`self.GetOverlappingActors` "/Game/BluePrint/Weapons/Rifles/BP_RifleWeaponsMaster.BP_RifleWeaponsMaster_C"))
  (bind _currentpuzzlepiece (`self.CurrentPuzzlePiece`))
  ;[1 1 1] Drop
  (:`Pressed`
    (if (`self.HoldingRifle`)
      (message `/Game/BluePrint/Weapons/BP_WeaponInteractions.GrabHolsteredGun` _overlappingactors)
      (if (not (`PrimitiveComponent.IsOverlappingComponent` (`self.RightHandCol`) (`self.RifleHolsterCol`)))
        ;[1 1 1] Deletes weapon(add in scad plus)
        (message `/Game/BluePrint/Weapons/BP_WeaponInteractions.Drop` _overlappingactors)
        (set `self.Hand Grips` "NewEnumerator0")
        (set `self.HoldingRifle` false))
      (elif (`self.HasPuzzlePiece`)
        (`PrimitiveComponent.SetSimulatePhysics` (`/Game/BluePrint/RadioTower/PuzzlePieces_Master.PuzzleMesh` _currentpuzzlepiece) true)
        (set `self.HasPuzzlePiece` false)
        (`PrimitiveComponent.SetCollisionResponseToChannel` (`/Game/BluePrint/RadioTower/PuzzlePieces_Master.Box` _currentpuzzlepiece) "ECC_Visibility" "ECR_Block")
        (`PrimitiveComponent.SetCollisionResponseToChannel` (`/Game/BluePrint/RadioTower/PuzzlePieces_Master.GrabCol` _currentpuzzlepiece) "ECC_Visibility" "ECR_Block")))))

(event `Key|MotionController_Left_Trigger`
  (params (Key :type "Key Structure"))
  ;[1 1 1] TurretSystemold
)

(event `PuzzlePieceGrab`
  (bind _widgetinteraction (`self.WidgetInteraction`))
  (bind _returnvalue (`SceneComponent.K2_GetComponentLocation` _widgetinteraction))
  ;[1 1 1] puzzle piece grab
  (if (or (`self.HasTrap`) (`self.HoldingHammer`) (`self.HasPuzzlePiece`))
    _
    (elif (`self.HoldingRifle`)
      (if (`self.RifleHolstered`)
        (bind _outhit (`KismetSystemLibrary.LineTraceSingle` _returnvalue (+ (* (`SceneComponent.GetForwardVector` _widgetinteraction) 100000.0) _returnvalue) "TraceTypeQuery1" :!label _label_3))
        (bind (_bblockinghit _binitialoverlap _time _distance _location _impactpoint _normal _impactnormal _physmat _hitactor _hitcomponent) (`GameplayStatics.BreakHitResult` _outhit))
        (if (`SceneComponent.IsSimulatingPhysics` _hitcomponent "None")
          (bind _aspuzzle_pieces_master (cast `/Game/BluePrint/RadioTower/PuzzlePieces_Master` _hitactor))
          (set `self.CurrentPuzzlePiece` _aspuzzle_pieces_master)
          (`PrimitiveComponent.SetSimulatePhysics` (`/Game/BluePrint/RadioTower/PuzzlePieces_Master.PuzzleMesh` _aspuzzle_pieces_master) false)
          (`self.K2_AttachToComponent` _aspuzzle_pieces_master (`self.GrabLoc`) "None" "SnapToTarget" "SnapToTarget" "KeepWorld" false)
          (set `self.HasPuzzlePiece` true)
          (`PrimitiveComponent.SetCollisionResponseToChannel` (`/Game/BluePrint/RadioTower/PuzzlePieces_Master.Box` _aspuzzle_pieces_master) "ECC_Visibility" "ECR_Ignore")
          (`PrimitiveComponent.SetCollisionResponseToChannel` (`/Game/BluePrint/RadioTower/PuzzlePieces_Master.GrabCol` _aspuzzle_pieces_master) "ECC_Visibility" "ECR_Ignore")
          (else
            (bind _aspuzzle_pieces_master_2 (cast `/Game/BluePrint/RadioTower/PuzzlePieces_Master` _hitactor))
            (bind _output_get (set `self.CurrentPuzzlePiece` _aspuzzle_pieces_master_2))
            (`self.K2_AttachToComponent` _aspuzzle_pieces_master_2 (`self.GrabLoc`) "None" "SnapToTarget" "SnapToTarget" "KeepWorld" false)
            (`PrimitiveComponent.SetCollisionResponseToChannel` (`/Game/BluePrint/RadioTower/PuzzlePieces_Master.Box` _output_get) "ECC_Visibility" "ECR_Ignore")
            (`PrimitiveComponent.SetCollisionResponseToChannel` (`/Game/BluePrint/RadioTower/PuzzlePieces_Master.GrabCol` _output_get) "ECC_Visibility" "ECR_Ignore")
            (set `self.HasPuzzlePiece` true)
            (`SceneComponent.SetVisibility` (`/Game/BluePrint/RadioTower/PuzzlePieces_Master.Gear` _output_get) false false))))
      (else
        (goto _label_3)))))

(event `Key|MotionController_Right_Trigger`
  (params (Key :type "Key Structure"))
  (bind _overlappingactors (`self.GetOverlappingActors` "/Game/BluePrint/Weapons/Rifles/BP_RifleWeaponsMaster.BP_RifleWeaponsMaster_C"))
  ;[1 1 1] Right trigger
  (:`Pressed`
    ;;[1 1 1] Checks if holding puzzle piece
    (if (`self.HasPuzzlePiece`)
      (`self.Teleport System`)
      (else
        ;;[1 1 1] Checks if holding rifle
        (if (`self.RifleHolstered`)
          (`|ExecutionSequence`
            (:`then_0`
              (`self.PuzzlePieceGrab` :!label _label_4))
            (:`then_1`
              (`self.HammerGrab` :!label _label_5))
            (:`then_2`
              (`self.Teleport System` :!label _label_6))
            (:`then_3`
              (`self.UpdateTrapLocation` :!label _label_7))
            (:`then_4`
              (`self.CheckTrap` :!label _label_8))
            (:`then_5`
              (if (`PrimitiveComponent.IsOverlappingComponent` (`self.RightHandCol`) (`self.RifleHolsterCol`))
                (message `/Game/BluePrint/Weapons/BP_WeaponInteractions.GrabGun` _overlappingactors null :!label _label_9) ; Grab gun
                (if (`self.HoldingRifle`)
                  (set `self.RifleHolstered` false)
                  (set `self.Hand Grips` "NewEnumerator1")
                  (set `WidgetInteractionComponent.bShowDebug` false (`self.WidgetInteraction`))
                  (if (`self.TutorialLevel`)
                    (set `self.Start theGame` true))))))
          (else
            (`|ExecutionSequence`
              (:`then_0`
                (if (`self.HoldingRifle`)
                  (message `/Game/BluePrint/Weapons/BP_WeaponInteractions.FireWeapon` _overlappingactors) ; Fires gun
                ))
              (:`then_1`
                (goto _label_5))
              (:`then_2`
                (goto _label_6))
              (:`then_3`
                (goto _label_7))
              (:`then_4`
                (goto _label_8))
              (:`then_5`
                (goto _label_9))
              (:`then_6`
                (goto _label_4))))))))
  (:`Released`
    (`|ExecutionSequence`
      (:`then_0`
        (`self.Place Trap`))
      (:`then_1`
        (message `/Game/BluePrint/Weapons/BP_WeaponInteractions.StopFiring` _overlappingactors) ; stop firing
      ))))

(event `Teleport System`
  (bind _widgetinteraction (`self.WidgetInteraction`))
  (bind _returnvalue (`SceneComponent.K2_GetComponentLocation` _widgetinteraction))
  ;[1 1 1] Teleport system
  (bind _outhit (`KismetSystemLibrary.LineTraceSingle` _returnvalue (+ (* (`SceneComponent.GetForwardVector` _widgetinteraction) 100000.0) (+ _returnvalue 1000.0)) "TraceTypeQuery1"))
  (`|ExecutionSequence`
    (:`then_0`
      (bind (_bblockinghit _binitialoverlap _time _distance _location _impactpoint _normal _impactnormal _physmat _hitactor) (`GameplayStatics.BreakHitResult` _outhit))
      (bind _asteleport_area (cast `/Game/BluePrint/RadioTower/TeleportArea` _hitactor))
      (`self.K2_SetActorLocation` (`/Game/BluePrint/RadioTower/TeleportArea.WorldLocatino` _asteleport_area) false true))
    (:`then_1`
      (bind _asvan (cast `/Game/BluePrint/VanAndPups/Van` _hitactor))
      (if (`/Game/BluePrint/VanAndPups/Van.CanTele` _asvan)
        (`self.K2_SetActorLocation` (`/Game/BluePrint/VanAndPups/Van.PlyWorldLoc` _asvan) false true)))))

(event `Key|MotionController_Left_Trigger`
  (params (Key :type "Key Structure"))
  (bind _overlappingactors (`self.GetOverlappingActors` "/Game/BluePrint/Weapons/Rifles/BP_RifleWeaponsMaster.BP_RifleWeaponsMaster_C"))
  ;[1 1 1] Reload and dropping ammo
  (:`Pressed`
    (`|ExecutionSequence`
      (:`then_0`
        (message `/Game/BluePrint/Weapons/BP_WeaponInteractions.Pump` _overlappingactors))
      (:`then_1`
        (if (`PrimitiveComponent.IsOverlappingComponent` (`self.AmmoPouchCol`) (`self.LeftHandCol`))
          (message `/Game/BluePrint/Weapons/BP_WeaponInteractions.Ammo` _overlappingactors)
          (`self.RumbleController` 0.5 "Left")))))
  (:`Released`
    (message `/Game/BluePrint/Weapons/BP_WeaponInteractions.StopPump` _overlappingactors)
    (set `self.InteractingWEapon` false)
    (if (`self.HoldingAmmo`)
      (message `/Game/BluePrint/Weapons/BP_WeaponInteractions.DropAmmo` _overlappingactors))))

(event `InputAction|RightReload`
  (params (Key :type "Key Structure"))
  ;[1 1 1] Special Fire
  (:`Pressed`
    (if (`self.HoldingRifle`)
      (if (`self.FingerGun?`)
        (`/Game/BluePrint/Weapons/Rifles/BP_FingerGun.DropTheHand` (`self.FingerGun`))
        (set `self.FingerGun?` false)
        (set `self.HoldingRifle` false)
        (set `self.Hand Grips` "NewEnumerator0")
        (else
          (message `/Game/BluePrint/Weapons/BP_WeaponInteractions.SwitchFireRate` (`self.GetOverlappingActors` "/Game/BluePrint/Weapons/Rifles/BP_RifleWeaponsMaster.BP_RifleWeaponsMaster_C"))))
      (else
        (bind _returnvalue (`|SpawnActorFromClass` "/Game/BluePrint/Weapons/Rifles/BP_FingerGun.BP_FingerGun_C" (`SceneComponent.K2_GetComponentToWorld` (`self.RightMC`)) "Undefined" "OverrideRootScale" null null))
        (bind _output_get (set `self.FingerGun` _returnvalue))
        (`/Game/BluePrint/Weapons/Rifles/BP_RifleWeaponsMaster.AttachToHand` _output_get)
        (set `self.FingerGun?` true)
        (set `self.Hand Grips` "NewEnumerator3")))))

(event `Hit`
  (bind _halfsphere (`self.halfSphere`))
  ;[1 1 1] Tomatoe headshot
  (`SceneComponent.SetHiddenInGame` _halfsphere false false)
  (`PrimitiveComponent.SetOnlyOwnerSee` (`self.halfSphere`) true)
  (`KismetSystemLibrary.Delay` 5.0)
  (`SceneComponent.SetHiddenInGame` _halfsphere true false))

(event `InputAxis|EnemyMoveForward`
  (params (AxisValue :type "Float (single-precision)"))
  ;[1 0.1719 0.1719] Enemy Controls
  ;;[1 1 1] Enemy movement
  (bind _asbp_villian_player (cast `/Game/BluePrint/Players/BP_VillianPlayer` (`GameplayStatics.GetPlayerPawn` 1)))
  (`self.AddMovementInput` _asbp_villian_player (`KismetMathLibrary.GetForwardVector` (`self.GetControlRotation` _asbp_villian_player)) AxisValue false))

(event `InputAction|EnemyAttack`
  (params (Key :type "Key Structure"))
  ;[1 0.1719 0.1719] Enemy Controls
  ;;[1 1 1] EnemyAttacking
  (:`Pressed`
    (bind _asbp_villian_player (cast `/Game/BluePrint/Players/BP_VillianPlayer` (`GameplayStatics.GetPlayerPawn` 1)))
    (if (`/Game/BluePrint/Players/BP_VillianPlayer.IsAiming` _asbp_villian_player)
      (`/Game/BluePrint/Players/BP_VillianPlayer.GunAttack` _asbp_villian_player)
      (else
        (set `/Game/BluePrint/Players/BP_VillianPlayer.IsAttacking` true _asbp_villian_player)
        (`/Engine/EditorBlueprintResources/StandardMacros.Gate` true :!via `Open` :!label _label_10
          (:`Exit`
            (`KismetSystemLibrary.Delay` 0.8)
            (`/Game/BluePrint/Players/BP_VillianPlayer.MeleeAttack` _asbp_villian_player))))))
  (:`Released`
    (bind _asbp_villian_player_2 (cast `/Game/BluePrint/Players/BP_VillianPlayer` (`GameplayStatics.GetPlayerPawn` 1)))
    (set `/Game/BluePrint/Players/BP_VillianPlayer.IsAttacking` false _asbp_villian_player_2)
    (goto _label_10 :!via `Close`)))

(event `InputAxis|EnemyMoveRight`
  (params (AxisValue :type "Float (single-precision)"))
  ;[1 0.1719 0.1719] Enemy Controls
  ;;[1 1 1] Enemy movement
  (bind _asbp_villian_player (cast `/Game/BluePrint/Players/BP_VillianPlayer` (`GameplayStatics.GetPlayerPawn` 1)))
  (`self.AddMovementInput` _asbp_villian_player (`KismetMathLibrary.GetRightVector` (`self.GetControlRotation` _asbp_villian_player)) AxisValue false))

(event `InputAxis|TurnRate`
  (params (AxisValue :type "Float (single-precision)"))
  ;[1 0.1719 0.1719] Enemy Controls
  ;;[1 1 1] Enemy looking
  (bind _asbp_villian_player (cast `/Game/BluePrint/Players/BP_VillianPlayer` (`GameplayStatics.GetPlayerPawn` 1)))
  (`self.AddControllerYawInput` _asbp_villian_player (* AxisValue (`/Game/BluePrint/Players/BP_VillianPlayer.BaseTurnRate` _asbp_villian_player) (`GameplayStatics.GetWorldDeltaSeconds`))))

(event `Key|Gamepad_LeftTrigger`
  (params (Key :type "Key Structure"))
  (bind _returnvalue (`GameplayStatics.GetPlayerPawn` 1))
  ;[1 0.1719 0.1719] Enemy Controls
  (:`Pressed`
    (bind _asbp_villian_player (cast `/Game/BluePrint/Players/BP_VillianPlayer` _returnvalue))
    (`/Game/BluePrint/Players/BP_VillianPlayer.SetAiming` _asbp_villian_player))
  (:`Released`
    (bind _asbp_villian_player_2 (cast `/Game/BluePrint/Players/BP_VillianPlayer` _returnvalue))
    (`/Game/BluePrint/Players/BP_VillianPlayer.NotAiming` _asbp_villian_player_2)))

(event `InputAxis|LookUpRate`
  (params (AxisValue :type "Float (single-precision)"))
  ;[1 0.1719 0.1719] Enemy Controls
  ;;[1 1 1] Enemy looking
  (bind _asbp_villian_player (cast `/Game/BluePrint/Players/BP_VillianPlayer` (`GameplayStatics.GetPlayerPawn` 1)))
  (`self.AddControllerPitchInput` _asbp_villian_player (* AxisValue (`/Game/BluePrint/Players/BP_VillianPlayer.BaseLookUpRate` _asbp_villian_player) (`GameplayStatics.GetWorldDeltaSeconds`))))

(event `Key|Gamepad_FaceButton_Left`
  (params (Key :type "Key Structure"))
  ;[1 0.1719 0.1719] Enemy Controls
  (:`Pressed`
    (bind _asbp_villian_player (cast `/Game/BluePrint/Players/BP_VillianPlayer` (`GameplayStatics.GetPlayerPawn` 1)))
    (`/Game/BluePrint/Players/BP_VillianPlayer.Reload` _asbp_villian_player)))

(fn `GrabGun`
  (params (HandInput :type "/Game/BluePrint/Players/BP_PlayerRightHands Object Reference"))
  (returns (Ammo :type "Actor Class Reference") (CurrentWeapon :type "/Game/BluePrint/Weapons/Rifles/BP_RifleWeaponsMaster Object Reference"))
  (return null null))

(fn `UserConstructionScript`
  (`SceneComponent.SetHiddenInGame` (`self.ScrapCounter`) false false))