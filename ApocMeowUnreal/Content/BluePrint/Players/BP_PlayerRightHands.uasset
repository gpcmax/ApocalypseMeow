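; VR motion-controller hand actor that grabs, fires and reloads rifles, animates hand grips and clicks in-game widgets.
; Tick gathers overlapping rifles, which trigger pulls message to fire and grab, passing grabbed ammo to the TestNewHandCh player character.
; It also spawns reload ammo on pouch overlap, plays haptic rumble and mirrors the hand mesh per side.
; Hammer, teleport, trap and puzzle-piece events are empty stubs.
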(event `CloseHand`
  (if (not (`self.HoldingWeapon`))
    (set `self.HandGrips` "NewEnumerator0")))

(event `RumbleController`
  (params (Scale :type "Float (double-precision)") (Hand :type "EControllerHand Enum" :default "Left"))
  ;[1 1 1] Motion controller rumble
  (`PlayerController.PlayHapticEffect` (`GameplayStatics.GetPlayerController` 0) "/Game/BluePrint/Players/MotionControllerHaptic.MotionControllerHaptic" Hand 1.0 false))

(event `/Game/BluePrint/Interface/BP_HandInterface.Hand_Trigger`
  ;[1 1 1] Allows user to interact with in game menus
  (`WidgetInteractionComponent.PressPointerKey` (`self.WidgetInteraction`) "LeftMouseButton"))

(event `/Game/BluePrint/Interface/BP_HandInterface.Hand_TriggerRelease`
  ;[1 1 1] Allows user to interact with in game menus
  (`WidgetInteractionComponent.ReleasePointerKey` (`self.WidgetInteraction`) "LeftMouseButton"))

(event `OpenHand`
  ;[1 1 1] Open close hand
  (set `self.HandGrips` "NewEnumerator1"))

(event `self.ReceiveTick`
  (params (DeltaSeconds :type "Float (single-precision)"))
  ;[1 1 1] Tick
  (set `self.WeaponArray` (`self.GetOverlappingActors` "/Game/BluePrint/Weapons/Rifles/BP_RifleWeaponsMaster.BP_RifleWeaponsMaster_C")))

(event `TriggerPull1`
  (params (`Hand Input` :type "/Game/BluePrint/Players/BP_PlayerRightHands Object Reference"))
  (set `self.HandInput` `Hand Input`)
  (if (not (`self.HasPuzzlePiece`))
    (if (`self.HoldingWeapon`)
      (`self.CloseHand`)
      (else
        (`self.OpenHand`)))
    (`|ExecutionSequence`
      (:`then_0`
        (message `/Game/BluePrint/Weapons/BP_WeaponInteractions.FireWeapon` (`self.WeaponArray`)))
      (:`then_1`
        (bind _ammo (message `/Game/BluePrint/Weapons/BP_WeaponInteractions.GrabGun` (`self.WeaponArray`) (`self.HandInput`))) ; Grab gun
        (set `/Game/BluePrint/Players/TestNewHandCh.Ammo to grab` _ammo (`self.TestChar`))
        (set `self.HoldingWeapon` true)))))

(event `HammerGrab`
  ;[1 1 1] Hammer Grab
)

(event `Teleport`
  ;[1 1 1] Teleport
)

(event `GrabAmmo`)

(event `UpdateTrapLocation`
  ;[1 1 1] UpdateTrapLocation
)

(event `CheckTrap`
  ;[1 1 1] CheckTrap
)

(event `ReloadGrab`
  (params (Hand :type "/Game/BluePrint/Players/BP_PlayerRightHands Object Reference") (Ammo :type "Actor Class Reference") (AmmoPack :type "/Game/BluePrint/Players/BP_AmmoSpawn Object Reference"))
  (bind _weapon (`/Game/BluePrint/Players/TestNewHandCh.Weapon` (`self.TestChar`)))
  (if (`PrimitiveComponent.IsOverlappingComponent` (`/Game/BluePrint/Players/BP_PlayerRightHands.HandCol` Hand) (`/Game/BluePrint/Players/BP_AmmoSpawn.AmmoCol` AmmoPack))
    (`/Game/BluePrint/Weapons/Rifles/BP_RifleWeaponsMaster.SpawnAndGrabAmmo` _weapon (`/Game/BluePrint/Weapons/Rifles/BP_RifleWeaponsMaster.AmmoTypeVar` _weapon) Hand)))

(event `PuzzlePieceGrab`
  ;[1 1 1] PuzzlePieceGrab
)

(event `EmptyGun`
  (message `/Game/BluePrint/Weapons/BP_WeaponInteractions.ReloadWeapon` (`self.WeaponArray`)))

(event `self.ReceiveBeginPlay`
  (bind _astest_new_hand_ch (cast `/Game/BluePrint/Players/TestNewHandCh` (`GameplayStatics.GetPlayerCharacter` 0)))
  (set `self.TestChar` _astest_new_hand_ch))

(fn `Ammo`
  (return))

(fn `GrabGun`
  (params (HandInput :type "/Game/BluePrint/Players/BP_PlayerRightHands Object Reference"))
  (returns (Ammo :type "Actor Class Reference") (CurrentWeapon :type "/Game/BluePrint/Weapons/Rifles/BP_RifleWeaponsMaster Object Reference"))
  (return null null))

(fn `TriggerPull`
  (params (HandInput :type "/Game/BluePrint/Players/BP_PlayerRightHands Object Reference"))
  (returns (Ammo :type "Actor Class Reference") (CurrentWeapon :type "/Game/BluePrint/Weapons/Rifles/BP_RifleWeaponsMaster Object Reference"))
  (set `self.HandInput` HandInput)
  (if (not (`self.HasPuzzlePiece`))
    (if (`self.HoldingWeapon`)
      (`self.CloseHand`)
      (else
        (`self.OpenHand`)))
    (`|ExecutionSequence`
      (:`then_0`
        (message `/Game/BluePrint/Weapons/BP_WeaponInteractions.FireWeapon` (`self.WeaponArray`)))
      (:`then_1`
        (bind (_ammo _currentweapon) (message `/Game/BluePrint/Weapons/BP_WeaponInteractions.GrabGun` (`self.WeaponArray`) (`self.HandInput`))) ; Grab gun
        (set `/Game/BluePrint/Players/TestNewHandCh.Ammo to grab` _ammo (`self.TestChar`))
        (set `self.HoldingWeapon` true)
        (return _ammo _currentweapon)))))

(fn `UserConstructionScript`
  (bind _textrender (`self.TextRender`))
  (set `MotionControllerComponent.Hand` (`self.Hand`) (`self.MotionController`))
  (if (`|EnumEquality` (`self.Hand`) "Right")
    (`SceneComponent.SetVisibility` _textrender true false)
    (switch `EControllerHand` (`self.Hand`)
      (:`Right`
        (`SceneComponent.SetWorldScale3D` (`self.HandMesh`) (1.0 -1.0 1.0))))
    (else
      (`SceneComponent.SetVisibility` _textrender false false)
      (switch `EControllerHand` (`self.Hand`)
        (:`Left`
          (`SceneComponent.SetWorldScale3D` (`self.HandMesh`) (1.0 1.0 1.0)))))))