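; BP_AmmoSpawn is an ammo supply point that hands ammo to the player through an overlap trigger, AmmoCol.
; When the right hand overlaps with no valid CurrentAmmo, it sends AmmoMessage to the player's weapon with that hand and AmmoToGrab, storing the result as CurrentAmmo.
; Other overlapping actors receive ReloadHipMessage with the player and this box.
; The Ammo and GrabGun functions are empty stubs.
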(event `self.AmmoCol.OnComponentBeginOverlap`
  (params (OverlappedComponent :type "PrimitiveComponent Object Reference") (OtherActor :type "Actor Object Reference") (OtherComp :type "PrimitiveComponent Object Reference") (OtherBodyIndex :type Integer) (bFromSweep :type Boolean) (SweepResult :type "HitResult Structure (by ref)"))
  (bind _astest_new_hand_ch (cast `/Game/BluePrint/Players/TestNewHandCh` (`GameplayStatics.GetPlayerCharacter` 0) :!pure true))
  (if (== OtherActor "/Game/BluePrint/Players/BP_PlayerRightHands.BP_PlayerRightHands")
    (`/Engine/EditorBlueprintResources/StandardMacros.IsValid` (`self.CurrentAmmo`)
      (:`Is Not Valid`
        (bind _asbp_player_right_hands (cast `/Game/BluePrint/Players/BP_PlayerRightHands` OtherActor))
        (bind _getammocurrent (message `/Game/BluePrint/Weapons/BP_WeaponInteractions.Ammo` (`/Game/BluePrint/Players/TestNewHandCh.Weapon` _astest_new_hand_ch) _asbp_player_right_hands (`/Game/BluePrint/Players/TestNewHandCh.Ammo to grab` _astest_new_hand_ch)))
        (set `self.CurrentAmmo` _getammocurrent)))
    (else
      (message `/Game/BluePrint/Weapons/BP_WeaponInteractions.ReloadHip` OtherActor null _astest_new_hand_ch self))))

(fn `Ammo`
  (return))

(fn `GrabGun`
  (params (HandInput :type "/Game/BluePrint/Players/BP_PlayerRightHands Object Reference"))
  (returns (Ammo :type "Actor Class Reference") (CurrentWeapon :type "/Game/BluePrint/Weapons/Rifles/BP_RifleWeaponsMaster Object Reference"))
  (return null null))

(fn `UserConstructionScript`)