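; Health component that tracks hit points for its owning actor and reacts to incoming damage.
; On BeginPlay it binds to the owner's OnTakeAnyDamage and forwards the damage amount to TakeDamage.
; TakeDamage subtracts from Health, clamped at zero, and destroys the owner at zero unless the IsVan flag is set.
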(event `self.ReceiveBeginPlay`
  (add `Actor.OnTakeAnyDamage` (`self.GetOwner`) (delegate `CustomEvent_0`)))

(event `CustomEvent_0`
  (params (DamagedActor :type "Actor Object Reference") (Damage :type "Float (double-precision)") (DamageType :type "DamageType Object Reference") (InstigatedBy :type "Controller Object Reference") (DamageCauser :type "Actor Object Reference"))
  (`self.TakeDamage` Damage))

(event `TakeDamage`
  (params (DamageDealt :type "Float (double-precision)"))
  (bind _output_get (set `self.Health` (`KismetMathLibrary.FClamp` (- (`self.Health`) DamageDealt) 0.0 1000000000000.0)))
  (if (<= _output_get 0.0)
    (if (not (`self.IsVan?`))
      (`Actor.K2_DestroyActor` (`self.GetOwner`)))))