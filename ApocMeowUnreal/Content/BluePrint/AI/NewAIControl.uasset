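; AI controller for BP_AI_Character that feeds the BB_ShooterDefender blackboard and deals automatic area damage.
; Tick scans every frame for the nearest "Threat" actor within aggro range and for fallen pets, also writing van location, spawn location and pet-holding state.
; From BeginPlay or Attack, a looping timer applies radial damage around the pawn, sparing "Villian"-tagged actors and setting Attacking on hits, until StopAttacking.
; ChangeSpeed sets the pawn's walk speed.
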(event `self.OnPossess`
  (params (PossessedPawn :type "Pawn Object Reference"))
  (`self.UseBlackboard` "/Game/BluePrint/AI/BB_ShooterDefender.BB_ShooterDefender"))

(event `Attack`
  (bind _returnvalue (`KismetSystemLibrary.K2_SetTimerDelegate` (delegate `CustomEvent_0`) 0.25 true :!label _label)))

(event `self.ReceiveBeginPlay`
  (goto _label))

(event `CustomEvent_0`
  (bind _outactors (`GameplayStatics.GetAllActorsWithTag` "Villian"))
  (bind _returnvalue (`GameplayStatics.ApplyRadialDamage` 5.0 (`self.K2_GetActorLocation` (`self.K2_GetPawn`)) 200.0 null _outactors null null true))
  (if _returnvalue
    (set `self.Attacking` true)
    (else
      (set `self.Attacking` false))))

(event `StopAttacking`
  (`KismetSystemLibrary.K2_ClearAndInvalidateTimerHandle` (stale `Attack` _returnvalue))
  (set `self.Attacking` false))

(event `self.ReceiveTick`
  (params (DeltaSeconds :type "Float (single-precision)"))
  (bind _threat (`self.Threat`))
  (bind _returnvalue (`AIBlueprintHelperLibrary.GetBlackboard` self))
  (bind _asbp_ai_character (cast `/Game/BluePrint/AI/BP_AI_Character` (`self.K2_GetPawn`) :!pure true))
  (`|ExecutionSequence`
    (:`then_0`
      (bind _outactors (`GameplayStatics.GetAllActorsWithTag` "Threat"))
      (bind _output_get (set `self.Threats` _outactors))
      (for _array_element _output_get
        (bind _returnvalue_2 (`self.GetDistanceTo` (`self.K2_GetPawn`) _array_element))
        (if (< _returnvalue_2 (`self.AggroRange`))
          (if (< _returnvalue_2 (`self.Lowest`))
            (set `self.Lowest` _returnvalue_2)
            (bind _output_get_2 (set `self.Threat` _array_element))
            (`BlackboardComponent.SetValueAsObject` (`AIBlueprintHelperLibrary.GetBlackboard` self) "Threat" _output_get_2))))
      (set `self.Lowest` 10000.0)
      (`/Engine/EditorBlueprintResources/StandardMacros.IsValid` _threat
        (:`Is Valid`
          (if (> (`self.GetDistanceTo` (`self.K2_GetPawn`) _threat) (`self.AggroRange`))
            (bind _output_get_3 (set `self.Threat` null :!label _label_2))
            (`BlackboardComponent.SetValueAsObject` (`AIBlueprintHelperLibrary.GetBlackboard` self) "Threat" _output_get_3)))
        (:`Is Not Valid`
          (goto _label_2))))
    (:`then_1`
      (bind _outactors_2 (`GameplayStatics.GetAllActorsOfClass` "/Game/BluePrint/VanAndPups/Pet_BP.Pet_BP_C"))
      (bind _output_get_4 (set `self.Pets` _outactors_2))
      (for _array_element_2 _output_get_4
        (if (`/Game/BluePrint/VanAndPups/Pet_BP.Fallen` _array_element_2)
          (bind _output_get_5 (set `self.Pet` _array_element_2))
          (`BlackboardComponent.SetValueAsObject` (`AIBlueprintHelperLibrary.GetBlackboard` self) "Pet" _output_get_5)
          (elif (== _array_element_2 (`self.Pet`))
            (bind _output_get_6 (set `self.Pet` null))
            (`BlackboardComponent.SetValueAsObject` (`AIBlueprintHelperLibrary.GetBlackboard` self) "Pet" _output_get_6)))))
    (:`then_2`
      (`BlackboardComponent.SetValueAsVector` _returnvalue "VanLoc" (0.0 0.0 0.0))
      (`BlackboardComponent.SetValueAsVector` _returnvalue "SpawnLoc" (`/Game/BluePrint/AI/BP_AI_Character.SpawnLoc` _asbp_ai_character))
      (`BlackboardComponent.SetValueAsBool` _returnvalue "HoldingPet" (`/Game/BluePrint/AI/BP_AI_Character.Holding` _asbp_ai_character)))))

(fn `ChangeSpeed`
  (params (Speed :type "Float (double-precision)"))
  (set `CharacterMovementComponent.MaxWalkSpeed` Speed (`Character.CharacterMovement` (cast `/Game/BluePrint/AI/BP_AI_Character` (`self.K2_GetPawn`) :!pure true))))

(fn `UserConstructionScript`)