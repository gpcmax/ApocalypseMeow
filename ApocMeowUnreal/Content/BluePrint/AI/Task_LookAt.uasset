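; Behavior tree task that turns a BP_AI_Character pawn to face the actor stored in the blackboard's Target key.
; Each AI tick computes the look-at rotation toward the target, interpolates toward it and applies only the yaw to the pawn.
; The task never calls Finish Execute, and a leftover AI_Shooter cast is never run.
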(event `self.ReceiveTickAI`
  (params (OwnerController :type "AIController Object Reference") (ControlledPawn :type "Pawn Object Reference") (DeltaSeconds :type "Float (single-precision)"))
  (bind _asbp_ai_character (cast `/Game/BluePrint/AI/BP_AI_Character` ControlledPawn))
  (bind (_returnvalue_roll _returnvalue_pitch _returnvalue_yaw) (`KismetMathLibrary.BreakRotator` (`KismetMathLibrary.RInterpTo` (`Actor.K2_GetActorRotation` _asbp_ai_character) (`KismetMathLibrary.FindLookAtRotation` (`Actor.K2_GetActorLocation` _asbp_ai_character) (`Actor.K2_GetActorLocation` (cast `Actor` (`BlackboardComponent.GetValueAsObject` (`AIBlueprintHelperLibrary.GetBlackboard` OwnerController) "Target") :!pure true))) DeltaSeconds 20.0)))
  (`Actor.K2_SetActorRotation` _asbp_ai_character (`KismetMathLibrary.MakeRotator` 0.0 0.0 _returnvalue_yaw) false))