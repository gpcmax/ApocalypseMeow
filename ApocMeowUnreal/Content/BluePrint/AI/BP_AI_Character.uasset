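; Enemy AI character that grabs the player's pet and awards scrap plus a random puzzle piece when destroyed.
; The construction script randomizes socketed armor, clothing, weapon and materials; armor adds MaxHealth, which BeginPlay resets.
; Tick handles ragdoll pet release and delayed death, and kills launched enemies on landing, raising their scrap reward if damaged midair.
; Overlapping a pet attaches it, stops attacking and destroys the enemy after a delay.
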(event `self.ReceiveBeginPlay`
  (set `self.MaxHealth` 50.0)
  (set `self.SpawnLoc` (`self.K2_GetActorLocation`)))

(event `self.ReceiveDestroyed`
  (bind _puzzlepieces (`self.PuzzlePieces`))
  (bind (_returnvalue_location _returnvalue_rotation) (`KismetMathLibrary.BreakTransform` (`SceneComponent.K2_GetComponentToWorld` (`self.ItemSpawner`))))
  (`|SpawnActorFromClass` (`|GetArrayItem` _puzzlepieces (`KismetMathLibrary.RandomIntegerInRange` 0 (`KismetArrayLibrary.Array_LastIndex` _puzzlepieces))) (`KismetMathLibrary.MakeTransform` _returnvalue_location _returnvalue_rotation (1.501737 1.501737 1.501737)) "Undefined" "OverrideRootScale" null null)
  (bind _asbp_vrchar_1 (cast `/Game/BluePrint/Players/BP_VRChar1` (`Controller.K2_GetPawn` (`GameplayStatics.GetPlayerController` 0)))
    (:`then`
      (set `/Game/BluePrint/Players/BP_VRChar1.ScrapInt` (+ (`/Game/BluePrint/Players/BP_VRChar1.ScrapInt` _asbp_vrchar_1) (`self.ScrapEarned`)) _asbp_vrchar_1))
    (:`CastFailed`
      (bind _asfirst_person_character (cast `/Game/FirstPersonBP/Blueprints/FirstPersonCharacter` (`Controller.K2_GetPawn` (`GameplayStatics.GetPlayerController` 0))))
      (set `/Game/FirstPersonBP/Blueprints/FirstPersonCharacter.Scrap` (+ (`/Game/FirstPersonBP/Blueprints/FirstPersonCharacter.Scrap` _asfirst_person_character) (`self.ScrapEarned`)) _asfirst_person_character)))
  (`GameplayStatics.PlaySound2D` "/Game/Audio/Scrap/clingclang2.clingclang2"))

(event `self.ReceiveTick`
  (params (DeltaSeconds :type "Float (single-precision)"))
  (bind _pet (`self.Pet`))
  (`|ExecutionSequence`
    (:`then_0`
      (if (`self.bRagDoll`)
        (`/Engine/EditorBlueprintResources/StandardMacros.IsValid` _pet
          (:`Is Valid`
            (`self.K2_DetachFromActor` _pet "KeepRelative" "KeepRelative" "KeepRelative")
            (`/Game/BluePrint/VanAndPups/Pet_BP.Dropped` _pet))
          (:`Is Not Valid`
            _))
        (`/Game/BluePrint/AI/NewAIControl.StopAttacking` (cast `/Game/BluePrint/AI/NewAIControl` (`self.GetController`) :!pure true))
        (`KismetSystemLibrary.Delay` 5.0)
        (`self.KillEnemies`)))
    (:`then_1`
      (if (and (not (`NavMovementComponent.IsFalling` (`self.CharacterMovement`))) (`self.Launched`))
        (`self.HurtAi` 10000.0)))
    (:`then_2`
      (if (`self.Launched`)
        (if (< (`/Game/BluePrint/AI/Health.Health` (`self.Health`)) (`self.OldHP`))
          (set `self.ScrapEarned` 60)
          (else
            (set `self.OldHP` (`/Game/BluePrint/AI/Health.Health` (`self.Health`)))))))))

(event `Launch`
  (bind _charactermovement (`self.CharacterMovement`))
  (`MovementComponent.StopMovementImmediately` (`self.CharacterMovement`))
  (set `/Game/BluePrint/AI/Health.Health` 1.0 (`self.Health`))
  (set `CharacterMovementComponent.GravityScale` 0.5 _charactermovement)
  (`CharacterMovementComponent.SetMovementMode` _charactermovement "MOVE_Falling" 0)
  (`self.LaunchCharacter` (0.0 0.0 1000.0) true true)
  (`CharacterMovementComponent.SetMovementMode` _charactermovement "MOVE_Falling" 0)
  (set `self.Launched` true)
  (set `self.ScrapEarned` 0))

(event `self.CapsuleComponent.OnComponentBeginOverlap`
  (params (OverlappedComponent :type "PrimitiveComponent Object Reference") (OtherActor :type "Actor Object Reference") (OtherComp :type "PrimitiveComponent Object Reference") (OtherBodyIndex :type Integer) (bFromSweep :type Boolean) (SweepResult :type "HitResult Structure (by ref)"))
  (bind _aspet_bp (cast `/Game/BluePrint/VanAndPups/Pet_BP` OtherActor :!pure true))
  (if (and (== (`GameplayStatics.GetObjectClass` OtherActor) "/Game/BluePrint/VanAndPups/Pet_BP.Pet_BP_C") (not (`self.Holding`)))
    (set `self.Pet` _aspet_bp)
    (`/Game/BluePrint/VanAndPups/Pet_BP.PickedUpByEnemy` _aspet_bp)
    (`self.K2_AttachToComponent` OtherActor (`self.Mesh`) "PupLoc" "SnapToTarget" "SnapToTarget" "KeepWorld" true)
    (set `self.Holding` true)
    (`/Game/BluePrint/AI/NewAIControl.StopAttacking` (cast `/Game/BluePrint/AI/NewAIControl` (`self.GetController`) :!pure true))
    (`KismetSystemLibrary.Delay` 75.0)
    (`self.K2_DestroyActor`)))

(fn `ArmorGenerator`
  (bind _shoulderrightarmor (`self.ShoulderRightArmor`))
  (bind _helmet (`self.helmet`))
  (bind _chestpiece (`self.chestpiece`))
  (bind _armbrace_left (`self.armbrace_left`))
  (bind _armbrace_right (`self.armbrace_right`))
  (bind _shoulderarmor_left (`self.shoulderarmor_left`))
  (`|ExecutionSequence`
    (:`then_0`
      (if (`self.ChestPieceVisible`)
        (set `self.MaxHealth` (+ (`self.MaxHealth`) 25.0))
        (`SceneComponent.SetVisibility` _chestpiece true false)
        (else
          (`SceneComponent.SetVisibility` _chestpiece false false))))
    (:`then_1`
      (if (`self.ArmBraceLeftVisible`)
        (set `self.MaxHealth` (+ (`self.MaxHealth`) 10.0))
        (`SceneComponent.SetVisibility` _armbrace_left true false)
        (else
          (`SceneComponent.SetVisibility` _armbrace_left false false))))
    (:`then_2`
      (if (`self.ArmBraceRightVisible`)
        (set `self.MaxHealth` (+ (`self.MaxHealth`) 10.0))
        (`SceneComponent.SetVisibility` _armbrace_right true false)
        (else
          (`SceneComponent.SetVisibility` _armbrace_right false false))))
    (:`then_3`
      (if (`self.ShoulderArmorLeftVisible`)
        (set `self.MaxHealth` (+ (`self.MaxHealth`) 15.0))
        (`SceneComponent.SetVisibility` _shoulderarmor_left true false)
        (else
          (`SceneComponent.SetVisibility` _shoulderarmor_left false false))))
    (:`then_4`
      (if (`self.ShoulderArmorRightVis`)
        (set `self.MaxHealth` (+ (`self.MaxHealth`) 15.0))
        (`SceneComponent.SetVisibility` _shoulderrightarmor true true)
        (else
          (`SceneComponent.SetVisibility` _shoulderrightarmor false true))))
    (:`then_5`
      (if (`self.bHasHelmet`)
        (if (`self.HasMohawk`)
          (`SceneComponent.SetVisibility` _helmet false false)
          (else
            (set `self.MaxHealth` (+ (`self.MaxHealth`) 10.0))
            (`SceneComponent.SetVisibility` _helmet true false)))
        (else
          (`SceneComponent.SetVisibility` _helmet false false))))))

(fn `ClothingGenerator`
  (bind _beltmesh (`self.BeltMesh`))
  (bind _bootsmesh (`self.BootsMesh`))
  (bind _mohawk (`self.mohawk`))
  (bind _pantsmesh (`self.PantsMesh`))
  (bind _shirtmesh (`self.ShirtMesh`))
  (`|ExecutionSequence`
    (:`then_0`
      (if (`self.PantsVisible`)
        (`SceneComponent.SetVisibility` _pantsmesh true false)
        (else
          (`SceneComponent.SetVisibility` _pantsmesh false false))))
    (:`then_1`
      (if (`self.ShirtVisible`)
        (`SceneComponent.SetVisibility` _shirtmesh true false)
        (else
          (`SceneComponent.SetVisibility` _shirtmesh false false))))
    (:`then_2`
      (if (`self.BeltVisible`)
        (`SceneComponent.SetVisibility` _beltmesh true false)
        (else
          (`SceneComponent.SetVisibility` _beltmesh false false))))
    (:`then_3`
      (if (`self.BootsVisible`)
        (`SceneComponent.SetVisibility` _bootsmesh true false)
        (else
          (`SceneComponent.SetVisibility` _bootsmesh false false))))
    (:`then_4`
      (if (`self.HasMohawk`)
        (if (`self.bHasHelmet`)
          (`SceneComponent.SetVisibility` _mohawk false false)
          (else
            (`SceneComponent.SetVisibility` _mohawk true false)))
        (else
          (`SceneComponent.SetVisibility` _mohawk false false))))))

(fn `HideArmor`
  (`|ExecutionSequence`
    (:`then_0`
      (`SceneComponent.SetVisibility` (`self.chestpiece`) false false))
    (:`then_1`
      (`SceneComponent.SetVisibility` (`self.armbrace_left`) false false))
    (:`then_2`
      (`SceneComponent.SetVisibility` (`self.armbrace_right`) false false))
    (:`then_3`
      (`SceneComponent.SetVisibility` (`self.shoulderarmor_left`) false false))
    (:`then_4`
      (`SceneComponent.SetVisibility` (`self.ShoulderRightArmor`) false false))
    (:`then_5`
      (`SceneComponent.SetVisibility` (`self.helmet`) false false))))

(fn `RandomBoolGenerator`
  (set `self.bIArmored` (`KismetMathLibrary.RandomBool`))
  (set `self.HasMohawk` (`KismetMathLibrary.RandomBool`))
  (set `self.ShirtVisible` (`KismetMathLibrary.RandomBool`))
  (set `self.ShoulderArmorLeftVisible` (`KismetMathLibrary.RandomBool`))
  (set `self.ArmBraceRightVisible` (`KismetMathLibrary.RandomBool`))
  (set `self.ChestPieceVisible` (`KismetMathLibrary.RandomBool`))
  (set `self.ArmBraceLeftVisible` (`KismetMathLibrary.RandomBool`))
  (set `self.ShoulderArmorRightVis` (`KismetMathLibrary.RandomBool`))
  (set `self.bHasHelmet` (`KismetMathLibrary.RandomBool`)))

(fn `UserConstructionScript`
  (bind _shirtmat (`self.ShirtMat`))
  (bind _mohawkmaterial (`self.MohawkMaterial`))
  (bind _weaponmesh (`self.WeaponMesh`))
  (bind _mesh (`self.Mesh`))
  (bind _mesh_2 (`self.Mesh`))
  (bind _mesh_3 (`self.Mesh`))
  (bind _helmetmat (`self.HelmetMat`))
  (`SceneComponent.K2_AttachToComponent` (`self.chestpiece`) _mesh "ChestPiece" "SnapToTarget" "SnapToTarget" "SnapToTarget" true)
  (`SceneComponent.K2_AttachToComponent` (`self.armbrace_left`) _mesh "LeftArmBand" "SnapToTarget" "SnapToTarget" "SnapToTarget" true)
  (`SceneComponent.K2_AttachToComponent` (`self.armbrace_right`) _mesh "RightArmBand" "SnapToTarget" "SnapToTarget" "SnapToTarget" true)
  (`SceneComponent.K2_AttachToComponent` (`self.shoulderarmor_left`) _mesh "LeftShoulderArmor" "SnapToTarget" "SnapToTarget" "SnapToTarget" true)
  (`SceneComponent.K2_AttachToComponent` (`self.FaceStuff`) (`self.Mesh`) "Head" "KeepRelative" "KeepRelative" "KeepWorld" true)
  (`SceneComponent.K2_AttachToComponent` (`self.mohawk`) _mesh_3 "Head_MSocket" "SnapToTarget" "SnapToTarget" "SnapToTarget" true)
  (`SceneComponent.K2_AttachToComponent` (`self.ShoulderRightArmor`) _mesh_3 "RightShoulderArmor" "SnapToTarget" "SnapToTarget" "SnapToTarget" true)
  (`SceneComponent.K2_AttachToComponent` (`self.helmet`) _mesh_2 "Helmet" "SnapToTarget" "SnapToTarget" "SnapToTarget" true)
  (`SceneComponent.K2_AttachToComponent` (`self.Weapon`) _mesh_2 "Weapon" "SnapToTarget" "SnapToTarget" "SnapToTarget" true)
  (`PrimitiveComponent.SetMaterial` (`self.mohawk`) 0 (`|GetArrayItem` _mohawkmaterial (`KismetMathLibrary.RandomIntegerInRange` 0 (`KismetArrayLibrary.Array_LastIndex` _mohawkmaterial))))
  (`PrimitiveComponent.SetMaterial` (`self.ShirtMesh`) 0 (`|GetArrayItem` _shirtmat (`KismetMathLibrary.RandomIntegerInRange` 0 (`KismetArrayLibrary.Array_LastIndex` _shirtmat))))
  (`PrimitiveComponent.SetMaterial` (`self.helmet`) 0 (`|GetArrayItem` _helmetmat (`KismetMathLibrary.RandomIntegerInRange` 0 (`KismetArrayLibrary.Array_LastIndex` _helmetmat))))
  (`StaticMeshComponent.SetStaticMesh` (`self.Weapon`) (`|GetArrayItem` _weaponmesh (`KismetMathLibrary.RandomIntegerInRange` 0 (`KismetArrayLibrary.Array_LastIndex` _weaponmesh))))
  (`self.RandomBoolGenerator`)
  (`|ExecutionSequence`
    (:`then_0`
      (`self.ClothingGenerator`))
    (:`then_1`
      (if (`self.bIArmored`)
        (`self.ArmorGenerator`)
        (else
          (`self.HideArmor`))))))