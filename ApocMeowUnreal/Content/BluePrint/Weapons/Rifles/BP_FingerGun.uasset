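; BP_FingerGun is a VR finger-gun rifle with a small five-round capacity, a detachable BP_FingerAmmp clip and an ammo counter.
; Firing calls FireRifle, updates the counter and spawns muzzle beam emitters, deactivating earlier ones from the Beam array.
; Reload empties and releases the clip, while dropping the gun also destroys the actor.
; The 2HandNode macro toggles second-hand grip on left-hand overlap, but its call and the ammo-spawning logic are unwired.
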(event `/Game/BluePrint/Weapons/BP_WeaponInteractions.ReloadWeapon`
  ;[1 1 1] Handle Reload weapon
  (set `self.MagInGun` false :!label _label)
  (bind _output_get (set `self.CurrentRifleAmmo` 0))
  (`TextRenderComponent.K2_SetText` (`self.AmmoCounterForRifle`) (`KismetTextLibrary.Conv_IntToText` _output_get))
  (`self.K2_DetachFromActor` (`self.AmmoVar`) "KeepWorld" "KeepWorld" "KeepWorld")
  (`/Game/BluePrint/Weapons/Ammo/BP_FingerAmmp.DropTheClipWater` (cast `/Game/BluePrint/Weapons/Ammo/BP_FingerAmmp` (`self.AmmoVar`) :!pure true)))

(event `self.ReceiveBeginPlay`
  ;[1 1 1] Event begin play
  (set `self.MaxRifleAmmo` 5)
  (bind _output_get (set `self.CurrentRifleAmmo` 0))
  (`TextRenderComponent.K2_SetText` (`self.AmmoCounterForRifle`) (`KismetTextLibrary.Conv_IntToText` _output_get)))

(event `DropAmmoToReload`
  ;[1 1 1] Handle Reload weapon
  (goto _label))

(event `/Game/BluePrint/Weapons/BP_WeaponInteractions.Drop`
  ;[1 1 1] Handles weapon drop
  (set `self.PlayerHasGun` false :!label _label_2)
  (`/Engine/EditorBlueprintResources/StandardMacros.IsValid` (`self.AmmoVar`)
    (:`Is Valid`
      (`self.K2_DetachFromActor` (`self.AmmoVar`) "KeepWorld" "KeepWorld" "KeepWorld")
      (`/Game/BluePrint/Weapons/Ammo/BP_FingerAmmp.DropTheClipWater` (cast `/Game/BluePrint/Weapons/Ammo/BP_FingerAmmp` (`self.AmmoVar`) :!pure true))
      (set `self.AmmoVar` null)
      (`self.K2_DetachFromActor` "KeepWorld" "KeepWorld" "KeepWorld")
      (`self.K2_DestroyActor`))
    (:`Is Not Valid`
      (set `self.Spawned?` false)
      (`self.K2_DetachFromActor` "KeepWorld" "KeepWorld" "KeepWorld")
      (`self.K2_DestroyActor`))))

(event `DropTheHand`
  ;[1 1 1] Handles weapon drop
  (goto _label_2))

(event `self.ReceiveTick`
  (params (DeltaSeconds :type "Float (single-precision)"))
  ;[1 1 1] Sets delta sec
  (set `self.DeltaSec` DeltaSeconds))

(event `/Game/BluePrint/Weapons/BP_WeaponInteractions.2ndHandGrip`
  ;[1 1 1] 2 Handed Grip
)

(event `/Game/BluePrint/Weapons/BP_WeaponInteractions.FireWeapon`
  (bind _beam (`self.Beam`))
  (bind _muzzle (`self.Muzzle`))
  (bind _output (`|GetArrayItem` _beam (- (`KismetArrayLibrary.Array_LastIndex` _beam) 1)))
  ;[1 1 1] FireWeapon
  (`self.FireRifle` :!label _label_3)
  (`TextRenderComponent.K2_SetText` (`self.AmmoCounterForRifle`) (`KismetTextLibrary.Conv_IntToText` (`self.CurrentRifleAmmo`)))
  (if (> (`self.CurrentRifleAmmo`) 0)
    (bind _returnvalue (`GameplayStatics.SpawnEmitterAtLocation` null (`SceneComponent.K2_GetComponentLocation` _muzzle) (`SceneComponent.K2_GetComponentRotation` _muzzle)))
    (`KismetArrayLibrary.Array_Add` (`self.Beam`) _returnvalue))
  (`/Engine/EditorBlueprintResources/StandardMacros.IsValid` _output
    (:`Is Valid`
      (`ActorComponent.Deactivate` _output))))

(event `/Game/BluePrint/Weapons/BP_WeaponInteractions.StopFiring`
  (bind _beam (`self.Beam`))
  (bind _output (`|GetArrayItem` _beam (`KismetArrayLibrary.Array_LastIndex` _beam)))
  ;[1 1 1] FireWeapon
  (`/Engine/EditorBlueprintResources/StandardMacros.IsValid` _output
    (:`Is Valid`
      (`ActorComponent.Deactivate` _output)
      (`/Engine/EditorBlueprintResources/StandardMacros.Gate` true :!via `Close` :!label _label_4
        (:`Exit`
          (goto _label_3))))
    (:`Is Not Valid`
      (goto _label_4 :!via `Close`))))

(event `/Game/BluePrint/Weapons/BP_WeaponInteractions.DropAmmo`
  ;[1 1 1] Drops ammo
  (`self.K2_DetachFromActor` (`self.AmmoVar`) "KeepWorld" "KeepWorld" "KeepWorld")
  (`/Game/BluePrint/Weapons/Ammo/BP_FingerAmmp.DropTheClipWater` (cast `/Game/BluePrint/Weapons/Ammo/BP_FingerAmmp` (`self.AmmoVar`) :!pure true)))

(fn `UserConstructionScript`
  (`parent.UserConstructionScript`))