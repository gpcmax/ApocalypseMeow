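; BP_SharkShot is a VR rifle, a child Blueprint that loads BP_SharkAmmo magazines and shows its round count.
; Firing launches a projectile, plays hand and gun montages, rumbles the right controller, then drops and hides the magazine.
; Reload and drop events detach the ammo, with drop also destroying the gun.
; Left-hand overlap toggles a two-hand grip gate, but the timeline that would drive it is unwired.
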(event `self.ReceiveTick`
  (params (DeltaSeconds :type "Float (single-precision)"))
  ;[1 1 1] Sets delta sec
  (set `self.DeltaSec` DeltaSeconds))

(event `/Game/BluePrint/Weapons/BP_WeaponInteractions.ReloadWeapon`
  ;[1 1 1] Handle Reload weapon
  (set `self.MagInGun` false :!label _label)
  (bind _output_get (set `self.CurrentRifleAmmo` 0))
  (`TextRenderComponent.K2_SetText` (`self.AmmoCounterForRifle`) (`KismetTextLibrary.Conv_IntToText` _output_get))
  (`self.K2_DetachFromActor` (`self.AmmoType`) "KeepWorld" "KeepWorld" "KeepWorld")
  (set `self.EReload` "NewEnumerator0")
  (`/Game/BluePrint/Weapons/Ammo/BP_SharkAmmo.DropTheClip` (cast `/Game/BluePrint/Weapons/Ammo/BP_SharkAmmo` (`self.AmmoType`) :!pure true)))

(event `self.ReceiveBeginPlay`
  ;[1 1 1] Event begin play
  (bind _output_get (set `self.CurrentRifleAmmo` 0))
  (`TextRenderComponent.K2_SetText` (`self.AmmoCounterForRifle`) (`KismetTextLibrary.Conv_IntToText` _output_get))
  (bind _asbp_vrchar_1 (cast `/Game/BluePrint/Players/BP_VRChar1` (`GameplayStatics.GetPlayerCharacter` 0)))
  (bind _output_get_2 (set `self.Player` _asbp_vrchar_1))
  (if (`/Game/BluePrint/Players/BP_VRChar1.SharkShotGunLoadedBefore` _output_get_2)
    (`SceneComponent.SetVisibility` (`self.AmmoTextTut`) false false)))

(event `DropAmmoToReload`
  ;[1 1 1] Handle Reload weapon
  (goto _label))

(event `/Game/BluePrint/Weapons/BP_WeaponInteractions.2ndHandGrip`
  ;[1 1 1] 2 Handed Grip
  (bind _asbp_vrchar_1 (cast `/Game/BluePrint/Players/BP_VRChar1` (`GameplayStatics.GetPlayerCharacter` 0)))
  (if (`PrimitiveComponent.IsOverlappingComponent` (`self.SecondHandCol`) (`VRMainCharacter.LeftHandCol` _asbp_vrchar_1))
    (`/Engine/EditorBlueprintResources/StandardMacros.Gate` true :!via `Toggle`
      (:`Exit`
        (`self.SecondHandGrip` (`self.DeltaSec`) _asbp_vrchar_1)))))

(event `/Game/BluePrint/Weapons/BP_WeaponInteractions.FireWeapon`
  (bind _ammovar (`self.AmmoVar`))
  ;[1 1 1] Fire weapons
  (`self.FireProjectile`)
  (`TextRenderComponent.K2_SetText` (`self.AmmoCounterForRifle`) (`KismetTextLibrary.Conv_IntToText` (`self.CurrentRifleAmmo`)))
  (bind _asbp_vrchar_1 (cast `/Game/BluePrint/Players/BP_VRChar1` (`GameplayStatics.GetPlayerCharacter` 0)))
  (`|PlayMontage` (`VRMainCharacter.RightHandMeshSK` _asbp_vrchar_1) "/Game/Characters/Player/Hand/Anims/Old/HandFireAnim_Montage.HandFireAnim_Montage"
    (:`then`
      (`|PlayMontage` (`self.RifleMesh`) "/Game/ART/WeaponMeshes/SharkShot/Anim/Fire_Montage.Fire_Montage"
        (:`then`
          (`/Game/BluePrint/Players/BP_VRChar1.RumbleController` _asbp_vrchar_1 1.0 "Right")
          (set `self.EReload` "NewEnumerator0")
          (message `/Game/BluePrint/Weapons/BP_WeaponInteractions.DropAmmo` (`self.GetOverlappingActors` "BP_SharkShot_C"))
          (`/Engine/EditorBlueprintResources/StandardMacros.IsValid` _ammovar
            (:`Is Valid`
              (`/Game/BluePrint/Weapons/Ammo/BP_SharkAmmo.DropTheClip` (cast `/Game/BluePrint/Weapons/Ammo/BP_SharkAmmo` _ammovar :!pure true))
              (`self.SetActorHiddenInGame` _ammovar true)
              (set `self.MagInGun` false))))))))

(event `/Game/BluePrint/Weapons/BP_WeaponInteractions.Ammo`
  ;[1 1 1] Spawns Ammo
  (bind _ammo (`self.SpawnAndGrabAmmo` "/Game/BluePrint/Weapons/Ammo/BP_SharkAmmo.BP_SharkAmmo_C"))
  (bind _asbp_shark_ammo (cast `/Game/BluePrint/Weapons/Ammo/BP_SharkAmmo` _ammo))
  (set `self.AmmoVar` _asbp_shark_ammo))

(event `/Game/BluePrint/Weapons/BP_WeaponInteractions.Drop`
  ;[1 1 1] Handles weapon drop
  (set `self.PlayerHasGun` false)
  (`/Engine/EditorBlueprintResources/StandardMacros.IsValid` (`self.AmmoVar`)
    (:`Is Valid`
      (set `/Game/BluePrint/Players/BP_VRChar1.RifleHolstered` false (`self.Player`))
      (set `self.RifleHolster?` false)
      (`self.K2_DetachFromActor` (`self.AmmoVar`) "KeepWorld" "KeepWorld" "KeepWorld")
      (`/Game/BluePrint/Weapons/Ammo/BP_SharkAmmo.DropTheClip` (cast `/Game/BluePrint/Weapons/Ammo/BP_SharkAmmo` (`self.AmmoVar`) :!pure true))
      (set `self.AmmoVar` null)
      (set `self.EReload` "NewEnumerator0")
      (`self.K2_DetachFromActor` "KeepWorld" "KeepWorld" "KeepWorld")
      (`self.K2_DestroyActor`))
    (:`Is Not Valid`
      (set `/Game/BluePrint/Players/BP_VRChar1.RifleHolstered` false (`self.Player`))
      (set `self.RifleHolster?` false)
      (set `self.Spawned?` false)
      (`self.K2_DetachFromActor` "KeepWorld" "KeepWorld" "KeepWorld")
      (`self.K2_DestroyActor`))))

(event `/Game/BluePrint/Weapons/BP_WeaponInteractions.DropAmmo`
  ;[1 1 1] Drops ammo
  (`self.K2_DetachFromActor` (`self.AmmoVar`) "KeepWorld" "KeepWorld" "KeepWorld")
  (`/Game/BluePrint/Weapons/Ammo/BP_SharkAmmo.DropTheClip` (cast `/Game/BluePrint/Weapons/Ammo/BP_SharkAmmo` (`self.AmmoType`) :!pure true)))

(event `/Game/BluePrint/Weapons/BP_WeaponInteractions.Grab`
  (params (AttachTo :type "SceneComponent Object Reference"))
  ;[1 1 1] test grab
)

(fn `UserConstructionScript`
  (`parent.UserConstructionScript`)
  (`SceneComponent.K2_AttachToComponent` (`self.MagLoc`) (`self.RifleMesh`) "Sled" "SnapToTarget" "KeepWorld" "KeepRelative" false))