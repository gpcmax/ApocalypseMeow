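; BP_SpecOpsShot is a VR rifle with grab, drop, firing, reload and an ammo counter.
; It spawns a BP_SpecOpdsAmmo magazine via SpawnAndGrabAmmo, detaches it on reload, and drops and hides it on every shot.
; Firing calls FireProjectile, updates the counter and rumbles the right controller.
; Left-hand overlap toggles a gate for SecondHandGrip, but the timeline feeding that gate is never started.
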(event `/Game/BluePrint/Weapons/BP_WeaponInteractions.ReloadWeapon`
  ;[1 1 1] Handle Reload weapon
  (set `self.MagInGun` false)
  (bind _output_get (set `self.CurrentRifleAmmo` 0))
  (`TextRenderComponent.K2_SetText` (`self.AmmoCounterForRifle`) (`KismetTextLibrary.Conv_IntToText` _output_get))
  (`self.K2_DetachFromActor` (`self.AmmoVar`) "KeepWorld" "KeepWorld" "KeepWorld")
  (`/Game/BluePrint/Weapons/Ammo/BP_SpecOpdsAmmo.DropTheClip` (cast `/Game/BluePrint/Weapons/Ammo/BP_SpecOpdsAmmo` (`self.AmmoVar`) :!pure true)))

(event `self.ReceiveBeginPlay`
  ;[1 1 1] Event begin play
  (bind _output_get (set `self.CurrentRifleAmmo` 0))
  (`TextRenderComponent.K2_SetText` (`self.AmmoCounterForRifle`) (`KismetTextLibrary.Conv_IntToText` _output_get)))

(event `self.ReceiveTick`
  (params (DeltaSeconds :type "Float (single-precision)"))
  ;[1 1 1] Sets delta sec
  (set `self.DeltaSec` DeltaSeconds))

(event `/Game/BluePrint/Weapons/BP_WeaponInteractions.Drop`
  ;[1 1 1] Handles weapon drop
  (set `self.PlayerHasGun` false)
  (set `self.AmmoVar` null)
  (`self.K2_DetachFromActor` "KeepWorld" "KeepWorld" "KeepWorld"))

(event `/Game/BluePrint/Weapons/BP_WeaponInteractions.2ndHandGrip`
  ;[1 1 1] 2 Handed Grip
  (bind _asbp_vrchar_1 (cast `/Game/BluePrint/Players/BP_VRChar1` (`GameplayStatics.GetPlayerCharacter` 0)))
  (if (`PrimitiveComponent.IsOverlappingComponent` (`self.SecondHandCol`) (`VRMainCharacter.LeftHandCol` _asbp_vrchar_1))
    (`/Engine/EditorBlueprintResources/StandardMacros.Gate` true :!via `Toggle`
      (:`Exit`
        (`self.SecondHandGrip` (`self.DeltaSec`) _asbp_vrchar_1)))))

(event `/Game/BluePrint/Weapons/BP_WeaponInteractions.FireWeapon`
  (bind _asbp_spec_opds_ammo (cast `/Game/BluePrint/Weapons/Ammo/BP_SpecOpdsAmmo` (`self.AmmoVar`) :!pure true))
  ;[1 1 1] Fire weapons
  (`self.FireProjectile`)
  (`TextRenderComponent.K2_SetText` (`self.AmmoCounterForRifle`) (`KismetTextLibrary.Conv_IntToText` (`self.CurrentRifleAmmo`)))
  (bind _asbp_vrchar_1 (cast `/Game/BluePrint/Players/BP_VRChar1` (`GameplayStatics.GetPlayerCharacter` 0)))
  (`/Game/BluePrint/Players/BP_VRChar1.RumbleController` _asbp_vrchar_1 1.0 "Right")
  (`/Game/BluePrint/Weapons/Ammo/BP_SpecOpdsAmmo.DropTheClip` _asbp_spec_opds_ammo)
  (`self.SetActorHiddenInGame` _asbp_spec_opds_ammo true))

(event `/Game/BluePrint/Weapons/BP_WeaponInteractions.Ammo`
  ;[1 1 1] Spawns Ammo
  (bind _ammo (`self.SpawnAndGrabAmmo` "/Game/BluePrint/Weapons/Ammo/BP_SpecOpdsAmmo.BP_SpecOpdsAmmo_C"))
  (bind _asbp_spec_opds_ammo (cast `/Game/BluePrint/Weapons/Ammo/BP_SpecOpdsAmmo` _ammo))
  (set `self.AmmoVar` _asbp_spec_opds_ammo))

(event `/Game/BluePrint/Weapons/BP_WeaponInteractions.DropAmmo`
  ;[1 1 1] Drops ammo
  (`self.K2_DetachFromActor` (`self.AmmoVar`) "KeepWorld" "KeepWorld" "KeepWorld")
  (`/Game/BluePrint/Weapons/Ammo/BP_SpecOpdsAmmo.DropTheClip` (cast `/Game/BluePrint/Weapons/Ammo/BP_SpecOpdsAmmo` (`self.AmmoVar`) :!pure true)))

(event `/Game/BluePrint/Weapons/BP_WeaponInteractions.Grab`
  (params (AttachTo :type "SceneComponent Object Reference"))
  ;[1 1 1] test grab
  (`self.K2_AttachToComponent` AttachTo "None" "SnapToTarget" "SnapToTarget" "SnapToTarget")
  (set `self.PlayerHasGun` true))

(fn `UserConstructionScript`
  (`parent.UserConstructionScript`))