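; VR rifle Blueprint (PewGun) that fires projectiles from its muzzle, with an ammo counter, montages, sound and controller rumble.
; Ammo requests spawn and grab a magazine, ejecting any loaded one first.
; Dropping the gun releases the magazine, clears holster state and destroys the actor.
; Two-handed grip checks left-hand overlap to toggle a gate, but the timeline feeding that gate never runs.
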(event `self.ReceiveBeginPlay`
  ;[1 1 1] Event begin play
  (set `self.MaxRifleAmmo` 5)
  (bind _output_get (set `self.CurrentRifleAmmo` 0))
  (`TextRenderComponent.K2_SetText` (`self.AmmoCounterForRifle`) (`KismetTextLibrary.Conv_IntToText` _output_get))
  (bind _asbp_vrchar_1 (cast `/Game/BluePrint/Players/BP_VRChar1` (`GameplayStatics.GetPlayerCharacter` 0)))
  (bind _output_get_2 (set `self.Player` _asbp_vrchar_1))
  (if (`/Game/BluePrint/Players/BP_VRChar1.PewGunLoadedBefore` _output_get_2)
    (`SceneComponent.SetVisibility` (`self.AmmoTextTut`) false false)))

(event `/Game/BluePrint/Weapons/BP_WeaponInteractions.Drop`
  ;[1 1 1] Handles weapon drop
  (set `self.PlayerHasGun` false)
  (`/Engine/EditorBlueprintResources/StandardMacros.IsValid` (`self.AmmoVar`)
    (:`Is Valid`
      (set `/Game/BluePrint/Players/BP_VRChar1.RifleHolstered` false (`self.Player`))
      (set `self.RifleHolster?` false)
      (`/Game/BluePrint/Weapons/Ammo/BP_JoltGunAmmo.DropTheClip` (cast `/Game/BluePrint/Weapons/Ammo/bp_PewGunAmmo` (`self.AmmoVar`) :!pure true))
      (`self.DropAmmoToReload`)
      (set `self.AmmoVar` null)
      (`self.K2_DetachFromActor` "KeepWorld" "KeepWorld" "KeepWorld")
      (`self.K2_DestroyActor`))
    (:`Is Not Valid`
      (set `/Game/BluePrint/Players/BP_VRChar1.RifleHolstered` false (`self.Player`))
      (set `self.RifleHolster?` false)
      (set `self.Spawned?` false)
      (`self.K2_DetachFromActor` "KeepWorld" "KeepWorld" "KeepWorld")
      (`self.K2_DestroyActor`))))

(event `/Game/BluePrint/Weapons/BP_WeaponInteractions.ReloadWeapon`
  ;[1 1 1] Handle Reload weapon
  (set `self.MagInGun` false :!label _label)
  (bind _output_get (set `self.CurrentRifleAmmo` 0))
  (`TextRenderComponent.K2_SetText` (`self.AmmoCounterForRifle`) (`KismetTextLibrary.Conv_IntToText` _output_get))
  (`self.K2_DetachFromActor` (`self.AmmoVar`) "KeepWorld" "KeepWorld" "KeepWorld")
  (`/Game/BluePrint/Weapons/Ammo/bp_PewGunAmmo.DropTheClip` (cast `/Game/BluePrint/Weapons/Ammo/bp_PewGunAmmo` (`self.AmmoVar`) :!pure true)))

(event `DropAmmoToReload`
  ;[1 1 1] Handle Reload weapon
  (goto _label))

(event `self.ReceiveTick`
  (params (DeltaSeconds :type "Float (single-precision)"))
  ;[1 1 1] Sets delta sec
  (set `self.DeltaSec` DeltaSeconds))

(event `/Game/BluePrint/Weapons/BP_WeaponInteractions.2ndHandGrip`
  ;[1 1 1] 2 Handed Grip
  (bind _asbp_vrchar_1 (cast `/Game/BluePrint/Players/BP_VRChar1` (`GameplayStatics.GetPlayerCharacter` 0)))
  (if (`PrimitiveComponent.IsOverlappingComponent` (`self.SecondHandCol`) (`VRMainCharacter.LeftHandCol` _asbp_vrchar_1))
    (`/Engine/EditorBlueprintResources/StandardMacros.Gate` true :!via `Toggle`
      (:`Exit`
        (`self.SecondHandGrip` (`self.DeltaSec`) _asbp_vrchar_1)
        (set `self.2HandedMode` true)))
    (else
      (set `self.2HandedMode` false))))

(event `/Game/BluePrint/Weapons/BP_WeaponInteractions.FireWeapon`
  (bind _currentrifleammo (`self.CurrentRifleAmmo`))
  (bind (_returnvalue_location _returnvalue_rotation) (`KismetMathLibrary.BreakTransform` (`SceneComponent.K2_GetComponentToWorld` (`self.Muzzle`))))
  ;[1 1 1] Fire weapons
  (if (> (`self.CurrentRifleAmmo`) 0)
    (`|SpawnActorFromClass` "/Game/BluePrint/Weapons/Projectile/Pew.Pew_C" (`KismetMathLibrary.MakeTransform` _returnvalue_location _returnvalue_rotation) "Undefined" "OverrideRootScale" null null)
    (set `self.CurrentRifleAmmo` (- _currentrifleammo 1))
    (`TextRenderComponent.K2_SetText` (`self.AmmoCounterForRifle`) (`KismetTextLibrary.Conv_IntToText` _currentrifleammo))
    ;[1 1 1] Handles fire anim
    (bind _asbp_vrchar_1 (cast `/Game/BluePrint/Players/BP_VRChar1` (`GameplayStatics.GetPlayerCharacter` 0)))
    (`|PlayMontage` (`VRMainCharacter.RightHandMeshSK` _asbp_vrchar_1) "/Game/Characters/Player/Hand/Anims/Old/HandFireAnim_Montage.HandFireAnim_Montage"
      (:`then`
        (`|PlayMontage` (`self.RifleMesh`) "/Game/ART/WeaponMeshes/PewGun/Anim/PewGun_Fire_LargeRecoil_Montage.PewGun_Fire_LargeRecoil_Montage"
          (:`then`
            (`GameplayStatics.PlaySoundAtLocation` "/Game/Audio/PewGun/PewGun_Fire_Cue.PewGun_Fire_Cue" (`SceneComponent.K2_GetComponentLocation` (`self.Muzzle`)))
            (`/Game/BluePrint/Players/BP_VRChar1.RumbleController` _asbp_vrchar_1 1.0 "Right")))))
    (else
      (`GameplayStatics.PlaySoundAtLocation` "/Game/Audio/DryFire/DryFireCue.DryFireCue" (`SceneComponent.K2_GetComponentLocation` (`self.Muzzle`))))))

(event `/Game/BluePrint/Weapons/BP_WeaponInteractions.DropAmmo`
  ;[1 1 1] Drops ammo
  (`self.K2_DetachFromActor` (`self.AmmoVar`) "KeepWorld" "KeepWorld" "KeepWorld")
  (`/Game/BluePrint/Weapons/Ammo/bp_PewGunAmmo.DropTheClip` (cast `/Game/BluePrint/Weapons/Ammo/bp_PewGunAmmo` (`self.AmmoVar`) :!pure true)))

(event `/Game/BluePrint/Weapons/BP_WeaponInteractions.Ammo`
  ;[1 1 1] Spawns Ammo
  (if (`self.MagInGun`)
    (`self.DropAmmoToReload`)
    (bind _ammo (`self.SpawnAndGrabAmmo` "/Game/BluePrint/Weapons/Ammo/bp_PewGunAmmo.bp_PewGunAmmo_C"))
    (bind _asbp_pew_gun_ammo (cast `/Game/BluePrint/Weapons/Ammo/bp_PewGunAmmo` _ammo))
    (set `self.AmmoVar` _asbp_pew_gun_ammo)
    (else
      (bind _ammo_2 (`self.SpawnAndGrabAmmo` "/Game/BluePrint/Weapons/Ammo/bp_PewGunAmmo.bp_PewGunAmmo_C"))
      (bind _asbp_pew_gun_ammo_2 (cast `/Game/BluePrint/Weapons/Ammo/bp_PewGunAmmo` _ammo_2))
      (set `self.AmmoVar` _asbp_pew_gun_ammo_2))))

(fn `UserConstructionScript`
  (`parent.UserConstructionScript`))