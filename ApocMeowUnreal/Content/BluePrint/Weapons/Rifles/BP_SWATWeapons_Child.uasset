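; VR SWAT rifle child Blueprint for the SplitFire gun, handling firing, magazines, fire-mode switching and holster cleanup on drop.
; Ammo requests spawn and grab a bp_SplitFireAmmo magazine, while reload or drop detaches it; dropping the gun also destroys it.
; Firing calls FireProjectile, then updates the counter and plays hand and recoil montages with controller rumble.
; Full-auto and two-hand grip use gates, but their timeline drivers and the 2HandNode call are unwired.
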(event `/Game/BluePrint/Weapons/BP_WeaponInteractions.ReloadWeapon`
  ;[1 1 1] Handle Reload weapon
  (set `self.MagInGun` false :!label _label)
  (bind _output_get (set `self.CurrentRifleAmmo` 0))
  (`TextRenderComponent.K2_SetText` (`self.AmmoCounterForRifle`) (`KismetTextLibrary.Conv_IntToText` _output_get))
  (`self.K2_DetachFromActor` (`self.AmmoType`) "KeepWorld" "KeepWorld" "KeepWorld")
  (`self.K2_DetachFromActor` (`self.AmmoVar`) "KeepWorld" "KeepWorld" "KeepWorld")
  (`/Game/BluePrint/Weapons/Ammo/bp_SplitFireAmmo.DropTheClip` (cast `/Game/BluePrint/Weapons/Ammo/bp_SplitFireAmmo` (`self.AmmoVar`) :!pure true)))

(event `DropAmmoToReload`
  ;[1 1 1] Handle Reload weapon
  (goto _label))

(event `/Game/BluePrint/Weapons/BP_WeaponInteractions.Drop`
  ;[1 1 1] Handles weapon drop
  (set `self.PlayerHasGun` false)
  (`/Engine/EditorBlueprintResources/StandardMacros.IsValid` (`self.AmmoVar`)
    (:`Is Valid`
      (set `/Game/BluePrint/Players/BP_VRChar1.RifleHolstered` false (`self.Player`))
      (set `self.RifleHolster?` false)
      (`self.K2_DetachFromActor` (`self.AmmoVar`) "KeepWorld" "KeepWorld" "KeepWorld")
      (`/Game/BluePrint/Weapons/Ammo/bp_SplitFireAmmo.DropTheClip` (cast `/Game/BluePrint/Weapons/Ammo/bp_SplitFireAmmo` (`self.AmmoVar`) :!pure true))
      (set `self.AmmoVar` null)
      (`self.K2_DetachFromActor` "KeepWorld" "KeepWorld" "KeepWorld")
      (`self.K2_DestroyActor`))
    (:`Is Not Valid`
      (set `/Game/BluePrint/Players/BP_VRChar1.RifleHolstered` false (`self.Player`))
      (set `self.RifleHolster?` false)
      (set `self.Spawned?` false)
      (`self.K2_DetachFromActor` "KeepWorld" "KeepWorld" "KeepWorld")
      (`self.K2_DestroyActor`))))

(event `self.ReceiveBeginPlay`
  ;[1 1 1] Event begin play
  (set `self.MaxRifleAmmo` 30)
  (bind _output_get (set `self.CurrentRifleAmmo` 0))
  (`TextRenderComponent.K2_SetText` (`self.AmmoCounterForRifle`) (`KismetTextLibrary.Conv_IntToText` _output_get))
  (bind _asbp_vrchar_1 (cast `/Game/BluePrint/Players/BP_VRChar1` (`GameplayStatics.GetPlayerCharacter` 0)))
  (bind _output_get_2 (set `self.Player` _asbp_vrchar_1))
  (if (`/Game/BluePrint/Players/BP_VRChar1.SplitFireGunLoadedBefore` _output_get_2)
    (`SceneComponent.SetVisibility` (`self.AmmoTextTut`) false false)))

(event `self.ReceiveTick`
  (params (DeltaSeconds :type "Float (single-precision)"))
  ;[1 1 1] Sets delta sec
  (set `self.DeltaSec` DeltaSeconds))

(event `/Game/BluePrint/Weapons/BP_WeaponInteractions.2ndHandGrip`
  ;[1 1 1] 2 Handed Grip
)

(event `/Game/BluePrint/Weapons/BP_WeaponInteractions.Stop2Hand`)

(event `/Game/BluePrint/Weapons/BP_WeaponInteractions.Ammo`
  ;[1 1 1] Spawns Ammo
  (if (`self.MagInGun`)
    (set `self.MagInGun` false)
    (bind _output_get (set `self.CurrentRifleAmmo` 0))
    (`TextRenderComponent.K2_SetText` (`self.AmmoCounterForRifle`) (`KismetTextLibrary.Conv_IntToText` _output_get))
    (`self.K2_DetachFromActor` (`self.AmmoVar`) "KeepWorld" "KeepWorld" "KeepWorld")
    (`/Game/BluePrint/Weapons/Ammo/bp_SplitFireAmmo.DropTheClip` (cast `/Game/BluePrint/Weapons/Ammo/bp_SplitFireAmmo` (`self.AmmoVar`) :!pure true))
    (bind _ammo (`self.SpawnAndGrabAmmo` "/Game/BluePrint/Weapons/Ammo/bp_SplitFireAmmo.bp_SplitFireAmmo_C"))
    (bind _asbp_split_fire_ammo (cast `/Game/BluePrint/Weapons/Ammo/bp_SplitFireAmmo` _ammo))
    (set `self.AmmoVar` _asbp_split_fire_ammo)
    (else
      (bind _ammo_2 (`self.SpawnAndGrabAmmo` null))
      (bind _asbp_split_fire_ammo_2 (cast `/Game/BluePrint/Weapons/Ammo/bp_SplitFireAmmo` _ammo_2))
      (set `self.AmmoVar` _asbp_split_fire_ammo_2)
      (set `self.SplitfireAmmo` _asbp_split_fire_ammo_2))))

(event `/Game/BluePrint/Weapons/BP_WeaponInteractions.FireWeapon`
  ;[1 1 1] Fire weapons
  (switch `/Game/BluePrint/ENUMs/FireRate` (`self.FireMode`)
    (:`NewEnumerator0`
      (`self.FireProjectile` :!label _label_2)
      (`TextRenderComponent.K2_SetText` (`self.AmmoCounterForRifle`) (`KismetTextLibrary.Conv_IntToText` (`self.CurrentRifleAmmo`)))
      (bind _asbp_vrchar_1 (cast `/Game/BluePrint/Players/BP_VRChar1` (`GameplayStatics.GetPlayerCharacter` 0)))
      (`|PlayMontage` (`VRMainCharacter.RightHandMeshSK` _asbp_vrchar_1) "/Game/Characters/Player/Hand/Anims/Old/HandFireAnim_Montage.HandFireAnim_Montage"
        (:`then`
          (`|PlayMontage` (`self.RifleMesh`) "/Game/ART/WeaponMeshes/SplitFire/Anim/Mont_SplitFireLargeRecoil.Mont_SplitFireLargeRecoil"
            (:`then`
              (`/Game/BluePrint/Players/BP_VRChar1.RumbleController` _asbp_vrchar_1 1.0 "Right"))))))
    (:`NewEnumerator1`
      (`/Engine/EditorBlueprintResources/StandardMacros.Gate` true :!via `Open` :!label _label_3
        (:`Exit`
          (`KismetSystemLibrary.Delay` 0.1)
          (goto _label_2))))))

(event `/Game/BluePrint/Weapons/BP_WeaponInteractions.StopFiring`
  ;[1 1 1] Fire weapons
  (goto _label_3 :!via `Close`))

(event `/Game/BluePrint/Weapons/BP_WeaponInteractions.DropAmmo`
  ;[1 1 1] Drops ammo
  (`self.K2_DetachFromActor` (`self.AmmoVar`) "KeepWorld" "KeepWorld" "KeepWorld")
  (`/Game/BluePrint/Weapons/Ammo/bp_SplitFireAmmo.DropTheClip` (cast `/Game/BluePrint/Weapons/Ammo/bp_SplitFireAmmo` (`self.AmmoVar`) :!pure true)))

(event `/Game/BluePrint/Weapons/BP_WeaponInteractions.SwitchFireRate`
  ;[1 1 1] Weapon fire rate
  (`/Engine/EditorBlueprintResources/StandardMacros.FlipFlop`
    (:`A`
      (set `self.FireMode` "NewEnumerator1"))
    (:`B`
      (set `self.FireMode` "NewEnumerator0"))))

(fn `UserConstructionScript`
  (`parent.UserConstructionScript`))