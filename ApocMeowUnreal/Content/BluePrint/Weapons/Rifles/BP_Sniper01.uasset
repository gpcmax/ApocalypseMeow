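; VR bolt-action sniper rifle with an ammo counter, detachable BP_SniperClip magazine and two-handed grip.
; Firing requires a round in the chamber, then plays hand and rifle montages, rumbles the controller and empties the chamber.
; Gated bolt logic maps left-hand position relative to the head to eject and chamber states.
; Reload detaches the clip; dropping the rifle releases any clip, clears holster flags and destroys the rifle.
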(event `self.ReceiveBeginPlay`
  ;[1 1 1] Event begin play
  (set `self.MaxRifleAmmo` 5)
  (bind _output_get (set `self.CurrentRifleAmmo` 0))
  (`TextRenderComponent.K2_SetText` (`self.AmmoCounterForRifle`) (`KismetTextLibrary.Conv_IntToText` _output_get))
  (bind _asbp_vrchar_1 (cast `/Game/BluePrint/Players/BP_VRChar1` (`GameplayStatics.GetPlayerPawn` 0)))
  (bind _output_get_2 (set `self.Player` _asbp_vrchar_1))
  (`SceneComponent.SetVisibility` (`self.BoltTut`) false false)
  (if (`/Game/BluePrint/Players/BP_VRChar1.SniperGunLoadedBefore` _output_get_2)
    (`SceneComponent.SetVisibility` (`self.AmmoTextTut`) false false)))

(event `/Game/BluePrint/Weapons/BP_WeaponInteractions.ReloadWeapon`
  ;[1 1 1] Handle Reload weapon
  (set `self.MagInGun` false :!label _label)
  (bind _output_get (set `self.CurrentRifleAmmo` 0))
  (`TextRenderComponent.K2_SetText` (`self.AmmoCounterForRifle`) (`KismetTextLibrary.Conv_IntToText` _output_get))
  (`self.K2_DetachFromActor` (`self.AmmoVar`) "KeepWorld" "KeepWorld" "KeepWorld")
  (`/Game/BluePrint/Weapons/Ammo/BP_SniperClip.DropTheSniperClip` (cast `/Game/BluePrint/Weapons/Ammo/BP_SniperClip` (`self.AmmoVar`) :!pure true)))

(event `DropAmmoToReload`
  ;[1 1 1] Handle Reload weapon
  (goto _label))

(event `/Game/BluePrint/Weapons/BP_WeaponInteractions.Drop`
  ;[1 1 1] Handles weapon drop
  (set `self.PlayerHasGun` false)
  (`/Engine/EditorBlueprintResources/StandardMacros.IsValid` (`self.AmmoVar`)
    (:`Is Valid`
      (set `/Game/BluePrint/Players/BP_VRChar1.RifleHolstered` false (`self.Player`))
      (set `self.RifleHolster?` false)
      (`self.K2_DetachFromActor` (`self.AmmoVar`) "KeepWorld" "KeepWorld" "KeepWorld")
      (`/Game/BluePrint/Weapons/Ammo/BP_SniperClip.DropTheSniperClip` (cast `/Game/BluePrint/Weapons/Ammo/BP_SniperClip` (`self.AmmoVar`) :!pure true))
      (set `self.AmmoVar` null)
      (`self.K2_DetachFromActor` "KeepWorld" "KeepWorld" "KeepWorld")
      (`self.K2_DestroyActor`))
    (:`Is Not Valid`
      (set `/Game/BluePrint/Players/BP_VRChar1.RifleHolstered` false (`self.Player`))
      (set `self.RifleHolster?` false)
      (set `self.Spawned?` false)
      (`self.K2_DetachFromActor` "KeepWorld" "KeepWorld" "KeepWorld")
      (`self.K2_DestroyActor`))))

(event `self.ReceiveTick`
  (params (DeltaSeconds :type "Float (single-precision)"))
  ;[1 1 1] Sets delta sec
  (set `self.DeltaSec` DeltaSeconds))

(event `/Game/BluePrint/Weapons/BP_WeaponInteractions.2ndHandGrip`
  ;[1 1 1] 2 Handed Grip
  (bind _asbp_vrchar_1 (cast `/Game/BluePrint/Players/BP_VRChar1` (`GameplayStatics.GetPlayerCharacter` 0)))
  (if (`PrimitiveComponent.IsOverlappingComponent` (`self.SecondHandCol`) (`VRMainCharacter.LeftHandCol` _asbp_vrchar_1))
    (`/Engine/EditorBlueprintResources/StandardMacros.Gate` true :!via `Open` :!label _label_2
      (:`Exit`
        (`self.SecondHandGrip` (`self.DeltaSec`) _asbp_vrchar_1)
        (set `self.2HandedMode` true)))
    (else
      (set `self.2HandedMode` false)
      (`self.Stop2HandGrip`)
      (goto _label_2 :!via `Close`))))

(event `/Game/BluePrint/Weapons/BP_WeaponInteractions.FireWeapon`
  ;[1 1 1] FireWeapon
  (switch `/Game/BluePrint/ENUMs/ShotGunStates` (`self.SniperStates`)
    (:`NewEnumerator0`
      (`/Engine/EditorBlueprintResources/StandardMacros.DoOnce` false :!label _label_3
        (:`Completed`
          (`self.FireProjectile`)
          (`TextRenderComponent.K2_SetText` (`self.AmmoCounterForRifle`) (`KismetTextLibrary.Conv_IntToText` (`self.CurrentRifleAmmo`)))
          (bind _asbp_vrchar_1 (cast `/Game/BluePrint/Players/BP_VRChar1` (`GameplayStatics.GetPlayerCharacter` 0)))
          (`|PlayMontage` (`VRMainCharacter.RightHandMeshSK` _asbp_vrchar_1) "/Game/Characters/Player/Hand/Anims/Old/HandFireAnim_Montage.HandFireAnim_Montage"
            (:`then`
              (`|PlayMontage` (`self.RifleMesh`) "/Game/ART/WeaponMeshes/SplitFire/Anim/Mont_SplitFireLargeRecoil.Mont_SplitFireLargeRecoil"
                (:`then`
                  (`/Game/BluePrint/Players/BP_VRChar1.RumbleController` _asbp_vrchar_1 1.0 "Right")
                  (set `self.SniperStates` "NewEnumerator1"))))))))))

(event `ExpellRound`
  ;[1 1 1] FireWeapon
  (goto _label_3 :!via `Reset`))

(event `/Game/BluePrint/Weapons/BP_WeaponInteractions.DropAmmo`
  ;[1 1 1] Drops ammo
  (`self.K2_DetachFromActor` (`self.AmmoVar`) "KeepWorld" "KeepWorld" "KeepWorld")
  (`/Game/BluePrint/Weapons/Ammo/BP_SniperClip.DropTheSniperClip` (cast `/Game/BluePrint/Weapons/Ammo/BP_SniperClip` (`self.AmmoVar`) :!pure true)))

(event `/Game/BluePrint/Weapons/BP_WeaponInteractions.Pump`
  (bind _player (`self.Player`))
  (bind _returnvalue_x (`KismetMathLibrary.BreakVector` (`VictoryBPFunctionLibrary.GetComponentRelativeLocation` (`/Game/BluePrint/Players/BP_VRChar1.playerHead` _player) (`VRMainCharacter.LeftHandCol` _player))))
  ;[1 1 1] Sniper bolt
  (if (`self.CanBolt`)
    (`/Engine/EditorBlueprintResources/StandardMacros.Gate` true :!via `Open` :!label _label_4
      (:`Exit`
        (bind _output_get (set `self.BoltLoc` (`KismetMathLibrary.MakeVector` 0.0 0.0 _returnvalue_x)))
        (if (> (`self.CurrentRifleAmmo`) 0)
          (`|ExecutionSequence`
            (:`then_0`
              (bind _returnvalue (`KismetMathLibrary.FClamp` (.z _output_get) 14.0 -18.0))
              (if (`KismetMathLibrary.InRange_FloatFloat` _returnvalue 9.0 16.0)
                (set `self.SniperStates` "NewEnumerator1")
                (`self.ExpellRound`)))
            (:`then_1`
              (if (`KismetMathLibrary.InRange_FloatFloat` _returnvalue -18.0 8.5)
                (set `self.SniperStates` "NewEnumerator0")
                (`/Engine/EditorBlueprintResources/StandardMacros.DoOnce` false
                  (:`Completed`
                    (`SceneComponent.SetVisibility` (`self.BoltTut`) false false)))))))))
    (else
      (goto _label_4 :!via `Close`))))

(event `/Game/BluePrint/Weapons/BP_WeaponInteractions.StopPump`
  ;[1 1 1] Sniper bolt
  (goto _label_4 :!via `Close`))

(event `self.SniperBolt.OnComponentBeginOverlap`
  (params (OverlappedComponent :type "PrimitiveComponent Object Reference") (OtherActor :type "Actor Object Reference") (OtherComp :type "PrimitiveComponent Object Reference") (OtherBodyIndex :type Integer) (bFromSweep :type Boolean) (SweepResult :type "HitResult Structure (by ref)"))
  (bind _asbp_vrchar_1 (cast `/Game/BluePrint/Players/BP_VRChar1` OtherActor))
  (if (`PrimitiveComponent.IsOverlappingComponent` (`VRMainCharacter.LeftHandCol` _asbp_vrchar_1) (`self.SniperBolt`))
    (set `self.CanBolt` true)
    (else
      (set `self.CanBolt` false))))

(fn `UserConstructionScript`
  (`parent.UserConstructionScript`)
  (`SceneComponent.K2_AttachToComponent` (`self.SniperBolt`) (`self.RifleMesh`) "Bolt" "KeepRelative" "KeepRelative" "KeepRelative" true))