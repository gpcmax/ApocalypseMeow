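; VR Jolt Gun rifle Blueprint that starts unloaded and shows its round count on an ammo counter.
; Firing calls FireProjectile, updates the counter, then plays a right-hand montage and rumbles that controller.
; Reload and drop events detach the BP_JoltGunAmmo magazine into physics, and Drop also destroys the gun.
; Magazine spawning and two-handed grip logic are present but unwired, leaving the second-hand grip event empty.
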(event `self.ReceiveTick`
  (params (DeltaSeconds :type "Float (single-precision)"))
  ;[1 1 1] Delta tick
  (set `self.DeltaSec` DeltaSeconds))

(event `self.ReceiveBeginPlay`
  ;[1 1 1] Begin play
  (set `self.MaxRifleAmmo` 15)
  (bind _output_get (set `self.CurrentRifleAmmo` 0))
  (`TextRenderComponent.K2_SetText` (`self.AmmoCounterForRifle`) (`KismetTextLibrary.Conv_IntToText` _output_get)))

(event `/Game/BluePrint/Weapons/BP_WeaponInteractions.2ndHandGrip`
  ;[1 1 1] 2 handed grip
)

(event `/Game/BluePrint/Weapons/BP_WeaponInteractions.FireWeapon`
  ;[1 1 1] Fire
  (`self.FireProjectile`)
  (`TextRenderComponent.K2_SetText` (`self.AmmoCounterForRifle`) (`KismetTextLibrary.Conv_IntToText` (`self.CurrentRifleAmmo`)))
  (bind _asbp_vrchar_1 (cast `/Game/BluePrint/Players/BP_VRChar1` (`GameplayStatics.GetPlayerCharacter` 0)))
  (`|PlayMontage` (`VRMainCharacter.RightHandMeshSK` _asbp_vrchar_1) "/Game/Characters/Player/Hand/Anims/Old/HandFireAnim_Montage.HandFireAnim_Montage"
    (:`then`
      (`/Game/BluePrint/Players/BP_VRChar1.RumbleController` _asbp_vrchar_1 0.5 "Right"))))

(event `/Game/BluePrint/Weapons/BP_WeaponInteractions.DropAmmo`
  (bind _asbp_jolt_gun_ammo (cast `/Game/BluePrint/Weapons/Ammo/BP_JoltGunAmmo` (`self.AmmoVar`) :!pure true))
  ;[1 1 1] Ammo drop
  (`self.K2_DetachFromActor` (`self.AmmoVar`) "KeepWorld" "KeepWorld" "KeepWorld")
  (`/Game/BluePrint/Weapons/Ammo/BP_JoltGunAmmo.DropTheClip` _asbp_jolt_gun_ammo)
  (`PrimitiveComponent.SetSimulatePhysics` (`/Game/BluePrint/Weapons/Ammo/BP_PistolAmmoMaster.PistolMagMesh` _asbp_jolt_gun_ammo) true)
  (`self.SetLifeSpan` _asbp_jolt_gun_ammo 5.0))

(event `/Game/BluePrint/Weapons/BP_WeaponInteractions.ReloadWeapon`
  (bind _asbp_jolt_gun_ammo (cast `/Game/BluePrint/Weapons/Ammo/BP_JoltGunAmmo` (`self.AmmoVar`) :!pure true))
  ;[1 1 1] Reload weapon
  (set `self.MagInGun` false :!label _label)
  (bind _output_get (set `self.CurrentRifleAmmo` 0))
  (`TextRenderComponent.K2_SetText` (`self.AmmoCounterForRifle`) (`KismetTextLibrary.Conv_IntToText` _output_get))
  (`self.K2_DetachFromActor` (`self.AmmoVar`) "KeepWorld" "KeepWorld" "KeepWorld")
  (`/Game/BluePrint/Weapons/Ammo/BP_JoltGunAmmo.DropTheClip` _asbp_jolt_gun_ammo)
  (`PrimitiveComponent.SetSimulatePhysics` (`/Game/BluePrint/Weapons/Ammo/BP_PistolAmmoMaster.PistolMagMesh` _asbp_jolt_gun_ammo) true))

(event `DropAmmoToReload`
  ;[1 1 1] Reload weapon
  (goto _label))

(event `/Game/BluePrint/Weapons/BP_WeaponInteractions.Drop`
  ;[1 1 1] Drop
  (set `self.PlayerHasGun` false)
  (`/Engine/EditorBlueprintResources/StandardMacros.IsValid` (`self.AmmoVar`)
    (:`Is Valid`
      (`/Game/BluePrint/Weapons/Ammo/BP_JoltGunAmmo.DropTheClip` (cast `/Game/BluePrint/Weapons/Ammo/BP_JoltGunAmmo` (`self.AmmoVar`) :!pure true))
      (`self.DropAmmoToReload`)
      (set `self.AmmoVar` null)
      (`self.K2_DetachFromActor` "KeepWorld" "KeepWorld" "KeepWorld")
      (`self.K2_DestroyActor`))
    (:`Is Not Valid`
      (set `self.Spawned?` false)
      (`self.K2_DetachFromActor` "KeepWorld" "KeepWorld" "KeepWorld")
      (`self.K2_DestroyActor`))))

(fn `UserConstructionScript`
  (`parent.UserConstructionScript`))