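; VR retro pixel rifle that fires projectiles with hand and gun animations, controller rumble and an ammo counter.
; Ammo events spawn and grab BP_RetroAmmo01 clips, ejecting any loaded one, while reloading detaches the clip and zeroes the count.
; Dropping the rifle releases its clip, clears holster state and destroys the actor.
; An overlap-gated two-hand grip macro exists but is unwired, leaving the grip event empty.
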(event `self.ReceiveBeginPlay`
  ;[1 1 1] Begin Play
  (set `self.MaxRifleAmmo` 10)
  (bind _output_get (set `self.CurrentRifleAmmo` 0))
  (`TextRenderComponent.K2_SetText` (`self.AmmoCounterForRifle`) (`KismetTextLibrary.Conv_IntToText` _output_get))
  (bind _asbp_vrchar_1 (cast `/Game/BluePrint/Players/BP_VRChar1` (`GameplayStatics.GetPlayerCharacter` 0)))
  (bind _output_get_2 (set `self.Player` _asbp_vrchar_1))
  (if (`/Game/BluePrint/Players/BP_VRChar1.RetroGunLoadedBefore` _output_get_2)
    (`SceneComponent.SetVisibility` (`self.AmmoTextTut`) false false)))

(event `self.ReceiveTick`
  (params (DeltaSeconds :type "Float (single-precision)"))
  ;[1 1 1] Delta Tick
  (set `self.DeltaSec` DeltaSeconds))

(event `/Game/BluePrint/Weapons/BP_WeaponInteractions.2ndHandGrip`
  ;[1 1 1] 2 handed grip
)

(event `/Game/BluePrint/Weapons/BP_WeaponInteractions.FireWeapon`
  ;[1 1 1] Fire Weapon
  (`self.FireProjectile`)
  (`TextRenderComponent.K2_SetText` (`self.AmmoCounterForRifle`) (`KismetTextLibrary.Conv_IntToText` (`self.CurrentRifleAmmo`)))
  (bind _asbp_vrchar_1 (cast `/Game/BluePrint/Players/BP_VRChar1` (`GameplayStatics.GetPlayerCharacter` 0)))
  (`|PlayMontage` (`VRMainCharacter.RightHandMeshSK` _asbp_vrchar_1) "/Game/Characters/Player/Hand/Anims/Old/HandFireAnim_Montage.HandFireAnim_Montage"
    (:`then`
      (`SkeletalMeshComponent.PlayAnimation` (`self.RifleMesh`) "/Game/ART/WeaponMeshes/Retro/Anim/PixelGun_Fire.PixelGun_Fire" false)
      (`/Game/BluePrint/Players/BP_VRChar1.RumbleController` _asbp_vrchar_1 0.5 "Right"))))

(event `/Game/BluePrint/Weapons/BP_WeaponInteractions.Ammo`
  ;[1 1 1] Spawn Ammo
  (if (`self.MagInGun`)
    (`self.DropAmmoToReload`)
    (bind _ammo (`self.SpawnAndGrabAmmo` "/Game/BluePrint/Weapons/Ammo/BP_RetroAmmo01.BP_RetroAmmo01_C"))
    (bind _asbp_retro_ammo_01 (cast `/Game/BluePrint/Weapons/Ammo/BP_RetroAmmo01` _ammo))
    (set `self.AmmoVar` _asbp_retro_ammo_01)
    (else
      (bind _ammo_2 (`self.SpawnAndGrabAmmo` "/Game/BluePrint/Weapons/Ammo/BP_RetroAmmo01.BP_RetroAmmo01_C"))
      (bind _asbp_retro_ammo_01_2 (cast `/Game/BluePrint/Weapons/Ammo/BP_RetroAmmo01` _ammo_2))
      (set `self.AmmoVar` _asbp_retro_ammo_01_2))))

(event `/Game/BluePrint/Weapons/BP_WeaponInteractions.DropAmmo`
  ;[1 1 1] Drop clip
  (`/Game/BluePrint/Weapons/Ammo/BP_RetroAmmo01.DropTheClip` (cast `/Game/BluePrint/Weapons/Ammo/BP_RetroAmmo01` (`self.AmmoVar`) :!pure true))
  (`self.K2_DetachFromActor` (`self.AmmoVar`) "KeepWorld" "KeepWorld" "KeepWorld"))

(event `/Game/BluePrint/Weapons/BP_WeaponInteractions.ReloadWeapon`
  (bind _asbp_retro_ammo_01 (cast `/Game/BluePrint/Weapons/Ammo/BP_RetroAmmo01` (`self.AmmoVar`) :!pure true))
  ;[1 1 1] Reload Weapon
  (set `self.MagInGun` false :!label _label)
  (bind _output_get (set `self.CurrentRifleAmmo` 0))
  (`TextRenderComponent.K2_SetText` (`self.AmmoCounterForRifle`) (`KismetTextLibrary.Conv_IntToText` _output_get))
  (`self.K2_DetachFromActor` (`self.AmmoVar`) "KeepWorld" "KeepWorld" "KeepWorld")
  (`/Game/BluePrint/Weapons/Ammo/BP_RetroAmmo01.DropTheClip` _asbp_retro_ammo_01)
  (`PrimitiveComponent.SetSimulatePhysics` (`/Game/BluePrint/Weapons/Ammo/BP_PistolAmmoMaster.PistolMagMesh` _asbp_retro_ammo_01) true))

(event `DropAmmoToReload`
  ;[1 1 1] Reload Weapon
  (goto _label))

(event `/Game/BluePrint/Weapons/BP_WeaponInteractions.Drop`
  ;[1 1 1] Drop weapon
  (set `self.PlayerHasGun` false)
  (`/Engine/EditorBlueprintResources/StandardMacros.IsValid` (`self.AmmoVar`)
    (:`Is Valid`
      (set `/Game/BluePrint/Players/BP_VRChar1.RifleHolstered` false (`self.Player`))
      (set `self.RifleHolster?` false)
      (`/Game/BluePrint/Weapons/Ammo/BP_JoltGunAmmo.DropTheClip` (cast `/Game/BluePrint/Weapons/Ammo/BP_RetroAmmo01` (`self.AmmoVar`) :!pure true))
      (`self.DropAmmoToReload`)
      (set `self.AmmoVar` null)
      (`self.K2_DetachFromActor` "KeepWorld" "KeepWorld" "KeepWorld")
      (`self.K2_DestroyActor`))
    (:`Is Not Valid`
      (set `/Game/BluePrint/Players/BP_VRChar1.RifleHolstered` false (`self.Player`))
      (set `self.RifleHolster?` false)
      (set `self.Spawned?` false)
      (`self.K2_DetachFromActor` "KeepWorld" "KeepWorld" "KeepWorld")
      (`self.K2_DestroyActor`))))

(fn `UserConstructionScript`
  (`parent.UserConstructionScript`))