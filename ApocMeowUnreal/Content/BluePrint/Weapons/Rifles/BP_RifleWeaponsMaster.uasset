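; Master Blueprint for VR rifles, handling right-hand pickup, holstering, two-handed aiming and ammo spawning for BP_VRChar1.
; Grab functions and holster events snap the rifle between the character's hand and holster components using overlap checks, updating state flags on both.
; Two-hand grip interpolates rotation toward the left controller, keeping right-hand roll, with speed scaled by left-hand velocity.
; Ammo functions attach new magazines to the character; Grab, Drop and reload events are empty, their old logic disconnected.
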(event `/Game/BluePrint/Weapons/BP_WeaponInteractions.HolsterTheGun`
  (bind _asbp_vrchar_1 (cast `/Game/BluePrint/Players/BP_VRChar1` (`GameplayStatics.GetPlayerCharacter` 0)))
  (if (not (`/Game/BluePrint/Players/BP_VRChar1.RifleHolstered` _asbp_vrchar_1))
    (`SceneComponent.K2_AttachToComponent` (`self.RifleZeroPoint`) (`/Game/BluePrint/Players/BP_VRChar1.RifleHolster` _asbp_vrchar_1) "None" "SnapToTarget" "SnapToTarget" "KeepWorld" true)
    (set `self.RifleHolster?` true)
    (set `/Game/BluePrint/Players/BP_VRChar1.RifleHolstered` true _asbp_vrchar_1)
    (set `/Game/BluePrint/Players/BP_VRChar1.Hand Grips` "NewEnumerator0" _asbp_vrchar_1)))

(event `/Game/BluePrint/Weapons/BP_WeaponInteractions.GrabHolsteredGun`
  (bind _riflezeropoint (`self.RifleZeroPoint`))
  (bind _asbp_vrchar_1 (cast `/Game/BluePrint/Players/BP_VRChar1` (`GameplayStatics.GetPlayerCharacter` 0)))
  (if (`self.PlayerHasGun`)
    (if (`PrimitiveComponent.IsOverlappingComponent` (`VRMainCharacter.RightHandCol` _asbp_vrchar_1) (`/Game/BluePrint/Players/BP_VRChar1.RifleHolsterCol` _asbp_vrchar_1))
      (if (`/Game/BluePrint/Players/BP_VRChar1.RifleHolstered` _asbp_vrchar_1)
        (`SceneComponent.K2_AttachToComponent` _riflezeropoint (`/Game/BluePrint/Players/BP_VRChar1.RifleInHand` _asbp_vrchar_1) "None" "SnapToTarget" "SnapToTarget" "KeepWorld" true)
        (set `self.RifleHolster?` false)
        (set `/Game/BluePrint/Players/BP_VRChar1.RifleHolstered` false _asbp_vrchar_1)
        (else
          (`SceneComponent.K2_AttachToComponent` _riflezeropoint (`/Game/BluePrint/Players/BP_VRChar1.RifleHolster` _asbp_vrchar_1) "None" "SnapToTarget" "SnapToTarget" "KeepWorld" true)
          (set `self.RifleHolster?` true)
          (set `/Game/BluePrint/Players/BP_VRChar1.RifleHolstered` true _asbp_vrchar_1)
          (set `/Game/BluePrint/Players/BP_VRChar1.Hand Grips` "NewEnumerator0" _asbp_vrchar_1))))))

(event `/Game/BluePrint/Weapons/BP_WeaponInteractions.Grab`
  (params (AttachTo :type "SceneComponent Object Reference")))

(event `/Game/BluePrint/Weapons/BP_WeaponInteractions.ReloadWeapon`)

(event `/Game/BluePrint/Weapons/BP_WeaponInteractions.Drop`)

(event `/Game/BluePrint/Weapons/BP_WeaponInteractions.ReloadHip`
  (params (HandIinput :type "/Game/BluePrint/Players/BP_PlayerRightHands Object Reference") (Player :type "/Game/BluePrint/Players/TestNewHandCh Object Reference") (AmmoBox :type "/Game/BluePrint/Players/BP_AmmoSpawn Object Reference")))

(fn `AttachToHand`
  (bind _asbp_vrchar_1 (cast `/Game/BluePrint/Players/BP_VRChar1` (`GameplayStatics.GetPlayerPawn` 0)))
  (if (`PrimitiveComponent.IsOverlappingComponent` (`VRMainCharacter.RightHandCol` _asbp_vrchar_1) (`self.RifleBoxCol`))
    (`self.K2_AttachToComponent` (`/Game/BluePrint/Players/BP_VRChar1.RifleInHand` _asbp_vrchar_1) "None" "SnapToTarget" "SnapToTarget" "KeepWorld")
    (set `self.PlayerHasGun` true)
    (set `/Game/BluePrint/Players/BP_VRChar1.HoldingRifle` true _asbp_vrchar_1)))

(fn `GrabGun`
  (params (HandInput :type "/Game/BluePrint/Players/BP_PlayerRightHands Object Reference"))
  (returns (Ammo :type "Actor Class Reference") (CurrentWeapon :type "/Game/BluePrint/Weapons/Rifles/BP_RifleWeaponsMaster Object Reference"))
  (bind _asbp_vrchar_1 (cast `/Game/BluePrint/Players/BP_VRChar1` (`GameplayStatics.GetPlayerPawn` 0)))
  (if (`PrimitiveComponent.IsOverlappingComponent` (`VRMainCharacter.RightHandCol` _asbp_vrchar_1) (`self.RifleBoxCol`))
    (`self.K2_AttachToComponent` (`/Game/BluePrint/Players/BP_VRChar1.RifleInHand` _asbp_vrchar_1) "None" "SnapToTarget" "SnapToTarget" "KeepWorld")
    (set `self.PlayerHasGun` true)
    (set `/Game/BluePrint/Players/BP_VRChar1.HoldingRifle` true _asbp_vrchar_1)
    (return (`self.AmmoTypeVar`) self)))

(fn `SecondHandGrip`
  (params (DeltaTime :type "Float (double-precision)") (VrChar :type "/Game/BluePrint/Players/BP_VRChar1 Object Reference"))
  (bind _rightmc (`VRMainCharacter.RightMC` VrChar))
  (bind _riflezeropoint (`self.RifleZeroPoint`))
  (bind _lefthandcol (`VRMainCharacter.LeftHandCol` VrChar))
  (bind _returnvalue_roll (`KismetMathLibrary.BreakRotator` (`SceneComponent.K2_GetComponentRotation` _rightmc)))
  (bind (_returnvalue_roll_2 _returnvalue_pitch _returnvalue_yaw) (`KismetMathLibrary.BreakRotator` (`KismetMathLibrary.FindLookAtRotation` (`SceneComponent.K2_GetComponentLocation` _rightmc) (`SceneComponent.K2_GetComponentLocation` (`VRMainCharacter.LeftMC` VrChar)))))
  (bind _returnvalue (`PrimitiveComponent.GetPhysicsLinearVelocity` _lefthandcol "None"))
  (bind _returnvalue_2 (`PrimitiveComponent.GetPhysicsAngularVelocityInDegrees` _lefthandcol "None"))
  (`SceneComponent.K2_SetWorldRotation` _riflezeropoint (`KismetMathLibrary.RInterpTo` (`SceneComponent.K2_GetComponentRotation` _riflezeropoint) (`KismetMathLibrary.MakeRotator` _returnvalue_roll _returnvalue_pitch _returnvalue_yaw) DeltaTime (`KismetMathLibrary.MapRangeUnclamped` (`KismetMathLibrary.VSize` (+ _returnvalue _returnvalue_2)) 0.0 150.0 10.0 20.0)) false false))

(fn `SpawnAmmoAndDropClip`
  (params (Ammo :type "Actor Class Reference") (NewParam :type "/Game/BluePrint/Weapons/Ammo/BP_PistolAmmoMaster Object Reference"))
  (returns (ammotype :type "Actor Object Reference"))
  (`/Game/BluePrint/Weapons/Ammo/BP_PistolAmmoMaster.DropTheClip` NewParam)
  (bind _output_get (set `self.CurrentRifleAmmo` 0))
  (`TextRenderComponent.K2_SetText` (`self.AmmoCounterForRifle`) (`KismetTextLibrary.Conv_IntToText` _output_get))
  (bind _asbp_vrchar_1 (cast `/Game/BluePrint/Players/BP_VRChar1` (`GameplayStatics.GetPlayerCharacter` 0)))
  (bind _ammospawnlocation (`/Game/BluePrint/Players/BP_VRChar1.AmmoSpawnLocation` _asbp_vrchar_1))
  (bind _returnvalue (`|SpawnActorFromClass` Ammo (`SceneComponent.K2_GetComponentToWorld` _ammospawnlocation) "Undefined" "OverrideRootScale" null null))
  (`self.K2_AttachToComponent` _returnvalue _ammospawnlocation "None" "SnapToTarget" "SnapToTarget" "SnapToTarget" true)
  (set `/Game/BluePrint/Players/BP_VRChar1.HoldingAmmo` true _asbp_vrchar_1)
  (return _returnvalue))

(fn `SpawnAndGrabAmmo`
  (params (`Ammo type` :type "Actor Class Reference") (Hand :type "/Game/BluePrint/Players/BP_PlayerRightHands Object Reference"))
  (returns (Ammo :type "Actor Object Reference"))
  (bind _asbp_vrchar_1 (cast `/Game/BluePrint/Players/BP_VRChar1` (`GameplayStatics.GetPlayerCharacter` 0)))
  (bind _ammospawnlocation (`/Game/BluePrint/Players/BP_VRChar1.AmmoSpawnLocation` _asbp_vrchar_1))
  (bind _returnvalue (`|SpawnActorFromClass` `Ammo type` (`SceneComponent.K2_GetComponentToWorld` _ammospawnlocation) "Undefined" "OverrideRootScale" null null))
  (`self.K2_AttachToComponent` _returnvalue _ammospawnlocation "None" "SnapToTarget" "SnapToTarget" "SnapToTarget" true)
  (set `/Game/BluePrint/Players/BP_VRChar1.HoldingAmmo` true _asbp_vrchar_1)
  (return _returnvalue))

(fn `Stop2HandGrip`
  (`SceneComponent.K2_SetWorldRotation` (`self.RifleZeroPoint`) (`self.RifleRot`) false false))

(fn `UserConstructionScript`)