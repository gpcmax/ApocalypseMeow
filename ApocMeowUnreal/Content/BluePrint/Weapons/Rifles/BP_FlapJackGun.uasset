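; VR flapjack rifle Blueprint that handles firing, magazine ejection and dropping, with an on-gun ammo counter.
; Firing spawns a projectile, updates the counter, plays hand and rifle montages, and rumbles the right controller.
; Reload and drop-ammo events detach the magazine and enable its physics, while dropping the gun destroys it.
; DropAmmoToReload jumps into the fire sequence; two-hand grip and ammo-spawning logic are unwired.
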(event `self.ReceiveBeginPlay`
  ;[1 1 1] Begin Play
  (set `self.MaxRifleAmmo` 10)
  (bind _output_get (set `self.CurrentRifleAmmo` 0))
  (`TextRenderComponent.K2_SetText` (`self.AmmoCounterForRifle`) (`KismetTextLibrary.Conv_IntToText` _output_get)))

(event `self.ReceiveTick`
  (params (DeltaSeconds :type "Float (single-precision)"))
  ;[1 1 1] Delta Seconds
  (set `self.DeltaSec` DeltaSeconds))

(event `/Game/BluePrint/Weapons/BP_WeaponInteractions.2ndHandGrip`
  ;[1 1 1] 2 Haned grip
)

(event `/Game/BluePrint/Weapons/BP_WeaponInteractions.FireWeapon`
  ;[1 1 1] Fire weapon
  (`self.FireProjectile` :!label _label)
  (`TextRenderComponent.K2_SetText` (`self.AmmoCounterForRifle`) (`KismetTextLibrary.Conv_IntToText` (`self.CurrentRifleAmmo`)))
  (bind _asbp_vrchar_1 (cast `/Game/BluePrint/Players/BP_VRChar1` (`GameplayStatics.GetPlayerCharacter` 0)))
  (`|PlayMontage` (`VRMainCharacter.RightHandMeshSK` _asbp_vrchar_1) "/Game/Characters/Player/Hand/Anims/Old/HandFireAnim_Montage.HandFireAnim_Montage"
    (:`then`
      (`|PlayMontage` (`self.RifleMesh`) "/Game/ART/WeaponMeshes/Pancake/Anim/flapjackgun_Fire_Montage.flapjackgun_Fire_Montage"
        (:`then`
          (`/Game/BluePrint/Players/BP_VRChar1.RumbleController` _asbp_vrchar_1 0.7 "Right"))))))

(event `DropAmmoToReload`
  ;[1 1 1] Fire weapon
  (goto _label))

(event `/Game/BluePrint/Weapons/BP_WeaponInteractions.DropAmmo`
  (bind _asbp_flap_jack_ammo (cast `/Game/BluePrint/Weapons/Ammo/BP_FlapJackAmmo` (`self.AmmoVar`) :!pure true))
  ;[1 1 1] Drop Ammo
  (`self.K2_DetachFromActor` (`self.AmmoVar`) "KeepWorld" "KeepWorld" "KeepWorld")
  (`/Game/BluePrint/Weapons/Ammo/BP_FlapJackAmmo.FlapjackClip` _asbp_flap_jack_ammo)
  (`PrimitiveComponent.SetSimulatePhysics` (`/Game/BluePrint/Weapons/Ammo/BP_PistolAmmoMaster.PistolMagMesh` _asbp_flap_jack_ammo) true)
  (`self.SetLifeSpan` 5.0))

(event `/Game/BluePrint/Weapons/BP_WeaponInteractions.ReloadWeapon`
  (bind _asbp_flap_jack_ammo (cast `/Game/BluePrint/Weapons/Ammo/BP_FlapJackAmmo` (`self.AmmoVar`) :!pure true))
  ;[1 1 1] Reload Weapon
  (set `self.MagInGun` false)
  (bind _output_get (set `self.CurrentRifleAmmo` 0))
  (`TextRenderComponent.K2_SetText` (`self.AmmoCounterForRifle`) (`KismetTextLibrary.Conv_IntToText` _output_get))
  (`self.K2_DetachFromActor` (`self.AmmoVar`) "KeepWorld" "KeepWorld" "KeepWorld")
  (`/Game/BluePrint/Weapons/Ammo/BP_FlapJackAmmo.FlapjackClip` _asbp_flap_jack_ammo)
  (`PrimitiveComponent.SetSimulatePhysics` (`/Game/BluePrint/Weapons/Ammo/BP_PistolAmmoMaster.PistolMagMesh` _asbp_flap_jack_ammo) true))

(event `/Game/BluePrint/Weapons/BP_WeaponInteractions.Drop`
  ;[1 1 1] Drop Weapon
  (set `self.PlayerHasGun` false)
  (`/Engine/EditorBlueprintResources/StandardMacros.IsValid` (`self.AmmoVar`)
    (:`Is Valid`
      (`/Game/BluePrint/Weapons/Ammo/BP_FlapJackAmmo.FlapjackClip` (cast `/Game/BluePrint/Weapons/Ammo/BP_FlapJackAmmo` (`self.AmmoVar`) :!pure true))
      (`self.DropAmmoToReload`)
      (set `self.AmmoVar` null)
      (`self.K2_DetachFromActor` "KeepWorld" "KeepWorld" "KeepWorld")
      (`self.K2_DestroyActor`))
    (:`Is Not Valid`
      (set `self.Spawned?` false)
      (`self.K2_DetachFromActor` "KeepWorld" "KeepWorld" "KeepWorld")
      (`self.K2_DestroyActor`))))

(fn `UserConstructionScript`
  (`parent.UserConstructionScript`))