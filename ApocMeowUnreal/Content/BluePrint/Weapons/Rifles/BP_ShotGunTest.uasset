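; VR pump-action shotgun weapon with magazine spawning and dropping, two-handed gripping and an ammo counter.
; Pumping reads the left hand's position relative to the player's head: the rear range ejects and re-arms firing, the front range chambers a round.
; Firing requires a chambered round and calls a five-muzzle spread shot.
; A collapsed 2HandNode toggles two-handed aim from left-hand overlap; dropping the gun releases any magazine and destroys the actor.
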(event `/Game/BluePrint/Weapons/BP_WeaponInteractions.ReloadWeapon`
  ;[1 1 1] Handle Reload weapon
  (set `self.MagInGun` false :!label _label)
  (bind _output_get (set `self.CurrentRifleAmmo` 0))
  (`TextRenderComponent.K2_SetText` (`self.AmmoCounterForRifle`) (`KismetTextLibrary.Conv_IntToText` _output_get))
  (`self.K2_DetachFromActor` (`self.AmmoVar`) "KeepWorld" "KeepWorld" "KeepWorld")
  (`/Game/BluePrint/Weapons/Ammo/BP_ShotGunMag.DropTheShotGunMag` (cast `/Game/BluePrint/Weapons/Ammo/BP_ShotGunMag` (`self.AmmoVar`) :!pure true)))

(event `DropAmmoToReload`
  ;[1 1 1] Handle Reload weapon
  (goto _label))

(event `/Game/BluePrint/Weapons/BP_WeaponInteractions.Drop`
  ;[1 1 1] Handles weapon drop
  (set `self.PlayerHasGun` false)
  (`/Engine/EditorBlueprintResources/StandardMacros.IsValid` (`self.AmmoVar`)
    (:`Is Valid`
      (set `/Game/BluePrint/Players/BP_VRChar1.RifleHolstered` false (`self.PLayer`))
      (set `self.RifleHolster?` false)
      (`self.K2_DetachFromActor` (`self.AmmoVar`) "KeepWorld" "KeepWorld" "KeepWorld")
      (`/Game/BluePrint/Weapons/Ammo/BP_ShotGunMag.DropTheShotGunMag` (cast `/Game/BluePrint/Weapons/Ammo/BP_ShotGunMag` (`self.AmmoVar`) :!pure true))
      (set `self.AmmoVar` null)
      (`self.K2_DetachFromActor` "KeepWorld" "KeepWorld" "KeepWorld")
      (`self.K2_DestroyActor`))
    (:`Is Not Valid`
      (set `/Game/BluePrint/Players/BP_VRChar1.RifleHolstered` false (`self.PLayer`))
      (set `self.RifleHolster?` false)
      (set `self.Spawned?` false)
      (`self.K2_DetachFromActor` "KeepWorld" "KeepWorld" "KeepWorld")
      (`self.K2_DestroyActor`))))

(event `self.ReceiveBeginPlay`
  ;[1 1 1] Event begin play
  (set `self.MaxRifleAmmo` 10)
  (bind _output_get (set `self.CurrentRifleAmmo` 0))
  (`TextRenderComponent.K2_SetText` (`self.AmmoCounterForRifle`) (`KismetTextLibrary.Conv_IntToText` _output_get))
  (bind _asbp_vrchar_1 (cast `/Game/BluePrint/Players/BP_VRChar1` (`GameplayStatics.GetPlayerPawn` 0)))
  (bind _output_get_2 (set `self.PLayer` _asbp_vrchar_1))
  (`SceneComponent.SetVisibility` (`self.PumpTut`) false false)
  (if (`/Game/BluePrint/Players/BP_VRChar1.ShotGunLoadedBefore` _output_get_2)
    (`SceneComponent.SetVisibility` (`self.PumpTut`) false false)
    (`SceneComponent.SetVisibility` (`self.LoadRoundText`) false false)))

(event `self.ReceiveTick`
  (params (DeltaSeconds :type "Float (single-precision)"))
  ;[1 1 1] Sets delta sec
  (set `self.DeltaSec` DeltaSeconds))

(event `/Game/BluePrint/Weapons/BP_WeaponInteractions.2ndHandGrip`
  ;[1 1 1] 2 Handed Grip
  (bind _asbp_vrchar_1 (cast `/Game/BluePrint/Players/BP_VRChar1` (`GameplayStatics.GetPlayerCharacter` 0)))
  (if (`PrimitiveComponent.IsOverlappingComponent` (`self.SecondHandCol`) (`VRMainCharacter.LeftHandCol` _asbp_vrchar_1))
    (`/Engine/EditorBlueprintResources/StandardMacros.Gate` true :!via `Open` :!label _label_2
      (:`Exit`
        (`self.SecondHandGrip` (`self.DeltaSec`) _asbp_vrchar_1)
        (set `self.2HandedMode` true)))
    (else
      (set `self.2HandedMode` false :!label _label_3)
      (`self.Stop2HandGrip`)
      (goto _label_2 :!via `Close`))))

(event `/Game/BluePrint/Weapons/BP_WeaponInteractions.Stop2Hand`
  (goto _label_3))

(event `/Game/BluePrint/Weapons/BP_WeaponInteractions.FireWeapon`
  ;[1 1 1] Fire
  (switch `/Game/BluePrint/ENUMs/ShotGunStates` (`self.ShotGunState`)
    (:`NewEnumerator0`
      (`/Engine/EditorBlueprintResources/StandardMacros.DoOnce` false :!label _label_4
        (:`Completed`
          (`self.FireSpreadShot` (`self.Muzzle01`) (`self.Muzzle02`) (`self.Muzzle03`) (`self.Muzzle04`) (`self.Muzzle05`))
          (`TextRenderComponent.K2_SetText` (`self.AmmoCounterForRifle`) (`KismetTextLibrary.Conv_IntToText` (`self.CurrentRifleAmmo`)))
          (set `self.ShotGunState` "NewEnumerator1"))))))

(event `ExpellRound`
  ;[1 1 1] Fire
  (goto _label_4 :!via `Reset`))

(event `/Game/BluePrint/Weapons/BP_WeaponInteractions.Ammo`
  ;[1 1 1] Spawns Ammo
  (if (`self.MagInGun`)
    (set `self.MagInGun` false)
    (bind _output_get (set `self.CurrentRifleAmmo` 0))
    (`TextRenderComponent.K2_SetText` (`self.AmmoCounterForRifle`) (`KismetTextLibrary.Conv_IntToText` _output_get))
    (`self.K2_DetachFromActor` (`self.AmmoVar`) "KeepWorld" "KeepWorld" "KeepWorld")
    (`/Game/BluePrint/Weapons/Ammo/BP_ShotGunMag.DropTheShotGunMag` (cast `/Game/BluePrint/Weapons/Ammo/BP_ShotGunMag` (`self.AmmoVar`) :!pure true))
    (bind _ammo (`self.SpawnAndGrabAmmo` "/Game/BluePrint/Weapons/Ammo/BP_ShotGunMag.BP_ShotGunMag_C"))
    (bind _asbp_shot_gun_mag (cast `/Game/BluePrint/Weapons/Ammo/BP_ShotGunMag` _ammo))
    (set `self.AmmoVar` _asbp_shot_gun_mag)
    (else
      (bind _ammo_2 (`self.SpawnAndGrabAmmo` "/Game/BluePrint/Weapons/Ammo/BP_ShotGunMag.BP_ShotGunMag_C"))
      (bind _asbp_shot_gun_mag_2 (cast `/Game/BluePrint/Weapons/Ammo/BP_ShotGunMag` _ammo_2))
      (set `self.AmmoVar` _asbp_shot_gun_mag_2))))

(event `/Game/BluePrint/Weapons/BP_WeaponInteractions.DropAmmo`
  ;[1 1 1] Drops ammo
  (`self.K2_DetachFromActor` (`self.AmmoVar`) "KeepWorld" "KeepWorld" "KeepWorld")
  (`/Game/BluePrint/Weapons/Ammo/BP_ShotGunMag.DropTheShotGunMag` (cast `/Game/BluePrint/Weapons/Ammo/BP_ShotGunMag` (`self.AmmoVar`) :!pure true)))

(event `self.Box.OnComponentBeginOverlap`
  (params (OverlappedComponent :type "PrimitiveComponent Object Reference") (OtherActor :type "Actor Object Reference") (OtherComp :type "PrimitiveComponent Object Reference") (OtherBodyIndex :type Integer) (bFromSweep :type Boolean) (SweepResult :type "HitResult Structure (by ref)"))
  ;[1 1 1] Can pump overlap
  (bind _asbp_vrchar_1 (cast `/Game/BluePrint/Players/BP_VRChar1` OtherActor))
  (if (`PrimitiveComponent.IsOverlappingComponent` (`VRMainCharacter.LeftHandCol` _asbp_vrchar_1) (`self.Box`))
    (set `self.CanPump` true)
    (else
      (set `self.CanPump` false))))

(event `Key|MotionController_Left_Trigger`
  (params (Key :type "Key Structure"))
  ;[1 1 1] Old
)

(event `/Game/BluePrint/Weapons/BP_WeaponInteractions.Pump`
  (bind _player (`self.PLayer`))
  (bind _returnvalue_x (`KismetMathLibrary.BreakVector` (`VictoryBPFunctionLibrary.GetComponentRelativeLocation` (`/Game/BluePrint/Players/BP_VRChar1.playerHead` _player) (`VRMainCharacter.LeftHandCol` _player))))
  ;[1 1 1] Pump gun
  (if (`self.CanPump`)
    (`/Engine/EditorBlueprintResources/StandardMacros.Gate` true :!via `Open` :!label _label_5
      (:`Exit`
        (bind _output_get (set `self.PumpLoc` (`KismetMathLibrary.MakeVector` 0.0 0.0 _returnvalue_x)))
        ;[1 1 1] Checks ammo
        (if (> (`self.CurrentRifleAmmo`) 0)
          (`|ExecutionSequence`
            (:`then_0`
              (bind _returnvalue (`KismetMathLibrary.FClamp` (.z _output_get) 47.979282 70.0))
              ;[1 1 1] Checks pump location. If at base ejects round
              (if (`KismetMathLibrary.InRange_FloatFloat` _returnvalue 45.0 55.0)
                (set `self.ShotGunState` "NewEnumerator2")
                (`self.ExpellRound`)))
            (:`then_1`
              ;[1 1 1] Checks pump location. if at front than loads a round
              (if (`KismetMathLibrary.InRange_FloatFloat` _returnvalue 57.25 70.0)
                (if (not (`self.Fired`))
                  (set `self.ShotGunState` "NewEnumerator0")
                  (`/Engine/EditorBlueprintResources/StandardMacros.DoOnce` false
                    (:`Completed`
                      (`SceneComponent.SetVisibility` (`self.PumpTut`) false false))))))))))
    (else
      (goto _label_5 :!via `Close`))))

(event `/Game/BluePrint/Weapons/BP_WeaponInteractions.StopPump`
  ;[1 1 1] Pump gun
  (goto _label_5 :!via `Close`))

(fn `UserConstructionScript`
  (bind _riflemesh (`self.RifleMesh`))
  (`parent.UserConstructionScript`)
  (`SceneComponent.K2_AttachToComponent` (`self.SecondHandCol`) (`self.RifleMesh`) "SK_Wep_Shotgun_Pump_01" "SnapToTarget" "SnapToTarget" "KeepRelative" true)
  (`SceneComponent.K2_AttachToComponent` (`self.PumpTut`) _riflemesh "Pump" "KeepRelative" "KeepRelative" "KeepRelative" true)
  (`SceneComponent.K2_AttachToComponent` (`self.LoadRoundText`) _riflemesh "Pump" "KeepRelative" "KeepRelative" "KeepRelative" true))