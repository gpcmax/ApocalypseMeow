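; BP_ShotGunMag1 is a shotgun magazine for the VR character that loads into BP_ShotGunTest on contact.
; When its ammo box collision overlaps the shotgun, it calls AttachToRifle with the gun, player pawn and MagLoc socket.
; DropTheShotGunMag turns on mesh physics, disables that collision, clears the player's MagWentIn flag and sets a short lifespan.
; DropAmmo and BeginPlay are empty.
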(event `self.AmmoBoxColl.OnComponentBeginOverlap`
  (params (OverlappedComponent :type "PrimitiveComponent Object Reference") (OtherActor :type "Actor Object Reference") (OtherComp :type "PrimitiveComponent Object Reference") (OtherBodyIndex :type Integer) (bFromSweep :type Boolean) (SweepResult :type "HitResult Structure (by ref)"))
  (bind _asbp_shot_gun_test (cast `/Game/BluePrint/Weapons/Rifles/BP_ShotGunTest` OtherActor))
  (bind _asbp_vrchar_1 (cast `/Game/BluePrint/Players/BP_VRChar1` (`GameplayStatics.GetPlayerPawn` 0)))
  (`self.AttachToRifle` _asbp_shot_gun_test _asbp_vrchar_1 "MagLoc"))

(event `self.ReceiveBeginPlay`)

(event `/Game/BluePrint/Weapons/BP_WeaponInteractions.DropAmmo`)

(event `DropTheShotGunMag`
  (`PrimitiveComponent.SetSimulatePhysics` (`self.PistolMagMesh`) true)
  (`PrimitiveComponent.SetCollisionEnabled` (`self.AmmoBoxColl`) "NoCollision")
  (bind _asbp_vrchar_1 (cast `/Game/BluePrint/Players/BP_VRChar1` (`GameplayStatics.GetPlayerPawn` 0)))
  (set `/Game/BluePrint/Players/BP_VRChar1.MagWentIn` false _asbp_vrchar_1)
  (`self.SetLifeSpan` 10.0))

(fn `UserConstructionScript`
  (`parent.UserConstructionScript`))