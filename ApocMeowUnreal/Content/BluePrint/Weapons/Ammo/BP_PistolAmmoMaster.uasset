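; Base magazine actor for a VR game that reloads a gun when its collision box overlaps the gun's ammo box.
; AttachToRifle refills an empty gun, updates its ammo counter and player flags, and snaps the mag to a bone socket or MagLoc; in shotgun mode it adds one round and destroys itself.
; NewAttach repeats the non-shotgun path without player flags and disables collision.
; DropTheClip enables physics, clears MagWentIn and expires the mag.
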(event `DropTheClip`
  (`PrimitiveComponent.SetSimulatePhysics` (`self.PistolMagMesh`) true)
  (`PrimitiveComponent.SetCollisionEnabled` (`self.AmmoBoxColl`) "NoCollision")
  (bind _asbp_vrchar_1 (cast `/Game/BluePrint/Players/BP_VRChar1` (`GameplayStatics.GetPlayerPawn` 0)))
  (set `/Game/BluePrint/Players/BP_VRChar1.MagWentIn` false _asbp_vrchar_1)
  (`self.SetLifeSpan` 10.0))

(fn `AttachToRifle`
  (params (RifleActor :type "/Game/BluePrint/Weapons/Rifles/BP_RifleWeaponsMaster Object Reference") (PlayerRef :type "/Game/BluePrint/Players/BP_VRChar1 Object Reference") (SocketLocation :type Name) (HasSkelMeshWithJoint :type Boolean) (ShotGun :type Boolean))
  (locals (Rifle :type "/Game/BluePrint/Weapons/Rifles/BP_RifleWeaponsMaster Object Reference") (Player :type "/Game/BluePrint/Players/BP_VRChar1 Object Reference") (IsShotty :type Boolean) (HasBone :type Boolean))
  (bind _player (`local.Player`))
  (bind _rifle (`local.Rifle`))
  (bind _rifle_2 (`local.Rifle`))
  (bind _rifle_3 (`local.Rifle`))
  (bind _magzeropoint (`self.MagZeroPoint`))
  (bind _player_2 (`local.Player`))
  (bind _output_get (set `local.Rifle` RifleActor))
  (set `local.Player` PlayerRef)
  (set `local.IsShotty` ShotGun)
  (set `local.HasBone` HasSkelMeshWithJoint)
  (if (`/Game/BluePrint/Weapons/Rifles/BP_RifleWeaponsMaster.MagInGun` _output_get)
    _
    (elif (`PrimitiveComponent.IsOverlappingComponent` (`/Game/BluePrint/Weapons/Rifles/BP_RifleWeaponsMaster.AmmoBox` (`local.Rifle`)) (`self.AmmoBoxColl`))
      (if (`local.IsShotty`)
        (if (== (`RifleWeaponsMaster.CurrentRifleAmmo` _rifle_3) (`RifleWeaponsMaster.MaxRifleAmmo` _rifle_3))
          (set `/Game/BluePrint/Weapons/Rifles/BP_RifleWeaponsMaster.MagInGun` false (`local.Rifle`))
          (set `/Game/BluePrint/Players/BP_VRChar1.HoldingAmmo` true _player_2)
          (set `/Game/BluePrint/Players/BP_VRChar1.MagWentIn` false _player_2)
          (else
            (bind _output_get_2 (set `RifleWeaponsMaster.CurrentRifleAmmo` (+ (`RifleWeaponsMaster.CurrentRifleAmmo` _rifle_2) 1) _rifle_2))
            (`TextRenderComponent.K2_SetText` (`RifleWeaponsMaster.AmmoCounterForRifle` _rifle_2) (`KismetTextLibrary.Conv_IntToText` _output_get_2))
            (`self.K2_DestroyActor`)))
        (else
          (set `/Game/BluePrint/Weapons/Rifles/BP_RifleWeaponsMaster.MagInGun` true (`local.Rifle`))
          (set `/Game/BluePrint/Players/BP_VRChar1.HoldingAmmo` false _player)
          (set `/Game/BluePrint/Players/BP_VRChar1.MagWentIn` true _player)
          (bind _output_get_3 (set `RifleWeaponsMaster.CurrentRifleAmmo` (`RifleWeaponsMaster.MaxRifleAmmo` _rifle) _rifle))
          (`TextRenderComponent.K2_SetText` (`RifleWeaponsMaster.AmmoCounterForRifle` _rifle) (`KismetTextLibrary.Conv_IntToText` _output_get_3))
          (if (`local.HasBone`)
            (`SceneComponent.K2_AttachToComponent` _magzeropoint (`RifleWeaponsMaster.RifleMesh` (`local.Rifle`)) SocketLocation "SnapToTarget" "SnapToTarget" "KeepWorld" true)
            (else
              (`SceneComponent.K2_AttachToComponent` _magzeropoint (`RifleWeaponsMaster.MagLoc` _rifle) "None" "SnapToTarget" "SnapToTarget" "KeepWorld" true))))))))

(fn `GrabGun`
  (params (HandInput :type "/Game/BluePrint/Players/BP_PlayerRightHands Object Reference"))
  (returns (Ammo :type "Actor Class Reference") (CurrentWeapon :type "/Game/BluePrint/Weapons/Rifles/BP_RifleWeaponsMaster Object Reference"))
  (return null null))

(fn `NewAttach`
  (params (RifleActor :type "/Game/BluePrint/Weapons/Rifles/BP_RifleWeaponsMaster Object Reference") (PlayerRef :type "/Game/BluePrint/Players/BP_PlayerRightHands Object Reference") (SocketLocation :type Name) (HasSkelJoint :type Boolean) (Shotgun :type Boolean))
  (locals (Rifle :type "/Game/BluePrint/Weapons/Rifles/BP_RifleWeaponsMaster Object Reference") (PlayerHand :type "/Game/BluePrint/Players/BP_PlayerRightHands Object Reference") (Shotty :type Boolean) (HasBone :type Boolean) (SocketName :type Name))
  (bind _rifle (`local.Rifle`))
  (set `local.Rifle` RifleActor)
  (set `local.PlayerHand` PlayerRef)
  (set `local.Shotty` Shotgun)
  (set `local.SocketName` SocketLocation)
  (set `local.HasBone` HasSkelJoint)
  (if (`/Game/BluePrint/Weapons/Rifles/BP_RifleWeaponsMaster.MagInGun` (`local.Rifle`))
    _
    (elif (`PrimitiveComponent.IsOverlappingComponent` (`/Game/BluePrint/Weapons/Rifles/BP_RifleWeaponsMaster.AmmoBox` (`local.Rifle`)) (`self.AmmoBoxColl`))
      (if (not (`local.Shotty`))
        (set `/Game/BluePrint/Weapons/Rifles/BP_RifleWeaponsMaster.MagInGun` true (`local.Rifle`))
        (bind _output_get (set `RifleWeaponsMaster.CurrentRifleAmmo` (`RifleWeaponsMaster.MaxRifleAmmo` _rifle) _rifle))
        (`TextRenderComponent.K2_SetText` (`RifleWeaponsMaster.AmmoCounterForRifle` _rifle) (`KismetTextLibrary.Conv_IntToText` _output_get))
        (if (`local.HasBone`)
          (`SceneComponent.K2_AttachToComponent` (`self.MagZeroPoint`) (`RifleWeaponsMaster.RifleMesh` (`local.Rifle`)) (`local.SocketName`) "SnapToTarget" "SnapToTarget" "KeepWorld" true)
          (`PrimitiveComponent.SetCollisionEnabled` (`self.AmmoBoxColl`) "NoCollision")
          (else
            (`SceneComponent.K2_AttachToComponent` (`self.MagZeroPoint`) (`RifleWeaponsMaster.MagLoc` (`local.Rifle`)) "None" "SnapToTarget" "SnapToTarget" "KeepWorld" true)
            (`PrimitiveComponent.SetCollisionEnabled` (`self.AmmoBoxColl`) "NoCollision")))))))

(fn `Reload`)

(fn `UserConstructionScript`)