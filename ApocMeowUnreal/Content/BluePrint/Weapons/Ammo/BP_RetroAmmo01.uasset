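; BP_RetroAmmo01 is a VR magazine pickup that loads the BP_PixelUpdated retro gun.
; When its collider overlaps the gun, it calls AttachToRifle with the gun and BP_VRChar1 pawn, then hides the gun's tutorial text on the first load.
; DropTheClip enables mesh physics, disables collision, clears the player's MagWentIn flag and sets a lifespan so the dropped clip despawns.
; Older inline attach-and-refill logic remains unconnected.
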(event `self.AmmoBoxColl.OnComponentBeginOverlap`
  (params (OverlappedComponent :type "PrimitiveComponent Object Reference") (OtherActor :type "Actor Object Reference") (OtherComp :type "PrimitiveComponent Object Reference") (OtherBodyIndex :type Integer) (bFromSweep :type Boolean) (SweepResult :type "HitResult Structure (by ref)"))
  (bind _asbp_pixel_updated (cast `/Game/BluePrint/Weapons/Rifles/BP_PixelUpdated` OtherActor))
  (bind _asbp_vrchar_1 (cast `/Game/BluePrint/Players/BP_VRChar1` (`GameplayStatics.GetPlayerPawn` 0)))
  (`self.AttachToRifle` _asbp_pixel_updated _asbp_vrchar_1)
  (if (not (`/Game/BluePrint/Players/BP_VRChar1.RetroGunLoadedBefore` _asbp_vrchar_1))
    (`SceneComponent.SetVisibility` (`/Game/BluePrint/Weapons/Rifles/BP_PixelUpdated.AmmoTextTut` _asbp_pixel_updated) false false)
    (set `/Game/BluePrint/Players/BP_VRChar1.RetroGunLoadedBefore` true _asbp_vrchar_1)))

(event `self.ReceiveBeginPlay`)

(event `/Game/BluePrint/Weapons/BP_WeaponInteractions.DropAmmo`)

(event `DropTheClip`
  (`PrimitiveComponent.SetSimulatePhysics` (`self.PistolMagMesh`) true)
  (`PrimitiveComponent.SetCollisionEnabled` (`self.AmmoBoxColl`) "NoCollision")
  (bind _asbp_vrchar_1 (cast `/Game/BluePrint/Players/BP_VRChar1` (`GameplayStatics.GetPlayerPawn` 0)))
  (set `/Game/BluePrint/Players/BP_VRChar1.MagWentIn` false _asbp_vrchar_1)
  (`self.SetLifeSpan` 10.0))

(fn `UserConstructionScript`
  (`parent.UserConstructionScript`))