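; BP_SharkAmmo is a magazine for the SharkShot gun that reloads it in VR.
; When its box overlaps the AmmoBox of a gun without a magazine, it snaps onto the gun, refills and displays ammo, and updates the VR character's state.
; The first load also hides the gun's tutorial text.
; DropTheClip enables mesh physics, disables box collision, clears the inserted flag and expires the actor after a short lifespan.
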(event `self.AmmoBoxColl.OnComponentBeginOverlap`
  (params (OverlappedComponent :type "PrimitiveComponent Object Reference") (OtherActor :type "Actor Object Reference") (OtherComp :type "PrimitiveComponent Object Reference") (OtherBodyIndex :type Integer) (bFromSweep :type Boolean) (SweepResult :type "HitResult Structure (by ref)"))
  (bind _asbp_shark_shot (cast `/Game/BluePrint/Weapons/Rifles/BP_SharkShot` OtherActor))
  (bind _asbp_vrchar_1 (cast `/Game/BluePrint/Players/BP_VRChar1` (`GameplayStatics.GetPlayerPawn` 0)))
  (if (`/Game/BluePrint/Weapons/Rifles/BP_RifleWeaponsMaster.MagInGun` _asbp_shark_shot)
    _
    (elif (`PrimitiveComponent.IsOverlappingComponent` (`/Game/BluePrint/Weapons/Rifles/BP_RifleWeaponsMaster.AmmoBox` _asbp_shark_shot) (`self.AmmoBoxColl`))
      (set `/Game/BluePrint/Weapons/Rifles/BP_SharkShot.EReload` "NewEnumerator1" _asbp_shark_shot)
      (set `/Game/BluePrint/Weapons/Rifles/BP_RifleWeaponsMaster.MagInGun` true _asbp_shark_shot)
      (set `/Game/BluePrint/Players/BP_VRChar1.HoldingAmmo` false _asbp_vrchar_1)
      (set `/Game/BluePrint/Players/BP_VRChar1.MagWentIn` true _asbp_vrchar_1)
      (bind _output_get (set `RifleWeaponsMaster.CurrentRifleAmmo` (`RifleWeaponsMaster.MaxRifleAmmo` _asbp_shark_shot) _asbp_shark_shot))
      (`TextRenderComponent.K2_SetText` (`RifleWeaponsMaster.AmmoCounterForRifle` _asbp_shark_shot) (`KismetTextLibrary.Conv_IntToText` _output_get))
      (`SceneComponent.K2_AttachToComponent` (`self.MagZeroPoint`) (`/Game/BluePrint/Weapons/Rifles/BP_SharkShot.SharkShotMag` _asbp_shark_shot) "None" "SnapToTarget" "SnapToTarget" "KeepWorld" true)
      (set `/Game/BluePrint/Weapons/Rifles/BP_SharkShot.EReload` "NewEnumerator1" _asbp_shark_shot)
      (if (not (`/Game/BluePrint/Players/BP_VRChar1.SharkShotGunLoadedBefore` _asbp_vrchar_1))
        (`SceneComponent.SetVisibility` (`/Game/BluePrint/Weapons/Rifles/BP_SharkShot.AmmoTextTut` _asbp_shark_shot) false false)
        (set `/Game/BluePrint/Players/BP_VRChar1.SharkShotGunLoadedBefore` true _asbp_vrchar_1)))))

(event `self.ReceiveBeginPlay`)

(event `DropTheClip`
  (`PrimitiveComponent.SetSimulatePhysics` (`self.PistolMagMesh`) true)
  (`PrimitiveComponent.SetCollisionEnabled` (`self.AmmoBoxColl`) "NoCollision")
  (bind _asbp_vrchar_1 (cast `/Game/BluePrint/Players/BP_VRChar1` (`GameplayStatics.GetPlayerPawn` 0)))
  (set `/Game/BluePrint/Players/BP_VRChar1.MagWentIn` false _asbp_vrchar_1)
  (`self.SetLifeSpan` 10.0))

(fn `UserConstructionScript`
  (`parent.UserConstructionScript`))