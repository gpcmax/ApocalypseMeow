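; BP_JoltGunAmmo is the magazine for the Jolt Gun, used by the VR player character.
; When its collision box overlaps a BP_JoltGun, it calls AttachToRifle with that gun and the player pawn.
; DropTheClip turns on mesh physics, disables the box collision, clears the player's MagWentIn flag and sets a short lifespan for cleanup.
; BeginPlay and DropAmmo are empty.
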(event `self.AmmoBoxColl.OnComponentBeginOverlap`
  (params (OverlappedComponent :type "PrimitiveComponent Object Reference") (OtherActor :type "Actor Object Reference") (OtherComp :type "PrimitiveComponent Object Reference") (OtherBodyIndex :type Integer) (bFromSweep :type Boolean) (SweepResult :type "HitResult Structure (by ref)"))
  (bind _asbp_jolt_gun (cast `/Game/BluePrint/Weapons/Rifles/BP_JoltGun` OtherActor))
  (bind _asbp_vrchar_1 (cast `/Game/BluePrint/Players/BP_VRChar1` (`GameplayStatics.GetPlayerPawn` 0)))
  (`self.AttachToRifle` _asbp_jolt_gun _asbp_vrchar_1))

(event `self.ReceiveBeginPlay`)

(event `/Game/BluePrint/Weapons/BP_WeaponInteractions.DropAmmo`)

(event `DropTheClip`
  (`PrimitiveComponent.SetSimulatePhysics` (`self.PistolMagMesh`) true)
  (`PrimitiveComponent.SetCollisionEnabled` (`self.AmmoBoxColl`) "NoCollision")
  (bind _asbp_vrchar_1 (cast `/Game/BluePrint/Players/BP_VRChar1` (`GameplayStatics.GetPlayerPawn` 0)))
  (set `/Game/BluePrint/Players/BP_VRChar1.MagWentIn` false _asbp_vrchar_1)
  (`self.SetLifeSpan` 10.0))

(fn `UserConstructionScript`
  (`parent.UserConstructionScript`))