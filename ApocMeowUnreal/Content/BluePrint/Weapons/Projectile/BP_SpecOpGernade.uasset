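; Spec Ops grenade projectile that explodes two seconds after its collision component registers a hit.
; The blast spawns a particle effect above the bullet mesh, plays an explosion sound and applies full, non-falloff radial damage before destroying the actor.
; All Van actors are excluded from the damage.
; The sphere overlap event is empty, and leftover attach-to-AI, damage-over-time and timed-detach nodes are disconnected.
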(event `self.Sphere.OnComponentBeginOverlap`
  (params (OverlappedComponent :type "PrimitiveComponent Object Reference") (OtherActor :type "Actor Object Reference") (OtherComp :type "PrimitiveComponent Object Reference") (OtherBodyIndex :type Integer) (bFromSweep :type Boolean) (SweepResult :type "HitResult Structure (by ref)")))

(event `self.CollisionComponent.OnComponentHit`
  (params (HitComponent :type "PrimitiveComponent Object Reference") (OtherActor :type "Actor Object Reference") (OtherComp :type "PrimitiveComponent Object Reference") (NormalImpulse :type "Vector Structure") (Hit :type "HitResult Structure (by ref)"))
  (bind _returnvalue (`SceneComponent.K2_GetComponentLocation` (`self.BulletMesh`)))
  (`KismetSystemLibrary.Delay` 2.0)
  (bind _outactors (`GameplayStatics.GetAllActorsOfClass` "/Game/BluePrint/VanAndPups/Van.Van_C"))
  (`GameplayStatics.SpawnEmitterAtLocation` "/Game/ART/Effects_2/Particle/p_gRENADE.p_gRENADE" (+ _returnvalue (0.0 0.0 100.0)))
  (`GameplayStatics.PlaySoundAtLocation` "/Game/Audio/Explosive/Explosive_Cue.Explosive_Cue" _returnvalue)
  (`GameplayStatics.ApplyRadialDamage` 50.0 (`SceneComponent.K2_GetComponentLocation` (`self.CollisionComponent`)) 1000.0 "/Script/Engine.DamageType" _outactors self null true)
  (`self.K2_DestroyActor`))

(fn `UserConstructionScript`)