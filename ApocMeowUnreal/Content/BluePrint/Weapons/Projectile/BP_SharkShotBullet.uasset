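; Shark projectile weapon bullet that latches onto AI characters and deals damage over time.
; BeginPlay turns off physics simulation below two shark bones while setting their blend weight to full.
; Sphere overlap attaches the bullet mesh to the victim, disables the sphere's collision and plays a timeline that calls HurtAi each update with a shark flag.
; After the timeline and a delay, it detaches and expires; the component hit event is empty.
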(event `self.ReceiveBeginPlay`
  (bind _bone02 (`self.Bone02`))
  (`|ExecutionSequence`
    (:`then_0`
      (`SkeletalMeshComponent.SetAllBodiesBelowSimulatePhysics` (`self.sharkprojectile`) (`self.Bone01`) false false)
      (`SkeletalMeshComponent.SetAllBodiesBelowPhysicsBlendWeight` (`self.sharkprojectile`) (`self.Bone01`) 1.0 false false))
    (:`then_1`
      (`SkeletalMeshComponent.SetAllBodiesBelowSimulatePhysics` (`self.sharkprojectile`) _bone02 false false)
      (`SkeletalMeshComponent.SetAllBodiesBelowPhysicsBlendWeight` (`self.sharkprojectile`) _bone02 1.0 false false))))

(event `self.CollisionComponent.OnComponentHit`
  (params (HitComponent :type "PrimitiveComponent Object Reference") (OtherActor :type "Actor Object Reference") (OtherComp :type "PrimitiveComponent Object Reference") (NormalImpulse :type "Vector Structure") (Hit :type "HitResult Structure (by ref)")))

(event `self.Sphere.OnComponentBeginOverlap`
  (params (OverlappedComponent :type "PrimitiveComponent Object Reference") (OtherActor :type "Actor Object Reference") (OtherComp :type "PrimitiveComponent Object Reference") (OtherBodyIndex :type Integer) (bFromSweep :type Boolean) (SweepResult :type "HitResult Structure (by ref)"))
  (bind _asbp_ai_character (cast `/Game/BluePrint/AI/BP_AI_Character` OtherActor))
  (`SceneComponent.K2_AttachToComponent` (`self.BulletMesh`) (`Character.Mesh` _asbp_ai_character) "None" "KeepWorld" "KeepWorld" "KeepWorld" false)
  (`PrimitiveComponent.SetCollisionEnabled` (`self.Sphere`) "NoCollision")
  (bind (_direction _hurt) (`Timeline|DamageOverTime`)
    (:`Update`
      (`AI_Character.HurtAi` _asbp_ai_character _hurt true))
    (:`Finished`
      (`KismetSystemLibrary.Delay` 5.0)
      (`self.K2_DetachFromActor` "KeepWorld" "KeepWorld" "KeepWorld")
      (`self.SetLifeSpan` 3.0))))

(fn `UserConstructionScript`)