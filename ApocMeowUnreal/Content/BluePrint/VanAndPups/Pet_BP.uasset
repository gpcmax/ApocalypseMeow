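; Pet actor for the van game: a randomly skinned cat or puppy that can fall from the van and be grabbed by enemies.
; The construction script picks a random mesh, flags puppies and applies a matching random material.
; Detaching teleports it to a fixed spot, enables physics and cries; if still fallen after a minute, it asks the van to spawn a new pet.
; Enemy pickup disables physics and collision and clears the fallen state.
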(event `Dropped`
  ;[1 1 1] Dropped
  (`/Game/BluePrint/VanAndPups/Van.Spawn New Pet` (`self.Van`) (`self.ID`) self)
  (`GameplayStatics.PlaySound2D` "/Game/Audio/KittenNoise/ding.ding"))

(event `DetatchedFromVan`
  ;[1 1 1] Falls from van
  (`self.K2_SetActorLocation` (-122.0 -315.0 570.0) false true)
  (`PrimitiveComponent.SetSimulatePhysics` (`self.PetMesh`) true)
  (set `self.Fallen` true)
  (if (`self.Puppy`)
    (set `self.Sound` "/Game/Audio/Puppies/puppyhurt1.puppyhurt1")
    (else
      (set `self.Sound` "/Game/Audio/KittenNoise/AC04_69_1_CatMeowsHighpitch.AC04_69_1_CatMeowsHighpitch")))
  (`GameplayStatics.SpawnSoundAttached` (`self.Sound`) (`self.PetMesh`) "None" (0.0 0.0 0.0) (struct) "KeepRelativeOffset" true)
  (`KismetSystemLibrary.Delay` 60.0)
  (if (`self.Fallen`)
    (`self.Dropped`)))

(event `PickedUpByEnemy`
  (bind _petmesh (`self.PetMesh`))
  ;[1 1 1] Picked up by enemy
  (`PrimitiveComponent.SetSimulatePhysics` _petmesh false)
  (`PrimitiveComponent.SetCollisionEnabled` _petmesh "NoCollision")
  (`PrimitiveComponent.SetCollisionEnabled` (`self.Sphere`) "NoCollision")
  (set `self.Fallen` false)
  (if (`self.Puppy`)
    (set `self.Sound` "/Game/Audio/Puppies/LF01_41_PuppyYelpWhineBarkA.LF01_41_PuppyYelpWhineBarkA")
    (else
      (set `self.Sound` "/Game/Audio/KittenNoise/AC04_69_1_CatMeowsHighpitch.AC04_69_1_CatMeowsHighpitch")))
  (`GameplayStatics.SpawnSoundAttached` (`self.Sound`) (`self.PetMesh`) "None" (0.0 0.0 0.0) (struct) "KeepRelativeOffset" true)
  (`PrimitiveComponent.SetCollisionResponseToAllChannels` (`self.Sphere`) "ECR_Ignore"))

(event `DestroySelf`
  ;[1 1 1] Kills pet
  (`self.K2_DestroyActor`))

(fn `UserConstructionScript`
  (locals (NewLocalVar_0 :type Integer :default 0))
  (bind _petmesh (`self.PetMesh`))
  (bind _meshes (`self.Meshes`))
  (bind _catmats (`self.CatMats`))
  (bind _puppymats (`self.PuppyMats`))
  (set `local.NewLocalVar_0` (`KismetMathLibrary.RandomIntegerInRange` 0 (- (`KismetArrayLibrary.Array_Length` _meshes) 1)))
  (`StaticMeshComponent.SetStaticMesh` _petmesh (`|GetArrayItem` _meshes (`local.NewLocalVar_0`)))
  (if (== (`local.NewLocalVar_0`) 1)
    (set `self.Puppy` true)
    (`PrimitiveComponent.SetMaterial` _petmesh 0 (`|GetArrayItem` _puppymats (`KismetMathLibrary.RandomIntegerInRange` 0 (- (`KismetArrayLibrary.Array_Length` _puppymats) 1))))
    (else
      (`PrimitiveComponent.SetMaterial` _petmesh 0 (`|GetArrayItem` _catmats (`KismetMathLibrary.RandomIntegerInRange` 0 (- (`KismetArrayLibrary.Array_Length` _catmats) 1)))))))