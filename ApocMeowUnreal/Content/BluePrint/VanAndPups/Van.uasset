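; Van actor that carries five spawned pets, shows its health and blocks or allows VR teleporting as the player overlaps its box.
; Damage shakes it toward a small random rotation and back, and can randomly detach a pet; SpawnNewPet restores dropped pets.
; Timeline_0, with no trigger wired in the graph, drives damage buildup, drop cooldown, shake gate and level reload when no pets remain.
; Another timeline swings the cooler lid.
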(event `self.ReceiveBeginPlay`
  (bind (_returnvalue_roll _returnvalue_pitch _returnvalue_yaw) (`KismetMathLibrary.BreakRotator` (`SceneComponent.K2_GetComponentRotation` (`self.DefaultSceneRoot`))))
  ;[1 1 1] Begin Play
  (set `self.PlyWorldLoc` (`SceneComponent.K2_GetComponentLocation` (`self.PlayLocation`)))
  (set `self.DefaultSpace` (`KismetMathLibrary.MakeRotator` _returnvalue_roll _returnvalue_pitch _returnvalue_yaw))
  (bind _output_get (set `self.PetLocArray` (`|MakeArray` (`self.Scene`) (`self.Scene1`) (`self.Scene2`) (`self.Scene3`) (`self.Scene4`))))
  (for (_array_element _array_index) _output_get
    (bind _returnvalue (`|SpawnActorFromClass` "/Game/BluePrint/VanAndPups/Pet_BP.Pet_BP_C" (`SceneComponent.K2_GetComponentToWorld` _array_element) "AlwaysSpawn" "OverrideRootScale" null _array_index self null))
    (`KismetArrayLibrary.Array_Add` (`self.PetsLeft`) _returnvalue)
    (`self.K2_AttachToActor` _returnvalue self "None" "KeepWorld" "KeepWorld" "KeepRelative" true))
  (set `self.PetsOnVan` (`self.PetsLeft`)))

(event `self.ReceiveTick`
  (params (DeltaSeconds :type "Float (single-precision)"))
  ;[1 1 1] Set HP Text
  (set `self.DeltaTime` DeltaSeconds)
  (`TextRenderComponent.K2_SetText` (`self.TextRender`) (`KismetTextLibrary.Conv_DoubleToText` (`/Game/BluePrint/AI/Health.Health` (`self.Health`)) "HalfToEven")))

(event `self.Box1.OnComponentBeginOverlap`
  (params (OverlappedComponent :type "PrimitiveComponent Object Reference") (OtherActor :type "Actor Object Reference") (OtherComp :type "PrimitiveComponent Object Reference") (OtherBodyIndex :type Integer) (bFromSweep :type Boolean) (SweepResult :type "HitResult Structure (by ref)"))
  ;[1 1 1] In tele collision
  (cast `/Game/BluePrint/Players/BP_VRChar1` OtherActor)
  (`PrimitiveComponent.SetCollisionResponseToChannel` (`self.Box1`) "ECC_Visibility" "ECR_Ignore")
  (`PrimitiveComponent.SetCollisionResponseToChannel` (`self.Capsule`) "ECC_Visibility" "ECR_Ignore")
  (set `self.CanTele` false))

(event `Spawn New Pet`
  (params (ID :type Integer) (Pet :type "Actor Object Reference"))
  ;[1 1 1] Add Pets Back To the Van When Dropped by Enemy
  (bind _returnvalue (`|SpawnActorFromClass` "/Game/BluePrint/VanAndPups/Pet_BP.Pet_BP_C" (`SceneComponent.K2_GetComponentToWorld` (`|GetArrayItem` (`self.PetLocArray`) ID)) "AlwaysSpawn" "OverrideRootScale" null ID self null))
  (`KismetArrayLibrary.Array_Add` (`self.PetsLeft`) _returnvalue)
  (`KismetArrayLibrary.Array_Add` (`self.PetsOnVan`) _returnvalue)
  (`self.K2_AttachToActor` _returnvalue self "None" "KeepWorld" "KeepWorld" "KeepRelative" true)
  (`self.K2_DestroyActor` Pet))

(event `self.Box1.OnComponentEndOverlap`
  (params (OverlappedComponent :type "PrimitiveComponent Object Reference") (OtherActor :type "Actor Object Reference") (OtherComp :type "PrimitiveComponent Object Reference") (OtherBodyIndex :type Integer))
  ;[1 1 1] out of tele collision
  (cast `/Game/BluePrint/Players/BP_VRChar1` OtherActor)
  (`PrimitiveComponent.SetCollisionResponseToChannel` (`self.Box1`) "ECC_Visibility" "ECR_Block")
  (`PrimitiveComponent.SetCollisionResponseToChannel` (`self.Capsule`) "ECC_Visibility" "ECR_Block")
  (set `self.CanTele` true))

(event `self.ReceiveAnyDamage`
  (params (Damage :type "Float (single-precision)") (DamageType :type "DamageType Object Reference") (InstigatedBy :type "Controller Object Reference") (DamageCauser :type "Actor Object Reference"))
  (bind _returnvalue (`self.K2_GetActorRotation`))
  (bind _returnvalue_2 (`self.K2_GetActorRotation`))
  (bind _defaultspace (`self.DefaultSpace`))
  (bind _petsonvan (`self.PetsOnVan`))
  (bind _defaultsceneroot (`self.DefaultSceneRoot`))
  (bind _targetrot (`self.TargetRot`))
  ;[1 1 1] Van Shaking and Pet Loss
  (set `self.TakingDamage` true)
  (`|ExecutionSequence`
    (:`then_0`
      (`self.SetTargetRot` :!label _label))
    (:`then_1`
      (`/Engine/EditorBlueprintResources/StandardMacros.Gate` true :!via `Open` :!label _label_2
        (:`Exit`
          ;;[1 1 1] Shake RV
          (if (`self.Reached`)
            (`SceneComponent.K2_SetWorldRotation` _defaultsceneroot (`KismetMathLibrary.RInterpTo` _returnvalue _defaultspace (`self.DeltaTime`) (`self.RotateSpeed`)) false false)
            (if (== _returnvalue _defaultspace :`ErrorTolerance` 0.01)
              (set `self.Reached` false)
              (`|ExecutionSequence`
                (:`then_0`
                  (goto _label :!via `Reset`))
                (:`then_1`
                  (goto _label_2 :!via `Close`))))
            (else
              (`SceneComponent.K2_SetWorldRotation` _defaultsceneroot (`KismetMathLibrary.RInterpTo` _returnvalue_2 _targetrot (`self.DeltaTime`) (`self.RotateSpeed`)) false false)
              (if (== _returnvalue_2 _targetrot :`ErrorTolerance` 0.01)
                (set `self.Reached` true)))))))
    (:`then_2`
      ;;[1 1 1] Lose Pets
      (if (`self.CanLosePet`)
        (if (<= (`KismetMathLibrary.RandomFloatInRange` 0.0 100.0) (+ (`self.Buildup`) (`self.VanHealthMultiplier`)))
          (for (_array_element _array_index) _petsonvan
            (if (== _array_index (`self.PetToDrop`))
              (`self.K2_DetachFromActor` _array_element "KeepRelative" "KeepRelative" "KeepRelative")
              (`/Game/BluePrint/VanAndPups/Pet_BP.DetatchedFromVan` _array_element)
              (`KismetArrayLibrary.Array_Remove` _petsonvan _array_index)))
          (set `self.PetToDrop` (`KismetMathLibrary.RandomIntegerInRange` 0 (- (`KismetArrayLibrary.Array_Length` _petsonvan) 1)))
          (set `self.CanLosePet` false))))
    (:`then_3`
      ;;[1 1 1] Stop Taking Damage
      (`KismetSystemLibrary.RetriggerableDelay` 1.0)
      (set `self.TakingDamage` false))))

(event `CloseLid`
  (bind (_direction _newtrack_2) (`Timeline|Timeline_1` :!via `PlayFromStart` :!label _label_3)
    (:`Update`
      (`SceneComponent.K2_SetRelativeRotation` (`self.cooler_top`) (`KismetMathLibrary.MakeRotator` 0.0 0.0 (+ _newtrack_2 -101.0)) false false))))

(event `OpenLid`
  (goto _label_3 :!via `Reverse`))

(fn `DamageBuildup`
  (params (TakingDamage :type Boolean))
  (if (and TakingDamage (<= (/ (`/Game/BluePrint/AI/Health.Health` (`self.Health`)) 4000.0) 0.9))
    (set `self.Buildup` (`KismetMathLibrary.FClamp` (+ (`self.Buildup`) 0.01) 0.0 15.0))
    (else
      (set `self.Buildup` (`KismetMathLibrary.FClamp` (- (`self.Buildup`) 1.0) 0.0 10000.0)))))

(fn `removePetsAndLoseGame`
  (bind _petsleft (`self.PetsLeft`))
  (for _array_element _petsleft
    (`/Engine/EditorBlueprintResources/StandardMacros.IsValid` _array_element
      (:`Is Not Valid`
        (`KismetArrayLibrary.Array_RemoveItem` _petsleft _array_element))))
  (if (<= (`KismetArrayLibrary.Array_Length` _petsleft) 0)
    (`GameplayStatics.OpenLevel` "MainLevel")))

(fn `ResetLosePet`
  (set `self.CanLosePet` true))

(fn `UserConstructionScript`)